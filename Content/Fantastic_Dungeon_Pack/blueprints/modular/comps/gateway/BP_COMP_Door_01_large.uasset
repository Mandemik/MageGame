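; BP_COMP_Door_01_large is a large double-leaf gateway door from the Fantastic Dungeon Pack's modular components that swings open and closed.
; OpenGate plays the GateHandle timeline, which rotates the left and right door meshes in opposite yaw directions through a rotator lerp.
; CloseGate reverses the same timeline, and the OpenAtStart flag triggers opening on BeginPlay.
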(event Custom|CloseGate
  (bind _progress (Timeline|GateHandle Reverse)
    (:Update
      (Transformation|SetRelativeRotation (Variables|Default|GetMOD_Gateway_Door_01_large_door_R) (Math|Rotator|Lerp(Rotator) "0, 0, 0" "0,-120.000000, 0" _progress) false false)
      (Transformation|SetRelativeRotation (Variables|Default|GetMOD_Gateway_Door_01_large_door_L) (Math|Rotator|Lerp(Rotator) "0, 0, 0" "0,120.000000, 0" _progress) false false))))

(event Custom|OpenGate
  (bind _progress (Timeline|GateHandle Play)
    (:Update
      (Transformation|SetRelativeRotation (Variables|Default|GetMOD_Gateway_Door_01_large_door_R) (Math|Rotator|Lerp(Rotator) "0, 0, 0" "0,-120.000000, 0" _progress) false false)
      (Transformation|SetRelativeRotation (Variables|Default|GetMOD_Gateway_Door_01_large_door_L) (Math|Rotator|Lerp(Rotator) "0, 0, 0" "0,120.000000, 0" _progress) false false))))

(event EventBeginPlay
  (if (Variables|Default|GetOpenAtStart)
    (CallFunction|OpenGate)))

(fn ConstructionScript)