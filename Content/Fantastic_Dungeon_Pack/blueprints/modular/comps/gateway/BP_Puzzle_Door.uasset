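; BP_Puzzle_Door is a dungeon gateway that opens when gemstones are activated in a set order.
; Each newly active gemstone is appended to the current sequence and compared with the proper sequence at that index, though the first is always accepted.
; A later mismatch deactivates every recorded gemstone and clears the sequence.
; An accepted entry prints a debug message and calls OpenGate once both sequences match in length.
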(event Custom|NewGemStoneActive
  (params (NewGemStone :type BP%20Gemstone%20Puzzle%20Object%20Reference))
  (bind _returnvalue (Utilities|Array|Add (Variables|Default|GetCurentSequence) NewGemStone))
  (if (or (== (Utilities|Array|Get(acopy) (Variables|Default|GetProperSequence) _returnvalue) NewGemStone) (== _returnvalue 0))
    (Development|PrintString "Super")
    (if (== (Utilities|Array|Length (Variables|Default|GetProperSequence)) (Utilities|Array|Length (Variables|Default|GetCurentSequence)))
      (CallFunction|OpenGate))
    (else
      (for _array_element (Variables|Default|GetCurentSequence)
        (Default|ActiveGemstone _array_element false))
      (Utilities|Array|Clear (Variables|Default|GetCurentSequence)))))

(fn ConstructionScript)