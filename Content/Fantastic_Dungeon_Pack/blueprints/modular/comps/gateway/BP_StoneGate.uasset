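; BP_StoneGate is a modular dungeon gate that slides between closed and open positions.
; On BeginPlay it binds an event to the brazier-active event of a referenced obelisk, or prints a warning if none is set.
; SwitchDoor flips the open state and plays or reverses a timeline that lerps the gate's scene component.
; The construction script applies the initial position from the open flag.
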(event Custom|SwitchDoor
  (bind _output_get (Variables|Default|SetDoorIsOpen? (not (Variables|Default|GetDoorIsOpen?))))
  (if _output_get
    (bind _progress (Timeline|OpenGate Play)
      (:Update
        (Transformation|SetRelativeLocation (Variables|Default|GetScene1) (Math|Vector|Lerp(Vector) "0, 0, 0" (Variables|Default|GetOpenLocation) _progress) false false)))
    (else
      (Timeline|OpenGate Reverse))))

(event EventBeginPlay
  (Utilities|IsValid (Variables|Default|GetObeliskRef)
    (:Is%20Valid
      (EventDispatchers|BindEventtoBrazierActive (Variables|Default|GetObeliskRef) (EventDispatchers|CreateEvent :!event Custom|SwitchDoor)))
    (:Is%20Not%20Valid
      (Development|PrintString "Obelisk ref is not set!"))))

(fn ConstructionScript
  (Transformation|SetRelativeLocation (Variables|Default|GetScene1) (select (Variables|Default|GetDoorIsOpen?) (Variables|Default|GetOpenLocation) "0, 0, 0") false false))