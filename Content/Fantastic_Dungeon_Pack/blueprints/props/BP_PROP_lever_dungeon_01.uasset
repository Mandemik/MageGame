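; Dungeon lever prop that toggles between on and off when interacted with.
; Each interaction flips LeverActive and plays or reverses the EnableLever timeline, which rotates the handle mesh on roll between its two end angles.
; When the timeline finishes, it calls LeverActivation with the current LeverActive state so other logic can react.
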(event EventInteractwithObject
  (params (InteractCauser :type BP%20Player%20Character%20Object%20Reference))
  (if (not (Variables|Default|GetLeverActive))
    (Variables|Default|SetLeverActive true)
    (bind _leverprogress (Timeline|EnableLever Play)
      (:Update
        (Transformation|SetRelativeRotation (Variables|Default|GetSM_PROP_lever_handle_dungeon_02) (Math|Rotator|MakeRotator (Math|Float|Lerp -6e+01 6e+01 _leverprogress) 0.0 0.0) false false))
      (:Finished
        (Default|CallLeverActivation (Variables|Default|GetLeverActive))))
    (else
      (Variables|Default|SetLeverActive false)
      (Timeline|EnableLever Reverse))))

(fn ConstructionScript)

(fn NewFunction0)