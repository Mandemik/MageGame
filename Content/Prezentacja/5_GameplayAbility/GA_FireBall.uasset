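; Gameplay ability that casts a fireball from the player character toward the point under the mouse cursor.
; On activation it caches the player, commits the ability and plays the self-cast montage, ending when that completes or is interrupted.
; A montage notify spawns a small projectile slightly in front of the player, using only the yaw toward the cursor hit, with the player as instigator.
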(event Ability|EventActivateAbility
  (CallFunction|SetVariables)
  (Ability|CommitAbility)
  (bind _notifyname (Animation|Montage|PlayMontage (Variables|/Script/Engine.Character|GetMesh (Variables|Default|GetPlayerRef)) "/Game/Animation/MagPacket/AM_SelfCast.AM_SelfCast")
    (:OnCompleted
      (Ability|EndAbility :!label _label))
    (:OnInterrupted
      (goto _label))
    (:OnNotifyBegin
      (switch name _notifyname
        (:Cast
          (CallFunction|SpawnFireBall))))))

(fn SpawnFireBall
  (bind _playerref (Variables|Default|GetPlayerRef))
  (bind _returnvalue (Pawn|GetController _playerref))
  (bind _returnvalue_2 (Transformation|GetActorLocation _playerref))
  (bind _asplayer_controller (Utilities|Casting|CastToPlayerController _returnvalue))
  (bind _hitresult (Game|Player|GetHitResultUnderCursorbyChannel _asplayer_controller "TraceTypeQuery1" true))
  (bind _returnvalue_3 (Math|Rotator|FindLookatRotation _returnvalue_2 (.location _hitresult)))
  (Game|SpawnActorfromClass "/Game/VFX/sA_Megapack_v1/sA_Projectilevfx/Vfx/Blueprints/BP_Projectile_2_Small.BP_Projectile_2_Small_C" (Math|Transform|MakeTransform (+ (Transformation|GetActorLocation (Variables|Default|GetPlayerRef)) (* (Math|Vector|GetForwardVector (Math|Rotator|MakeRotator 0.0 0.0 (.yaw _returnvalue_3))) (Variables|Default|GetFireballOffset))) (Math|Rotator|MakeRotator 0.0 0.0 (.yaw _returnvalue_3))) "AdjustIfPossibleButAlwaysSpawn" 0 (Variables|Default|GetPlayerRef)) ; Spawn projectile
)

(fn SetVariables
  (bind _asbp_player_character (Utilities|Casting|CastToBP_PlayerCharacter (.owneractor (Ability|GetActorInfo))))
  (Variables|Default|SetPlayerRef _asbp_player_character))