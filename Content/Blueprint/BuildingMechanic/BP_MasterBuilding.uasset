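; BP_MasterBuilding is an interactable build station where the player spends inventory items to unlock buildings.
; A sphere overlap shows its prompt widget and registers it with the player; interacting swaps the HUD for a cached W_BuildHud.
; TryToCreateBuilding finds the named DT_BuildingList row, checks and removes its cost through the InventoryManager.
; It then enables the matching-class actor in BuildingArray rather than spawning one, and reports the quest objective.
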(event OnComponentBeginOverlap(Sphere)
  (params (OverlappedComponent :type Primitive%20Component%20Object%20Reference) (OtherActor :type Actor%20Object%20Reference) (OtherComp :type Primitive%20Component%20Object%20Reference) (OtherBodyIndex :type Integer) (bFromSweep :type Boolean) (SweepResult :type Hit%20Result%20Structure%20%28by%20ref%29))
  (bind _asbp_player_character (Utilities|Casting|CastToBP_PlayerCharacter OtherActor))
  (Development|PrintString (Utilities|String|Append (Utilities|GetDisplayName OtherActor) " overlap  Start with me"))
  (Class|BPInteractionInterface|CanInteractwithMe(Message) _asbp_player_character true self)
  (Rendering|SetVisibility (Variables|Default|GetWidget) true false))

(event OnComponentEndOverlap(Sphere)
  (params (OverlappedComponent :type Primitive%20Component%20Object%20Reference) (OtherActor :type Actor%20Object%20Reference) (OtherComp :type Primitive%20Component%20Object%20Reference) (OtherBodyIndex :type Integer))
  (bind _asbp_player_character (Utilities|Casting|CastToBP_PlayerCharacter OtherActor))
  (Development|PrintString (Utilities|String|Append (Utilities|GetDisplayName OtherActor) " overlap  End with me"))
  (Class|BPInteractionInterface|CanInteractwithMe(Message) _asbp_player_character false)
  (Rendering|SetVisibility (Variables|Default|GetWidget) false false))

(event Custom|CloseWidget
  (UserInterface|Viewport|AddtoViewport (Variables|/Game/Blueprint/Core/BP_PlayerCharacter.BP_PlayerCharacter_C|GetHudRef (Variables|Default|GetCauser)) 0)
  (Widget|RemovefromParent (Variables|Default|GetBuildWidgetRef))
  (Input|SetInputModeGameandUI (.AsPlayer%20Controller (Utilities|Casting|CastToPlayerController (Pawn|GetController (Variables|Default|GetCauser)))) (Variables|/Game/Blueprint/Core/BP_PlayerCharacter.BP_PlayerCharacter_C|GetHudRef (Variables|Default|GetCauser)) "DoNotLock" true))

(event EventInteractwithObject
  (params (InteractCauser :type BP%20Player%20Character%20Object%20Reference))
  (bind _buildwidgetref (Variables|Default|GetBuildWidgetRef))
  (bind _w_buildwidget (Variables|/Game/UI/W_BuildHud.W_BuildHud_C|GetW_BuildWidget _buildwidgetref))
  (bind _output_get (Variables|Default|SetCauser InteractCauser))
  (Widget|RemovefromParent (Variables|/Game/Blueprint/Core/BP_PlayerCharacter.BP_PlayerCharacter_C|GetHudRef _output_get))
  (Utilities|IsValid (Variables|Default|GetBuildWidgetRef)
    (:Is%20Valid
      _)
    (:Is%20Not%20Valid
      (CallFunction|CreateWidget (.AsPlayer%20Controller (Utilities|Casting|CastToPlayerController (Pawn|GetController _output_get))))))
  (UserInterface|Viewport|AddtoViewport (Variables|Default|GetBuildWidgetRef) 0)
  (Input|SetInputModeUIOnly (.AsPlayer%20Controller (Utilities|Casting|CastToPlayerController (Pawn|GetController _output_get))) (Variables|Default|GetBuildWidgetRef) "DoNotLock")
  (Variables|/Game/UI/W_BuildWidget.W_BuildWidget_C|SetMasterActor _w_buildwidget self)
  (EventDispatchers|BindEventtoCloseWidget _w_buildwidget (EventDispatchers|CreateEvent :!event Custom|CloseWidget))
  (Development|PrintString "Interact with Build Master"))

(fn ConstructionScript)

(fn TrytoCreateBuilding
  (params (BuildName :type String))
  (bind _outrownames (DataTable|GetDataTableRowNames (Variables|Default|GetBuildingDataTable)))
  (bind _array_element (Utilities|Array|ForEachLoopwithBreak _outrownames)
    (:LoopBody
      (bind _returnvalue (Utilities|GetDataTableRow "/Game/Blueprint/BuildingMechanic/Data/DT_BuildingList.DT_BuildingList" _array_element)
        (:then
          (if (Utilities|Enum|Equal(Enum) (.build_name _returnvalue) BuildName)
            (bind _hadenough_ (CallFunction|CheckRequireItems (.build_cost_array _returnvalue)))
            (if _hadenough_
              (CallFunction|RemoveRequireItems (.build_cost_array _returnvalue))
              (bind _array_element_2 (Utilities|Array|ForEachLoopwithBreak (Variables|Default|GetBuildingArray))
                (:LoopBody
                  (if (== (Utilities|GetClass _array_element_2) (.build_class _returnvalue))
                    (Default|EnableBuilding _array_element_2 true)
                    (Default|TryFinishObjective (Variables|Default|GetManager_QuestTarget) (Utilities|String|StringToName BuildName) (Variables|Default|GetCauser))
                    (return true))))
              (else
                (Development|PrintString "Not Enought Material")
                (return false)))))))))

(fn RemoveRequireItems
  (params (RequireItemList :type Map%20of%20EItems%20Enums%20to%20Integers :default "NewEnumerator6"))
  (bind _keys (Utilities|Map|Keys RequireItemList))
  (for _array_element _keys
    (Default|RemoveItem (Variables|/Game/Blueprint/Core/BP_PlayerCharacter.BP_PlayerCharacter_C|GetInventoryManager (Variables|Default|GetCauser)) _array_element (.Value (Utilities|Map|Find RequireItemList _array_element)))))

(fn CheckRequireItems
  (params (RequireItemList :type Map%20of%20EItems%20Enums%20to%20Integers :default "NewEnumerator6"))
  (bind _keys (Utilities|Map|Keys RequireItemList))
  (for _array_element _keys
    (bind _hadenough_ (Default|CheckItemAmmount (Variables|/Game/Blueprint/Core/BP_PlayerCharacter.BP_PlayerCharacter_C|GetInventoryManager (Variables|Default|GetCauser)) _array_element (.Value (Utilities|Map|Find RequireItemList _array_element))))
    (if (not _hadenough_)
      (LocalVariables|SetHadEnough false)))
  (return (LocalVariables|GetHadEnough)))

(fn CreateWidget
  (params (OwningPlayer :type Player%20Controller%20Object%20Reference))
  (bind _returnvalue (UserInterface|CreateWidget "/Game/UI/W_BuildHud.W_BuildHud_C" OwningPlayer))
  (Variables|Default|SetBuildWidgetRef _returnvalue))