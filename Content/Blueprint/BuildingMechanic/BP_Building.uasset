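; BP_Building is a building actor that can be switched between enabled and disabled states.
; EnableBuilding stores IsEnable, then shows or hides the static mesh with its children and toggles collision between query-and-physics and none.
; BeginPlay and the save-system ActorLoaded event both reapply IsEnable, keeping visibility and collision in sync with that flag.
; ComponentsToSave returns no components.
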(event Custom|EnableBuilding
  (params (Enable :type Boolean))
  (bind _output_get (Variables|Default|SetIsEnable Enable))
  (if _output_get
    (Rendering|SetVisibility (Variables|Debug|GetStaticMeshComponent) true true)
    (Collision|SetCollisionEnabled (Variables|Debug|GetStaticMeshComponent) "QueryAndPhysics")
    (else
      (Rendering|SetVisibility (Variables|Debug|GetStaticMeshComponent) false true)
      (Collision|SetCollisionEnabled (Variables|Debug|GetStaticMeshComponent) "NoCollision"))))

(event EventBeginPlay
  (CallFunction|EnableBuilding (Variables|Default|GetIsEnable)))

(event EventActorLoaded
  (CallFunction|EnableBuilding (Variables|Default|GetIsEnable)))

(fn ConstructionScript)

(fn ComponentstoSave
  (return 0))