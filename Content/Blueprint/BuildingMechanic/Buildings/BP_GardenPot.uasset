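; BP_GardenPot is an interactable garden pot building where the player plants seeds and collects herbs.
; Interaction follows the pot state, exchanging seeds or herbs with the causer's inventory, while ImprovePlant turns a planted seed into a random Moonlight Herb or Bloody Root.
; A timeline drives a dynamic material's appearance, reversing on removal to clear the mesh while interaction stays blocked.
; ActorLoaded rebuilds the visual from the pot state.
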(event Custom|PlayPlantAnimation
  (bind _plant (Variables|Default|GetPlant))
  (bind _returnvalue (Rendering|Material|CreateDynamicMaterialInstance _plant 0 (Rendering|Material|GetMaterial _plant 0) "None" :!class /Script/Engine.PrimitiveComponent))
  (Rendering|Material|SetVectorParameterValue _returnvalue "EmmisionColor" (Variables|Default|GetPlantColor) :!class /Script/Engine.MaterialInstanceDynamic)
  (bind (_direction _progress) (Timeline|PlantSeedAnimation PlayFromStart)
    (:Update
      (Rendering|Material|SetScalarParameterValue _returnvalue "Appearance" _progress :!class /Script/Engine.MaterialInstanceDynamic))
    (:Finished
      (switch Utilities|FlowControl|Switch|SwitchonETimelineDirection _direction
        (:Backward
          (Variables|Default|SetBlockInteraction false)
          (Components|StaticMesh|SetStaticMesh (Variables|Default|GetPlant) 0))))))

(event Custom|PlayHarvestAnimation
  (Variables|Default|SetBlockInteraction true)
  (bind (_direction _progress) (Timeline|PlantSeedAnimation ReverseFromEnd)
    (:Update
      (Rendering|Material|SetScalarParameterValue (stale Custom|PlayPlantAnimation _returnvalue) "Appearance" _progress :!class /Script/Engine.MaterialInstanceDynamic))
    (:Finished
      (switch Utilities|FlowControl|Switch|SwitchonETimelineDirection _direction
        (:Backward
          (Variables|Default|SetBlockInteraction false)
          (Components|StaticMesh|SetStaticMesh (Variables|Default|GetPlant) 0))))))

(event EventActorLoaded
  (switch Utilities|FlowControl|Switch|SwitchonE_PotProgress (Variables|Default|GetPotProgress)
    (:NewEnumerator0
      (CallFunction|SetupEmptyVisual))
    (:NewEnumerator1
      (CallFunction|SetupPlantedVisual))
    (:NewEnumerator2
      (CallFunction|SetupGrowUpVisual))))

(fn ConstructionScript
  (|CallParentFunction))

(fn InteractwithBuilding
  (|CallParentFunction)
  (if (not (Variables|Default|GetBlockInteraction))
    (switch Utilities|FlowControl|Switch|SwitchonE_PotProgress (Variables|Default|GetPotProgress)
      (:NewEnumerator0
        (CallFunction|PlantSeed))
      (:NewEnumerator1
        (CallFunction|RemoveSeed))
      (:NewEnumerator2
        (CallFunction|CollectFruts)))))

(fn SetupPlantedVisual
  (bind _plant (Variables|Default|GetPlant))
  (Components|StaticMesh|SetStaticMesh _plant (Variables|Default|GetSeedMesh))
  (Rendering|Material|SetMaterial _plant 0 (Variables|Default|GetSeedMaterial))
  (CallFunction|PlayPlantAnimation))

(fn SetupGrowUpVisual
  (bind _plant (Variables|Default|GetPlant))
  (Components|StaticMesh|SetStaticMesh _plant (Variables|Default|GetGrowUpMesh))
  (switch Utilities|FlowControl|Switch|SwitchonEItems (Variables|Default|GetHerbType)
    (:NewEnumerator23
      (LocalVariables|SetMaterialToSet (Variables|Default|GetMoonLightMaterial)))
    (:NewEnumerator24
      (LocalVariables|SetMaterialToSet (Variables|Default|GetBloodyRootsMaterial))))
  (Rendering|Material|SetMaterial _plant 0 (LocalVariables|GetMaterialToSet))
  (CallFunction|PlayPlantAnimation))

(fn SetupEmptyVisual
  (CallFunction|PlayHarvestAnimation))

(fn ImprovePlant
  (if (Utilities|Enum|Equal(Enum) (Variables|Default|GetPotProgress) "NewEnumerator1")
    (Variables|Default|SetPotProgress "NewEnumerator2")
    (Variables|Default|SetHerbType (select (Math|Random|RandomBool) "NewEnumerator24" "NewEnumerator23"))
    (CallFunction|SetupGrowUpVisual)))

(fn PlantSeed
  (bind _causer (Variables|Default|GetCauser))
  (bind _inventorymanager (Variables|/Game/Blueprint/Core/BP_PlayerCharacter.BP_PlayerCharacter_C|GetInventoryManager _causer))
  (bind _hadenough_ (Default|CheckItemAmmount _inventorymanager "NewEnumerator31" 1))
  (if _hadenough_
    (bind _success_ (Default|RemoveItem _inventorymanager "NewEnumerator31" 1))
    (if _success_
      (Variables|Default|SetPotProgress "NewEnumerator1")
      (CallFunction|SetupPlantedVisual))))

(fn RemoveSeed
  (bind _success (Default|AddItem (Variables|/Game/Blueprint/Core/BP_PlayerCharacter.BP_PlayerCharacter_C|GetInventoryManager (Variables|Default|GetCauser)) "NewEnumerator31" 1))
  (if _success
    (Variables|Default|SetPotProgress "NewEnumerator0")
    (CallFunction|SetupEmptyVisual)))

(fn CollectFruts
  (bind _success (Default|AddItem (Variables|/Game/Blueprint/Core/BP_PlayerCharacter.BP_PlayerCharacter_C|GetInventoryManager (Variables|Default|GetCauser)) (Variables|Default|GetHerbType) 1))
  (if _success
    (Variables|Default|SetPotProgress "NewEnumerator0")
    (CallFunction|SetupEmptyVisual)))