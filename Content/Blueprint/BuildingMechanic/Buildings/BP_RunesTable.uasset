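; BP_RunesTable is a placeable building in the building mechanic that gives the interacting player access to rune setup.
; Interacting runs the parent logic, attempts to finish the "Interact" quest objective through the quest target manager, then calls SetupRunes on the causer.
; Its show-up animation also toggles a desk drawer interior mesh's visibility before running the parent animation.
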(fn ConstructionScript
  (|CallParentFunction))

(fn ComponentstoSave
  (return 0))

(fn CustomShowUpAnimation
  (params (ShowIt :type Boolean))
  (Rendering|SetVisibility (Variables|Default|GetSM_PROP_desk_drawer_01_interior_02) ShowIt false)
  (|CallParentFunction ShowIt))

(fn InteractwithBuilding
  (bind _causer (Variables|Default|GetCauser))
  (|CallParentFunction)
  (Default|TryFinishObjective (Variables|Default|GetManager_QuestTarget) "Interact" _causer)
  (Default|SetupRunes _causer))