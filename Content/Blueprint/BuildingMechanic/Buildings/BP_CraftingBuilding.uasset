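; BP_CraftingBuilding is a building Blueprint that crafts items using the inventory of its Causer.
; TryCreateItem scans DT_CraftingList for the row matching the requested item enum and reads its cost map.
; CheckRequireItem tests each cost against the InventoryManager; if all pass, RemoveRequireItems deducts them and one crafted item is added.
; Otherwise it prints a not-enough-material message and returns false.
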(fn ConstructionScript
  (|CallParentFunction))

(fn TryCreateItem
  (params (ItemToCreate :type EItems%20Enum :default "NewEnumerator6"))
  (bind _outrownames (DataTable|GetDataTableRowNames "/Game/Blueprint/BuildingMechanic/Data/DT_CraftingList.DT_CraftingList"))
  (bind _array_element (Utilities|Array|ForEachLoopwithBreak _outrownames)
    (:LoopBody
      (bind _returnvalue (Utilities|GetDataTableRow "/Game/Blueprint/BuildingMechanic/Data/DT_CraftingList.DT_CraftingList" _array_element)
        (:then
          (if (Utilities|Enum|Equal(Enum) (.crafting_item_enum _returnvalue) ItemToCreate)
            (bind _hadenough_ (CallFunction|CheckRequireItem (.crafting_item_cost_array _returnvalue)))
            (if _hadenough_
              (CallFunction|RemoveRequireItems (.crafting_item_cost_array _returnvalue))
              (bind _success (Default|AddItem (Variables|/Game/Blueprint/Core/BP_PlayerArenaCharacter.BP_PlayerArenaCharacter_C|GetInventoryManager (Variables|Default|GetCauser)) ItemToCreate 1))
              (return _success)
              (else
                (Development|PrintString "Not Enought Material")
                (return false)))))))))

(fn CheckRequireItem
  (params (RequireItemList :type Map%20of%20EItems%20Enums%20to%20Integers :default "NewEnumerator6"))
  (bind _keys (Utilities|Map|Keys RequireItemList))
  (for _array_element _keys
    (bind _hadenough_ (Default|CheckItemAmmount (Variables|/Game/Blueprint/Core/BP_PlayerArenaCharacter.BP_PlayerArenaCharacter_C|GetInventoryManager (Variables|Default|GetCauser)) _array_element (.Value (Utilities|Map|Find RequireItemList _array_element))))
    (if (not _hadenough_)
      (LocalVariables|SetHadEnough false)))
  (return (LocalVariables|GetHadEnough)))

(fn RemoveRequireItems
  (params (ItemsToRemoved :type Map%20of%20EItems%20Enums%20to%20Integers :default "NewEnumerator6"))
  (bind _keys (Utilities|Map|Keys ItemsToRemoved))
  (for _array_element _keys
    (Default|RemoveItem (Variables|/Game/Blueprint/Core/BP_PlayerArenaCharacter.BP_PlayerArenaCharacter_C|GetInventoryManager (Variables|Default|GetCauser)) _array_element (.Value (Utilities|Map|Find ItemsToRemoved _array_element)))))