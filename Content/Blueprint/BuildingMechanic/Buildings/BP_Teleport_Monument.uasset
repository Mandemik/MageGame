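; BP_Teleport_Monument is a building that teleports the player to another map through its teleport HUD widget.
; On opening the widget it binds an event to the teleport widget's TeleportMe, printing a warning if the widget is not a W_TeleportHud.
; The teleport event closes the widget, tries to finish the "Reach" quest objective, then has BP_GameInstance switch to the destination level, flagged as monument travel.
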(event Custom|TeleportPlayerWithMonument
  (params (Destiny :type Name))
  (bind _returnvalue (Game|GetGameInstance))
  (bind (_asbp_game_instance _bsuccess) (Utilities|Casting|CastToBP_GameInstance _returnvalue))
  (CallFunction|BuildingWidgetClosed "Hidden")
  (if _bsuccess
    (Default|TryFinishObjective (Variables|Default|GetManager_QuestTarget) "Reach" (Variables|Default|GetCauser))
    (Default|SwitchMap _asbp_game_instance Destiny true)))

(event EventBeginPlay
  (Development|PrintString "Hello"))

(fn ConstructionScript
  (|CallParentFunction))

(fn InteractwithBuilding
  (|CallParentFunction))

(fn OpenBuildingWidget
  (|CallParentFunction)
  (bind _asw_teleport_hud (Utilities|Casting|CastToW_TeleportHud (Variables|Default|GetWidgetRef))
    (:then
      (EventDispatchers|BindEventtoTeleportMe (Variables|/Game/UI/W_TeleportHud.W_TeleportHud_C|GetW_TeleportWidget _asw_teleport_hud) (EventDispatchers|CreateEvent :!event Custom|TeleportPlayerWithMonument)))
    (:CastFailed
      (Development|PrintString "Wrong Widget For Teleport Monument"))))