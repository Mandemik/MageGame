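; BP_EnchantingTable is a building Blueprint for an enchanting table that opens an alchemy-style crafting HUD.
; It extends parent building logic, registering itself as the crafting building on the W_AlchemicHud's inner widget.
; Opening the widget blends the player's view to a child actor, and closing blends it back to the Causer.
; The show-up animation override also toggles a desk drawer mesh's visibility.
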(event EventBuildingWidgetClosed
  (params (InVisibility :type ESlateVisibility%20Enum :default "Visible"))
  (bind _causer (Variables|Default|GetCauser))
  (|CallParentFunction InVisibility)
  (Game|Player|SetViewTargetwithBlend (Variables|/Game/Blueprint/Core/BP_PlayerArenaCharacter.BP_PlayerArenaCharacter_C|GetPlayerControlerRef _causer) _causer 0.5 "VTBlend_Linear" 0.0 false))

(fn ConstructionScript
  (|CallParentFunction))

(fn ComponentstoSave
  (return 0))

(fn CustomShowUpAnimation
  (params (ShowIt :type Boolean))
  (Rendering|SetVisibility (Variables|Default|GetSM_PROP_desk_drawer_01_interior_02) ShowIt false)
  (|CallParentFunction ShowIt))

(fn CreateBuildingWidget
  (|CallParentFunction)
  (bind _asw_alchemic_hud (Utilities|Casting|CastToW_AlchemicHud (Variables|Default|GetWidgetRef)))
  (Variables|/Game/UI/W_AlchemicWidget.W_AlchemicWidget_C|SetCraftingBuildingRef (Variables|/Game/UI/W_AlchemicHud.W_AlchemicHud_C|GetW_AlchemicWidget _asw_alchemic_hud) self))

(fn OpenBuildingWidget
  (|CallParentFunction)
  (Game|Player|SetViewTargetwithBlend (Variables|/Game/Blueprint/Core/BP_PlayerArenaCharacter.BP_PlayerArenaCharacter_C|GetPlayerControlerRef (Variables|Default|GetCauser)) (Variables|/Script/Engine.ChildActorComponent|GetChildActor (Variables|Default|GetChildActor)) 0.5 "VTBlend_Cubic" 0.0 false))