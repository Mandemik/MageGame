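; Base building actor that can be enabled or disabled and opens a UI when the player interacts with it.
; Enabling toggles collision and plays or reverses a timeline driving "Appearance" on dynamic materials, with an empty CustomShowUpAnimation hook, and is reapplied on load.
; Sphere overlap registers the player for interaction and shows a prompt widget.
; Interaction opens BuildingWidget, hiding the HUD and freezing movement until that widget is hidden.
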(event OnComponentBeginOverlap(Sphere)
  (params (OverlappedComponent :type Primitive%20Component%20Object%20Reference) (OtherActor :type Actor%20Object%20Reference) (OtherComp :type Primitive%20Component%20Object%20Reference) (OtherBodyIndex :type Integer) (bFromSweep :type Boolean) (SweepResult :type Hit%20Result%20Structure%20%28by%20ref%29))
  (bind _asbp_player_character (Utilities|Casting|CastToBP_PlayerArenaCharacter OtherActor))
  (Development|PrintString (Utilities|String|Append (Utilities|GetDisplayName OtherActor) " overlap  Start with me"))
  (bind _output_get (Variables|Default|SetCauser _asbp_player_character))
  (Class|BPInteractionInterface|CanInteractwithMe(Message) _output_get true self)
  (Rendering|SetVisibility (Variables|Default|GetWidget) true false))

(event OnComponentEndOverlap(Sphere)
  (params (OverlappedComponent :type Primitive%20Component%20Object%20Reference) (OtherActor :type Actor%20Object%20Reference) (OtherComp :type Primitive%20Component%20Object%20Reference) (OtherBodyIndex :type Integer))
  (bind _asbp_player_character (Utilities|Casting|CastToBP_PlayerArenaCharacter OtherActor))
  (Development|PrintString (Utilities|String|Append (Utilities|GetDisplayName OtherActor) " overlap  End with me"))
  (Variables|Default|SetCauser 0)
  (Class|BPInteractionInterface|CanInteractwithMe(Message) _asbp_player_character false)
  (Rendering|SetVisibility (Variables|Default|GetWidget) false false))

(event Custom|EnableBuilding
  (params (Enable :type Boolean))
  (bind _output_get (Variables|Default|SetIsEnable Enable))
  (if _output_get
    (Rendering|SetVisibility (Variables|Debug|GetStaticMeshComponent) true true)
    (Collision|SetCollisionEnabled (Variables|Debug|GetStaticMeshComponent) "QueryAndPhysics")
    (Rendering|SetVisibility (Variables|Default|GetWidget) false false)
    (CallFunction|ShowAnimation true)
    (else
      (Rendering|SetVisibility (Variables|Debug|GetStaticMeshComponent) false true)
      (Collision|SetCollisionEnabled (Variables|Debug|GetStaticMeshComponent) "NoCollision")
      (CallFunction|ShowAnimation false))))

(event Custom|ShowAnimation
  (params (ShowIt :type Boolean))
  (if ShowIt
    (CallFunction|CustomShowUpAnimation false)
    (bind (_direction _showprogress) (Timeline|Timeline_0 Play)
      (:Update
        (for _array_element (Variables|Default|GetMaterialArray)
          (Rendering|Material|SetScalarParameterValue _array_element "Appearance" _showprogress :!class /Script/Engine.MaterialInstanceDynamic)))
      (:Finished
        (switch Utilities|FlowControl|Switch|SwitchonETimelineDirection _direction
          (:Forward
            (CallFunction|CustomShowUpAnimation true))
          (:Backward
            (CallFunction|CustomShowUpAnimation false)))))
    (else
      (Timeline|Timeline_0 Reverse))))

(event Custom|BuildingWidgetClosed
  (params (InVisibility :type ESlateVisibility%20Enum :default "Visible"))
  (if (Utilities|Enum|Equal(Enum) InVisibility "Hidden")
    (UserInterface|Viewport|AddtoViewport (Variables|/Game/Blueprint/Core/BP_PlayerArenaCharacter.BP_PlayerArenaCharacter_C|GetHudRef (Variables|Default|GetCauser)) 0)
    (Rendering|SetVisibility (Variables|Default|GetWidget) true false)
    (Pawn|Components|CharacterMovement|SetMovementMode (Variables|/Script/Engine.Character|GetCharacterMovement (Variables|Default|GetCauser)) "MOVE_Walking" 0)
    (Input|SetInputModeGameandUI (.AsPlayer%20Controller (Utilities|Casting|CastToPlayerController (Pawn|GetController (Variables|Default|GetCauser)))) (Variables|/Game/Blueprint/Core/BP_PlayerArenaCharacter.BP_PlayerArenaCharacter_C|GetHudRef (Variables|Default|GetCauser)) "DoNotLock" true)))

(event EventBeginPlay
  (CallFunction|CreateMaterialArray)
  (CallFunction|EnableBuilding (Variables|Default|GetIsEnable)))

(event EventInteractwithObject
  (params (InteractCauser :type BP%20Player%20Arena%20Character%20Object%20Reference))
  (Development|PrintString (Utilities|String|Append (Utilities|GetDisplayName InteractCauser) " interact with " (Utilities|GetObjectName self)))
  (CallFunction|InteractwithBuilding))

(event EventActorLoaded
  (CallFunction|EnableBuilding (Variables|Default|GetIsEnable)))

(fn ConstructionScript)

(fn CreateMaterialArray
  (bind _staticmeshcomponent (Variables|Debug|GetStaticMeshComponent))
  (bind _output_get (LocalVariables|SetMeshList (Components|GetChildrenComponents _staticmeshcomponent false)))
  (Utilities|Array|Add _output_get _staticmeshcomponent)
  (for _array_element (LocalVariables|GetMeshList)
    (bind _asstatic_mesh_component (Utilities|Casting|CastToStaticMeshComponent _array_element))
    (Utilities|IsValid (Rendering|Material|GetMaterial _asstatic_mesh_component 0)
      (:Is%20Valid
        (bind _returnvalue (Rendering|Material|CreateDynamicMaterialInstance _asstatic_mesh_component 0 (Rendering|Material|GetMaterial _asstatic_mesh_component 0) "None" :!class /Script/Engine.PrimitiveComponent))
        (Utilities|Array|Add (Variables|Default|GetMaterialArray) _returnvalue)))))

(fn CustomShowUpAnimation
  (params (ShowIt :type Boolean)))

(fn InteractwithBuilding
  (if (Utilities|IsValidClass (Variables|Default|GetBuildingWidget))
    (CallFunction|OpenBuildingWidget)))

(fn OpenBuildingWidget
  (bind _causer (Variables|Default|GetCauser))
  (if (Utilities|IsValid (Variables|Default|GetWidgetRef))
    (Widget|SetVisibility (Variables|Default|GetWidgetRef) "Visible")
    (else
      (CallFunction|CreateBuildingWidget)))
  (Widget|RemovefromParent (Variables|/Game/Blueprint/Core/BP_PlayerArenaCharacter.BP_PlayerArenaCharacter_C|GetHudRef _causer))
  (Input|SetInputModeUIOnly (.AsPlayer%20Controller (Utilities|Casting|CastToPlayerController (Pawn|GetController _causer))) (Variables|Default|GetWidgetRef) "DoNotLock")
  (Rendering|SetVisibility (Variables|Default|GetWidget) false false)
  (Pawn|Components|CharacterMovement|DisableMovement (Variables|/Script/Engine.Character|GetCharacterMovement (Variables|Default|GetCauser)))
  (EventDispatchers|BindEventtoOnVisibilityChanged (Variables|Default|GetWidgetRef) (EventDispatchers|CreateEvent :!event Custom|BuildingWidgetClosed)))

(fn CreateBuildingWidget
  (bind _returnvalue (UserInterface|CreateWidget (Variables|Default|GetBuildingWidget) (Game|GetPlayerController 0)))
  (bind _output_get (Variables|Default|SetWidgetRef _returnvalue))
  (UserInterface|Viewport|AddtoViewport _output_get 0))

(fn ComponentstoSave
  (return 0))