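; BP_ItemComponent is an actor component that gives its owner chance-based item drops.
; TryDropItem walks the ItemaToDropProcent map and rolls each item independently against its percentage, so one call can drop several or none.
; Each successful roll calls DropItem, which spawns a BP_DroppedItem carrying that item at the owner's transform with a small random horizontal offset.
; The event graph is empty, so drops occur only when these functions are called.
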(event EventBeginPlay)

(event EventTick
  (params (DeltaSeconds :type Float%20%28single-precision%29)))

(fn DropItem
  (params (Item :type EItems%20Enum :default "NewEnumerator0"))
  (bind _returnvalue (Components|GetOwner))
  (bind _returnvalue_2 (Math|Random|RandomFloatinRange -2e+01 2e+01))
  (bind _returnvalue_3 (Transformation|GetActorTransform _returnvalue))
  (Game|SpawnActorfromClass "/Game/InventorySystem/Blueprints/BP_DroppedItem.BP_DroppedItem_C" (Math|Transform|MakeTransform (+ (.location _returnvalue_3) (Math|Vector|MakeVector _returnvalue_2 _returnvalue_2 0.0)) (.rotation _returnvalue_3) (.scale _returnvalue_3)) "Undefined" 0 Item 1 0))

(fn TryDropItem
  (bind _keys (Utilities|Map|Keys (Variables|Default|GetItemaToDropProcent)))
  (for _array_element _keys
    (if (and (.ReturnValue (Utilities|Map|Find (Variables|Default|GetItemaToDropProcent) _array_element)) (< (Math|Random|RandomFloatinRange 0.0 1e+02) (.Value (Utilities|Map|Find (Variables|Default|GetItemaToDropProcent) _array_element))))
      (CallFunction|DropItem _array_element))))