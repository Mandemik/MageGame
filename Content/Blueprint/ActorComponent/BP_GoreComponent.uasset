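; Actor component that adds blood and gore effects to its owning humanoid when it takes damage or dies.
; On BeginPlay it binds to the owner's damage event and, for BP_Humanoid owners, the death event.
; Damage spawns a particle system and a short-lived decal snapped to a random listed bone on the mesh.
; Death spawns a configurable gore actor at the owner's location after a delay.
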(event Custom|OnOwnerTakeDamage
  (params (DamagedActor :type Actor%20Object%20Reference) (Damage :type Float%20%28single-precision%29) (DamageType :type Damage%20Type%20Object%20Reference) (InstigatedBy :type Controller%20Object%20Reference) (DamageCauser :type Actor%20Object%20Reference))
  (bind _returnvalue (Transformation|GetActorLocation DamagedActor))
  (Utilities|FlowControl|Sequence
    (:then_0
      (Utilities|IsValid (Variables|Default|GetBloodHitPartickle)
        (:Is%20Valid
          (Niagara|SpawnSystematLocation (Variables|Default|GetBloodHitPartickle) _returnvalue))))
    (:then_1
      (Utilities|IsValid (Variables|Default|GetBloodHitDecal)
        (:Is%20Valid
          (bind _returnvalue_2 (Rendering|Decal|SpawnDecalatLocation (Variables|Default|GetBloodHitDecal) "32.000000,16.000000,16.000000" _returnvalue "0.000000,0.000000,0.000000" 5.0))
          (Transformation|AttachComponentToComponent _returnvalue_2 (Variables|/Script/Engine.Character|GetMesh (Variables|Default|GetOwnerHumanoid)) (.OutItem (Utilities|Array|Random (Variables|Default|GetBonesForDecales))) "SnapToTarget" "KeepWorld" "KeepWorld" true))))))

(event Custom|OnCharacterdDie
  (bind _ownerhumanoid (Variables|Default|GetOwnerHumanoid))
  (bind _deathgoreactor (Variables|Default|GetDeathGoreActor))
  (Utilities|FlowControl|Delay 4.0)
  (if (Utilities|IsValidClass _deathgoreactor)
    (Game|SpawnActorfromClass _deathgoreactor (Math|Transform|MakeTransform (Transformation|GetActorLocation _ownerhumanoid) "0, 0, 0" "1.000000,1.000000,1.000000") "Undefined" 0 _ownerhumanoid _ownerhumanoid)))

(event EventBeginPlay
  (EventDispatchers|BindEventtoOnTakeAnyDamage (Components|GetOwner) (EventDispatchers|CreateEvent :!event Custom|OnOwnerTakeDamage))
  (bind _asbp_humanoid (Utilities|Casting|CastToBP_Humanoid (Components|GetOwner)))
  (bind _output_get (Variables|Default|SetOwnerHumanoid _asbp_humanoid))
  (EventDispatchers|BindEventtoOnDie _output_get (EventDispatchers|CreateEvent :!event Custom|OnCharacterdDie)))