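; Player mage character for the arena, linking input to Ability System abilities, the HUD, inventory quick bar and death menu.
; Skill slots press ability input IDs, while holding mix-spell mode turns the three slots into runes matched against combo abilities on offset IDs.
; A looping timer optionally turns the control rotation toward cursor or right stick.
; A timeline drives dash velocity, and Tick overrides the audio listener using camera boom rotation.
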(event Custom|MakeDash
  (params (DashDistance :type Float%20%28double-precision%29))
  (bind _progressmultiply (Timeline|Dash PlayFromStart)
    (:Update
      (Variables|/Script/Engine.MovementComponent|SetVelocity (Variables|Character|GetCharacterMovement) (Math|Vector|MakeVector (.x (* (Transformation|GetActorForwardVector) (* _progressmultiply (* DashDistance 3.3)))) (.y (* (Transformation|GetActorForwardVector) (* _progressmultiply (* DashDistance 3.3)))) (.z (Variables|/Script/Engine.MovementComponent|GetVelocity (Variables|Character|GetCharacterMovement))))))
    (:Finished
      (Default|CallRollEnded))))

(event EventBeginPlay
  (|CallParentFunction)
  (CallFunction|SetVariables)
  (Variables|/Script/Engine.PlayerController|SetbShowMouseCursor (Variables|Default|GetPlayerControlerRef) true)
  (CallFunction|ApplyPlayerHud)
  (CallFunction|SetupAbilites))

(event EventCharacterDie
  (bind _hudref (Variables|Default|GetHudRef))
  (|CallParentFunction)
  (Default|ShowUpGameplayMenu _hudref true)
  (Input|SetInputModeUIOnly (Variables|Default|GetPlayerControlerRef) (Variables|/Game/UI/W_PlayerHud.W_PlayerHud_C|GetW_GameplayMenu _hudref) "DoNotLock"))

(event EventTick
  (params (DeltaSeconds :type Float%20%28single-precision%29))
  (bind _returnvalue (Transformation|GetActorRotation))
  (bind _cameraboom (Variables|Default|GetCameraBoom))
  (bind _returnvalue_2 (Transformation|GetWorldRotation _cameraboom))
  (bind _returnvalue_3 (* _returnvalue -1.0))
  (bind _returnvalue_4 (Math|Rotator|CombineRotators _returnvalue_3 _returnvalue_2))
  (Class|PlayerController|SetAudioListenerOverride (Variables|Default|GetPlayerControlerRef) (Variables|Character|GetMesh) "0, 0, 0" (Math|Rotator|MakeRotator (.roll _returnvalue_4) (.pitch _returnvalue_4) (+ (.yaw _returnvalue_4) 9e+01))))

(event EventActorLoaded
  (CallFunction|SetupAbilites))

(event EventAddPoints
  (params (PointsToAdd :type Float%20%28double-precision%29))
  (Default|AddPoints (Variables|Default|GetPlayerStateMage) PointsToAdd))

(event Custom|ActiveDefenceSlot
  (Default|ActiveSlot#Defence (Variables|Default|GetHudRef)))

(event Custom|ActiveCombo
  (params (ComboNumber :type Integer))
  (switch int ComboNumber
    (:1
      (Default|ActiveSlot#1 (Variables|Default|GetHudRef))
      (Audio|PlaySound2D (Variables|Default|GetRune#1Sound) 1.0 1.0 0.0 0 0)
      (bind _returnvalue (Utilities|Array|Add (Variables|Mixing|GetCurrentComboArray) "NewEnumerator3"))
      (CallFunction|CheckComboArray _returnvalue))
    (:2
      (Default|ActiveSlot#2 (Variables|Default|GetHudRef))
      (Audio|PlaySound2D (Variables|Default|GetRune#2Sound) 1.0 1.0 0.0 0 0)
      (bind _returnvalue_2 (Utilities|Array|Add (Variables|Mixing|GetCurrentComboArray) "NewEnumerator0"))
      (CallFunction|CheckComboArray _returnvalue_2))
    (:3
      (Default|ActiveSlot#3 (Variables|Default|GetHudRef))
      (Audio|PlaySound2D (Variables|Default|GetRune#3Sound) 1.0 1.0 0.0 0 0)
      (bind _returnvalue_3 (Utilities|Array|Add (Variables|Mixing|GetCurrentComboArray) "NewEnumerator1"))
      (CallFunction|CheckComboArray _returnvalue_3))))

(event Custom|CheckComboArray
  (params (AddedIndex :type Integer))
  (bind (_founded _skilldata) (CallFunction|CheckCurrentIndex AddedIndex))
  (if _founded
    (if (== (Utilities|Array|Length (Variables|/Game/AbilitySystem/DataTable/SkillData.SkillData_C|GetComboArray _skilldata)) (Utilities|Array|Length (Variables|Mixing|GetCurrentComboArray)))
      (Class|AbilitySystemComponent|PressInputID (Variables|Default|GetAbilitySystemComp) (+ (Utilities|Array|FindItem (Variables|Default|GetComboAbilities) _skilldata) 10))
      (Utilities|Array|Clear (Variables|Mixing|GetCurrentComboArray) :!label _label))
    (else
      (goto _label))))

(event Input|ActionEvents|InputActionActiveSkillSlotTwo
  (params (Key :type Key%20Structure :default "None"))
  ;[1 1 1] AbilitySystem Controll
  (:Pressed
    (if (not (Variables|Default|GetBlockSkillUse))
      (if (not (Variables|Default|GetMixSpellMode))
        (Class|AbilitySystemComponent|PressInputID (Variables|Default|GetAbilitySystemComp) 2)
        (Default|ActiveSlot#2 (Variables|Default|GetHudRef))
        (else
          (CallFunction|ActiveCombo 2)))))
  (:Released
    (Class|AbilitySystemComponent|ReleaseInputID (Variables|Default|GetAbilitySystemComp) 2)))

(event Input|ActionEvents|InputActionActiveSkillSlotThree
  (params (Key :type Key%20Structure :default "None"))
  ;[1 1 1] AbilitySystem Controll
  (:Pressed
    (if (not (Variables|Default|GetBlockSkillUse))
      (if (not (Variables|Default|GetMixSpellMode))
        (Class|AbilitySystemComponent|PressInputID (Variables|Default|GetAbilitySystemComp) 3)
        (Default|ActiveSlot#3 (Variables|Default|GetHudRef))
        (else
          (CallFunction|ActiveCombo 3)))))
  (:Released
    (Class|AbilitySystemComponent|ReleaseInputID (Variables|Default|GetAbilitySystemComp) 3)))

(event Input|ActionEvents|InputActionActiveMixSpellMode
  (params (Key :type Key%20Structure :default "None"))
  (:Pressed
    (Variables|Default|SetMixSpellMode true))
  (:Released
    (Variables|Default|SetMixSpellMode false)
    (Utilities|Array|Clear (Variables|Mixing|GetCurrentComboArray))))

(event Input|ActionEvents|InputActionActiveSkillSlotMovement
  (params (Key :type Key%20Structure :default "None"))
  (:Pressed
    (if (not (Variables|Default|GetBlockSkillUse))
      (Class|AbilitySystemComponent|PressInputID (Variables|Default|GetAbilitySystemComp) 4)))
  (:Released
    (Class|AbilitySystemComponent|ReleaseInputID (Variables|Default|GetAbilitySystemComp) 4)))

(event Input|ActionEvents|InputActionActiveSkillSlotDefence
  (params (Key :type Key%20Structure :default "None"))
  (:Pressed
    (if (not (Variables|Default|GetBlockSkillUse))
      (Class|AbilitySystemComponent|PressInputID (Variables|Default|GetAbilitySystemComp) 5)
      (Default|ActiveSlot#Defence (Variables|Default|GetHudRef))))
  (:Released
    (Class|AbilitySystemComponent|ReleaseInputID (Variables|Default|GetAbilitySystemComp) 5)))

(event Input|ActionEvents|InputActionOpenInventory
  (params (Key :type Key%20Structure :default "None"))
  (bind _hudref (Variables|Default|GetHudRef))
  (bind _w_inventoryicon (Variables|/Game/UI/W_PlayerHud.W_PlayerHud_C|GetW_InventoryIcon _hudref))
  ;[1 1 1] HUD Controll
  (:Pressed
    (Default|ToggleInventoryOpen (Variables|Default|GetInventoryManager))
    (UserInterface|Animation|PlayAnimation _w_inventoryicon (Variables|/Game/UI/W_SetupIcon.W_SetupIcon_C|GetIconPressed _w_inventoryicon) 0.0 1 "Forward" 1.0 false)
    (Variables|Default|SetIsBeingControlled? (not (Variables|Default|GetIsBeingControlled?)))))

(event Input|ActionEvents|InputActionActiveSkillSlotOne
  (params (Key :type Key%20Structure :default "None"))
  ;[1 1 1] AbilitySystem Controll
  (:Pressed
    (if (not (Variables|Default|GetBlockSkillUse))
      (if (not (Variables|Default|GetMixSpellMode))
        (Class|AbilitySystemComponent|PressInputID (Variables|Default|GetAbilitySystemComp) 1)
        (Default|ActiveSlot#1 (Variables|Default|GetHudRef))
        (else
          (CallFunction|ActiveCombo 1)))))
  (:Released
    (Class|AbilitySystemComponent|ReleaseInputID (Variables|Default|GetAbilitySystemComp) 1)))

(event Input|ActionEvents|InputActionActiveQuickBar
  (params (Key :type Key%20Structure :default "None"))
  ;[1 1 1] HUD Controll
  (:Pressed
    (CallFunction|UseInventoryQuickBar)))

(event Input|ActionEvents|InputActionOpenGameplayMenu
  (params (Key :type Key%20Structure :default "None"))
  ;[1 1 1] HUD Controll
  (:Pressed
    (Default|ShowUpGameplayMenu (Variables|Default|GetHudRef) true)))

(event Input|GamepadEvents|GamepadRightX
  (params (AxisValue :type Float%20%28single-precision%29))
  (if true
    (Variables|Default|SetRightThumbstickRotation (Math|Rotator|MakeRotator (.roll (Math|Rotator|MakeRotfromZ (Math|Vector|MakeVector AxisValue (stale Input|GamepadEvents|GamepadRightY AxisValue) 0.0))) (.pitch (Math|Rotator|MakeRotfromZ (Math|Vector|MakeVector AxisValue (stale Input|GamepadEvents|GamepadRightY AxisValue) 0.0))) (- (.yaw (Math|Rotator|MakeRotfromZ (Math|Vector|MakeVector AxisValue (stale Input|GamepadEvents|GamepadRightY AxisValue) 0.0))) -45.0)))))

(event Input|GamepadEvents|GamepadRightY
  (params (AxisValue :type Float%20%28single-precision%29))
  (if true
    (Variables|Default|SetRightThumbstickRotation (Math|Rotator|MakeRotator (.roll (Math|Rotator|MakeRotfromZ (Math|Vector|MakeVector (stale Input|GamepadEvents|GamepadRightX AxisValue) AxisValue 0.0))) (.pitch (Math|Rotator|MakeRotfromZ (Math|Vector|MakeVector (stale Input|GamepadEvents|GamepadRightX AxisValue) AxisValue 0.0))) (- (.yaw (Math|Rotator|MakeRotfromZ (Math|Vector|MakeVector (stale Input|GamepadEvents|GamepadRightX AxisValue) AxisValue 0.0))) -45.0)))))

(event Input|KeyboardEvents|NumPadEight
  (params (Key :type Key%20Structure :default "None"))
  (:Pressed
    (CallFunction|EnableRadgoll)))

(fn ConstructionScript)

(fn ApplyPassiveManaRegenartion
  (Class|BaseCharacter|InitializeAbility "/Game/AbilitySystem/PlayerAbility/ManaRegenerate/GA_ManaRegenerate.GA_ManaRegenerate_C"))

(fn ApplyPlayerHud
  (Utilities|IsValid (Variables|Default|GetHudRef)
    (:Is%20Not%20Valid
      (bind _returnvalue (UserInterface|CreateWidget "/Game/UI/W_PlayerHud.W_PlayerHud_C" (.AsPlayer%20Controller (Utilities|Casting|CastToPlayerController (Pawn|GetController))) self))
      (bind _output_get (Variables|Default|SetHudRef _returnvalue))
      (UserInterface|Viewport|AddtoViewport _output_get 0))))

(fn SetupActiveSkill
  (params (SkillToAdd :type Skill%20Data%20Object%20Reference) (SkillSlot :type E_SkillSlot%20Enum :default "NewEnumerator0"))
  (bind _returnvalue (Math|Conversions|ToInteger(Byte) SkillSlot))
  (bind _activeskills (Variables|Default|GetActiveSkills))
  (Class|AbilitySystemComponent|ClearAllAbilitieswithInputID (Variables|Default|GetAbilitySystemComp) _returnvalue)
  (Class|BaseCharacter|InitializeAbility (Variables|/Game/AbilitySystem/DataTable/SkillData.SkillData_C|GetAbilityClass SkillToAdd) 0 _returnvalue)
  (Default|SetupActiveSkillIcone (Variables|Default|GetHudRef) SkillSlot (Variables|/Game/AbilitySystem/DataTable/SkillData.SkillData_C|GetTexture SkillToAdd))
  (Utilities|Map|Remove _activeskills SkillSlot)
  (Utilities|Map|Add _activeskills SkillSlot SkillToAdd))

(fn ActiveSkillfromCombination
  (switch Utilities|FlowControl|Switch|SwitchonE_RuneType (Utilities|Array|Get(acopy) (Variables|Mixing|GetCurrentComboArray))
    (:NewEnumerator3
      (Abilities|TryActivateAbilitybyClass (Variables|Default|GetAbilitySystemComp) "/Game/AbilitySystem/PlayerAbility/FireLaser/GA_FireLaser.GA_FireLaser_C" true))
    (:NewEnumerator0
      (Abilities|TryActivateAbilitybyClass (Variables|Default|GetAbilitySystemComp) "/Game/AbilitySystem/PlayerAbility/FireWave/GA_FireWave.GA_FireWave_C" true))))

(fn SetupRunes)

(fn SetupAbilites
  (CallFunction|SetupStartingAbility)
  (CallFunction|ApplyPassiveManaRegenartion)
  (CallFunction|IniteComboAbility (Variables|Default|GetComboAbilities)))

(fn SetControlRotation
  (bind _playercontrolerref (Variables|Default|GetPlayerControlerRef))
  (if (Variables|/Game/Blueprint/Core/BP_CustomPlayerControler.BP_CustomPlayerControler_C|GetIsGamepadUse (Variables|Default|GetPlayerControlerRef))
    (Pawn|SetControlRotation _playercontrolerref (Variables|Default|GetRightThumbstickRotation))
    (else
      (Pawn|SetControlRotation _playercontrolerref (Math|Rotator|FindLookatRotation (Transformation|GetWorldLocation (Variables|Default|GetCapsuleComponent)) (.location (.HitResult (Class|PlayerController|GetHitResultUnderCursorforObjects (Variables|Default|GetPlayerControlerRef) (Utilities|Array|MakeArray "ObjectTypeQuery1" "ObjectTypeQuery2") true))))))))

(fn EnableRotationtoMousePosition
  (params (Condition :type Boolean) (AutoTurnOff :type Boolean) (AutoTurnOffDelay :type Float%20%28double-precision%29))
  (if Condition
    (Variables|/Script/Engine.CharacterMovementComponent|SetbOrientRotationToMovement (Variables|Character|GetCharacterMovement) false)
    (bind _returnvalue (Utilities|Time|SetTimerbyEvent (EventDispatchers|CreateEvent :!event SetControlRotation) 0.01 true))
    (Variables|Default|SetSetControlRotationLoop _returnvalue)
    (if AutoTurnOff
      (bind _returnvalue_2 (Utilities|Time|SetTimerbyEvent (EventDispatchers|CreateEvent :!event DisableRotationfromAutoTurnOFF) AutoTurnOffDelay))
      (Variables|Default|SetEnableRotationTurnOff _returnvalue_2))
    (else
      (Variables|/Script/Engine.CharacterMovementComponent|SetbOrientRotationToMovement (Variables|Character|GetCharacterMovement) true)
      (Utilities|Time|ClearandInvalidateTimerbyHandle (Variables|Default|GetSetControlRotationLoop)))))

(fn SetupStartingAbility
  (bind _keys (Utilities|Map|Keys (Variables|Default|GetActiveSkills)))
  (for _array_element _keys
    (if (.ReturnValue (Utilities|Map|Find (Variables|Default|GetActiveSkills) _array_element))
      (CallFunction|SetupActiveSkill (.Value (Utilities|Map|Find (Variables|Default|GetActiveSkills) _array_element)) _array_element))))

(fn IniteComboAbility
  (params (RuneAbilities :type Array%20of%20Skill%20Data%20Object%20References))
  (for (_array_element _array_index) RuneAbilities
    (Class|BaseCharacter|InitializeAbility (Variables|/Game/AbilitySystem/DataTable/SkillData.SkillData_C|GetAbilityClass _array_element) 0 (+ _array_index 10))))

(fn SetVariables
  (bind _inventorymanagercomponent (CallFunction|GetInventoryManager self))
  (Variables|Default|SetInventoryManager _inventorymanagercomponent)
  (bind _asbp_custom_player_controler (Utilities|Casting|CastToBP_CustomPlayerControler (Pawn|GetController)))
  (Variables|Default|SetPlayerControlerRef _asbp_custom_player_controler)
  (bind _asbp_mage_player_state (Utilities|Casting|CastToBP_MagePlayerState (Variables|Default|GetPlayerState)))
  (Variables|Default|SetPlayerStateMage _asbp_mage_player_state))

(fn DisableRotationfromAutoTurnOFF
  (CallFunction|EnableRotationtoMousePosition false false 0.0))

(fn SynctoElement(
  (params (New%20Element :type E_Elements%20Enum :default "NewEnumerator0")))

(fn SetupRunHud
  (Variables|/Game/UI/W_RuneHud.W_RuneHud_C|SetRuneType (Variables|/Game/UI/W_PlayerRunesHud.W_PlayerRunesHud_C|GetW_AbilitySlot1 (Variables|/Game/UI/W_PlayerHud.W_PlayerHud_C|GetW_PlayerRuneHud (Variables|Default|GetHudRef))) (Variables|Mixing|GetRuneSlot_1))
  (Variables|/Game/UI/W_RuneHud.W_RuneHud_C|SetRuneType (Variables|/Game/UI/W_PlayerRunesHud.W_PlayerRunesHud_C|GetW_AbilitySlot2 (Variables|/Game/UI/W_PlayerHud.W_PlayerHud_C|GetW_PlayerRuneHud (Variables|Default|GetHudRef))) (Variables|Mixing|GetRuneSlot_2))
  (Variables|/Game/UI/W_RuneHud.W_RuneHud_C|SetRuneType (Variables|/Game/UI/W_PlayerRunesHud.W_PlayerRunesHud_C|GetW_AbilitySlot3 (Variables|/Game/UI/W_PlayerHud.W_PlayerHud_C|GetW_PlayerRuneHud (Variables|Default|GetHudRef))) (Variables|Mixing|GetRuneSlot_3)))

(fn UseInventoryQuickBar
  (Default|UseQuickSlotItem (Variables|Default|GetInventoryManager) (Variables|Default|GetQuickBarItem) self))

(fn GetQuickBarNumber
  (bind _amount (Default|GetItemAmount (Variables|Default|GetInventoryManager) (Variables|Default|GetQuickBarItem)))
  (return _amount))

(fn DisplayMapWidget
  (params (MapName :type Text))
  (Utilities|IsValid (Variables|Default|GetHudRef)
    (:Is%20Valid
      _)
    (:Is%20Not%20Valid
      (CallFunction|ApplyPlayerHud)))
  (Default|PlayLocationPopUp (Variables|Default|GetHudRef) MapName))

(fn CheckCurrentIndex
  (params (IndexToCheck :type Integer))
  (for _array_element (Variables|Default|GetComboAbilities)
    (if (Utilities|Enum|Equal(Enum) (Utilities|Array|Get(acopy) (Variables|/Game/AbilitySystem/DataTable/SkillData.SkillData_C|GetComboArray _array_element) IndexToCheck) (Utilities|Array|Get(acopy) (Variables|Mixing|GetCurrentComboArray) IndexToCheck))
      (LocalVariables|SetCorrectIndexFounded true)
      (LocalVariables|SetCorrectSkillData _array_element)))
  (return (LocalVariables|GetCorrectIndexFounded) (LocalVariables|GetCorrectSkillData)))

(fn ComponentstoSave
  (return (Utilities|Array|MakeArray (Variables|Default|GetAbilitySystemComp))))