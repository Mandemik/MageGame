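; Arena game mode that handles level completion, saved enemy deaths and debug cheats.
; On completion it keeps the best star count per level in BP_MagePlayerState, shows a HUD popup, then switches to MageMap through the game instance.
; When the actor loads from a save, it destroys pawns recorded as killed on the current level.
; Cheat events cover immortality via GameplayEffect, speed, ability unlocks, killing all humanoid AI and finishing levels.
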(event Custom|GameplayLevelCompleted
  (params (Stars :type Integer))
  (CallFunction|AddLevelStars (Variables|/Game/Blueprint/Core/BP_GameInstance.BP_GameInstance_C|GetLastGameplayLevel (.AsBP%20Game%20Instance (Utilities|Casting|CastToBP_GameInstance (Game|GetGameInstance)))) Stars)
  (Default|PlayLocationPopUp (Variables|/Game/Blueprint/Core/BP_PlayerArenaCharacter.BP_PlayerArenaCharacter_C|GetHudRef (Variables|Default|GetPlayerRef)) "Level Completed!")
  (Utilities|FlowControl|Delay 2.0)
  (Default|SwitchMap (.AsBP%20Game%20Instance (Utilities|Casting|CastToBP_GameInstance (Game|GetGameInstance))) "MageMap"))

(event EventActorLoaded
  (CallFunction|DestroySavedEnemysonCurrentLevel))

(event EventBeginPlay
  (bind _asbp_player_arena_character (Utilities|Casting|CastToBP_PlayerArenaCharacter (Game|GetPlayerCharacter 0))
    (:then
      (Variables|Default|SetPlayerRef _asbp_player_arena_character))
    (:CastFailed
      (Development|PrintString "GAME MODE CAN FIND PLAYER CLASS!!" true true "(R=1.000000,G=0.051568,B=0.000000,A=1.000000)"))))

(event EventBlueprintCheatUnlockAbility
  (params (enable :type Boolean))
  (bind _playerref (Variables|Default|GetPlayerRef))
  (if enable
    (Default|SetupRunes _playerref)
    (Default|SetupActiveSkill _playerref "/Game/AbilitySystem/DataTable/SkillDataAsset/Dash_SkillData.Dash_SkillData" "NewEnumerator2")))

(event EventBlueprintCheatImmortality
  (params (enable :type Boolean))
  (if enable
    (bind _returnvalue (GameplayEffects|ApplyGameplayEffectToSelf :self (Variables|/Script/MagBuildGame.BaseCharacter|GetAbilitySystemComp (Variables|Default|GetPlayerRef)) :GameplayEffectClass "/Game/AbilitySystem/Status/Blocks/GE_BlockDamageAll.GE_BlockDamageAll_C"))
    (Variables|Default|SetCheatBlockDamageAll _returnvalue)
    (else
      (GameplayEffects|RemoveActiveGameplayEffect (Variables|/Script/MagBuildGame.BaseCharacter|GetAbilitySystemComp (Variables|Default|GetPlayerRef)) (Variables|Default|GetCheatBlockDamageAll) -1))))

(event EventBlueprintCheatKillAllAi
  (params (enable :type Boolean))
  (bind _returnvalue (Game|GetPlayerController 0))
  (if enable
    (bind _outactors (Actor|GetAllActorsOfClass "/Game/Blueprint/AI/BP_AI_Humanoid.BP_AI_Humanoid_C"))
    (for _array_element _outactors
      (Game|Damage|ApplyDamage _array_element 9999999.0 _returnvalue _returnvalue "/Game/Blueprint/Core/DT_MagDamageType.DT_MagDamageType_C"))))

(event EventBlueprintCheatFinishLevelwithStars
  (params (Starsnumber :type Integer))
  (CallFunction|GameplayLevelCompleted Starsnumber))

(event EventBlueprintCheatSuperSpeed
  (params (enable :type Boolean))
  (bind _playerref (Variables|Default|GetPlayerRef))
  (bind _charactermovement (Variables|/Script/Engine.Character|GetCharacterMovement _playerref))
  (if enable
    (Variables|/Script/Engine.CharacterMovementComponent|SetMaxWalkSpeed _charactermovement 2e+03)
    (else
      (Variables|/Script/Engine.CharacterMovementComponent|SetMaxWalkSpeed _charactermovement 475.0))))

(fn ConstructionScript)

(fn DestroySavedEnemysonCurrentLevel
  (bind _returnvalue (Game|GetCurrentLevelName true))
  (LocalVariables|SetCurrentLevelName _returnvalue)
  (bind _keys (Utilities|Map|Keys (Variables|Default|GetDestoyedAiPawns)))
  (for _array_element _keys
    (Utilities|IsValid _array_element
      (:Is%20Valid
        (if (and (.ReturnValue (Utilities|Map|Find (Variables|Default|GetDestoyedAiPawns) _array_element)) (Utilities|Enum|Equal(Enum) (LocalVariables|GetCurrentLevelName) (.Value (Utilities|Map|Find (Variables|Default|GetDestoyedAiPawns) _array_element))))
          (Actor|DestroyActor _array_element))))))

(fn AddLevelStars
  (params (LevelName :type Name) (Stars :type Integer))
  (bind _asbp_mage_player_state (Utilities|Casting|CastToBP_MagePlayerState (Variables|/Script/Engine.Pawn|GetPlayerState (Game|GetPlayerCharacter 0))))
  (if (.ReturnValue (Utilities|Map|Find (Variables|/Game/Blueprint/Core/BP_MagePlayerState.BP_MagePlayerState_C|GetStarLevelMap _asbp_mage_player_state) LevelName))
    (if (> Stars (.Value (Utilities|Map|Find (Variables|/Game/Blueprint/Core/BP_MagePlayerState.BP_MagePlayerState_C|GetStarLevelMap _asbp_mage_player_state) LevelName)))
      (Utilities|Map|Remove (Variables|/Game/Blueprint/Core/BP_MagePlayerState.BP_MagePlayerState_C|GetStarLevelMap _asbp_mage_player_state) LevelName)
      (Utilities|Map|Add (Variables|/Game/Blueprint/Core/BP_MagePlayerState.BP_MagePlayerState_C|GetStarLevelMap _asbp_mage_player_state) LevelName Stars :!label _label))
    (else
      (goto _label))))

(fn ComponentstoSave
  (return 0))