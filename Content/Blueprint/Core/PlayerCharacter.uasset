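; Player character Blueprint that sets up the player's HUD, mouse cursor and Gameplay Ability System abilities when play begins.
; BeginPlay shows the cursor, creates the HUD widget with a reference back to the character, and initializes a fireball ability.
; It then initializes the mana regeneration ability and activates it immediately by class, so regeneration runs as a passive.
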(event EventBeginPlay
  (Variables|/Script/Engine.PlayerController|SetbShowMouseCursor (.AsPlayer%20Controller (Utilities|Casting|CastToPlayerController (Pawn|GetController))) true)
  (CallFunction|ApplyPlayerHud)
  (Class|BaseCharacter|InitializeAbility "/Game/AbilitySystem/Ability/Fireball/GA_FireBall.GA_FireBall_C")
  (CallFunction|ApplyPassiveManaRegenartion))

(fn ConstructionScript)

(fn ApplyPassiveManaRegenartion
  (Class|BaseCharacter|InitializeAbility "/Game/AbilitySystem/Ability/ManaRegenerate/GA_ManaRegenerate.GA_ManaRegenerate_C")
  (Abilities|TryActivateAbilitybyClass (Variables|Default|GetAbilitySystemComp) "/Game/AbilitySystem/Ability/ManaRegenerate/GA_ManaRegenerate.GA_ManaRegenerate_C" true))

(fn ApplyPlayerHud
  (bind _returnvalue (UserInterface|CreateWidget "/Game/UI/W_PlayerHud.W_PlayerHud_C" (.AsPlayer%20Controller (Utilities|Casting|CastToPlayerController (Pawn|GetController))) self))
  (bind _output_get (Variables|Default|SetHudRef _returnvalue))
  (UserInterface|Viewport|AddtoViewport _output_get 0))