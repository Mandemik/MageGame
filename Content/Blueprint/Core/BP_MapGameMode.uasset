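; Map game mode for the arena game that handles level progression, saved world state and player cheats.
; On login it has every BP_MasterGrid load saved grids for the joining player; on load it destroys AI pawns recorded as killed in the current level.
; NextLevelPlease streams through numbered arena sublevels, moving player 0 to a player start under a HUD fade.
; Cheats toggle immortality via a GameplayEffect and speed, or unlock runes and Dash.
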(event Custom|NextLevelPlease
  (bind _returnvalue (Game|GetPlayerCharacter 0))
  (bind _levelnumber (Variables|Default|GetLevelNumber))
  (bind _asbp_player_arena_character (Utilities|Casting|CastToBP_PlayerArenaCharacter _returnvalue))
  (bind _returnvalue_2 (Utilities|Select :Index _levelnumber :Option%200 "Arena_Gameplay_ZombieMarch" :Option%201 "Arena_Gameplay_ZombieSpawn" :Option%202 "Arena_Gameplay_GoblinMeet" :Option%203 ""))
  (bind _hudref (Variables|/Game/Blueprint/Core/BP_PlayerArenaCharacter.BP_PlayerArenaCharacter_C|GetHudRef _asbp_player_arena_character))
  (Utilities|FlowControl|Sequence
    (:then_0
      (Utilities|FlowControl|Delay 3.0)
      (Math|Integer|IncrementInt (Variables|Default|GetLevelNumber)
        (:%20%20
          (if (not (== (Variables|Default|GetLastSubLevelName) ""))
            (Game|UnloadStreamLevel(byName) (Variables|Default|GetLastSubLevelName) false))
          (Variables|Default|SetLastSubLevelName _returnvalue_2)
          (Game|LoadStreamLevel(byName) _returnvalue_2 true true)
          (Transformation|SetActorLocation (Game|GetPlayerCharacter 0) (Transformation|GetActorLocation (Class|GameModeBase|FindPlayerStart (Game|GetPlayerController 0))) false false))))
    (:then_1
      (Utilities|FlowControl|Delay 2.85)
      (UserInterface|Animation|PlayAnimation _hudref (Variables|/Game/UI/W_PlayerHud.W_PlayerHud_C|GetQuickFade _hudref) 0.0 1 "Forward" 1.0 false))))

(event EventPostLogin
  (params (NewPlayer :type Player%20Controller%20Object%20Reference))
  ;[1 1 1] On login to the server, load past created grids
  (Utilities|FlowControl|Delay 2.0)
  (bind _outactors (Actor|GetAllActorsOfClass "/Game/PlayerBuildingSystem/Blueprints/BuildingBlueprints/BuildGrids/BP_MasterGrid.BP_MasterGrid_C"))
  (if (> (Utilities|Array|Length _outactors) 0)
    (for _array_element _outactors
      (Default|ServerLoadGridsonJoin _array_element NewPlayer))))

(event EventActorLoaded
  (CallFunction|DestroySavedEnemysonCurrentLevel))

(event EventBlueprintCheatUnlockAbility
  (params (enable :type Boolean))
  (if enable
    (bind _asbp_player_arena_character (Utilities|Casting|CastToBP_PlayerArenaCharacter (Game|GetPlayerCharacter 0)))
    (Default|SetupRunes _asbp_player_arena_character)
    (Default|SetupActiveSkill _asbp_player_arena_character "/Game/AbilitySystem/DataTable/SkillDataAsset/Dash_SkillData.Dash_SkillData" "NewEnumerator2")))

(event EventBlueprintCheatImmortality
  (params (enable :type Boolean))
  (if enable
    (bind _asbp_player_arena_character (Utilities|Casting|CastToBP_PlayerArenaCharacter (Game|GetPlayerCharacter 0)))
    (bind _returnvalue (GameplayEffects|ApplyGameplayEffectToSelf :self (Variables|/Script/MagBuildGame.BaseCharacter|GetAbilitySystemComp _asbp_player_arena_character) :GameplayEffectClass "/Game/AbilitySystem/Status/Blocks/GE_BlockDamageAll.GE_BlockDamageAll_C"))
    (Variables|Default|SetCheatBlockDamageAll _returnvalue)
    (else
      (bind _asbp_player_arena_character_2 (Utilities|Casting|CastToBP_PlayerArenaCharacter (Game|GetPlayerCharacter 0)))
      (GameplayEffects|RemoveActiveGameplayEffect (Variables|/Script/MagBuildGame.BaseCharacter|GetAbilitySystemComp _asbp_player_arena_character_2) (Variables|Default|GetCheatBlockDamageAll) -1))))

(event EventBlueprintCheatSuperSpeed
  (params (enable :type Boolean))
  (if enable
    (bind _asbp_player_arena_character (Utilities|Casting|CastToBP_PlayerArenaCharacter (Game|GetPlayerCharacter 0)))
    (Variables|/Script/Engine.CharacterMovementComponent|SetMaxWalkSpeed (Variables|/Script/Engine.Character|GetCharacterMovement _asbp_player_arena_character) 2e+03)
    (else
      (bind _asbp_player_arena_character_2 (Utilities|Casting|CastToBP_PlayerArenaCharacter (Game|GetPlayerCharacter 0)))
      (Variables|/Script/Engine.CharacterMovementComponent|SetMaxWalkSpeed (Variables|/Script/Engine.Character|GetCharacterMovement _asbp_player_arena_character_2) 475.0))))

(fn ConstructionScript)

(fn DestroySavedEnemysonCurrentLevel
  (bind _returnvalue (Game|GetCurrentLevelName true))
  (LocalVariables|SetCurrentLevelName _returnvalue)
  (bind _keys (Utilities|Map|Keys (Variables|Default|GetDestoyedAiPawns)))
  (for _array_element _keys
    (Utilities|IsValid _array_element
      (:Is%20Valid
        (if (and (.ReturnValue (Utilities|Map|Find (Variables|Default|GetDestoyedAiPawns) _array_element)) (Utilities|Enum|Equal(Enum) (LocalVariables|GetCurrentLevelName) (.Value (Utilities|Map|Find (Variables|Default|GetDestoyedAiPawns) _array_element))))
          (Actor|DestroyActor _array_element))))))

(fn ComponentstoSave
  (return 0))