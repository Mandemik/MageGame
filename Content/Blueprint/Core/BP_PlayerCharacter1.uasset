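; BP_PlayerCharacter1 is a player character Blueprint that handles camera boom moves and object interaction.
; Timelines lerp the boom's rotation toward the camera component's target, or its location to a custom point and back above the actor, disabling collision testing.
; An interface-style event records the current interactable, which InteractionToggle messages unless an open chest needs toggling first.
; Zoom events are empty; the zoom timeline and collision re-enable logic are disconnected.
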(event Custom|StartCameraMove
  (Variables|Default|SetStartingCameraRotation (Variables|/Script/Engine.SceneComponent|GetRelativeRotation (Variables|Default|GetCameraBoom)))
  (bind _time (Timeline|Timeline_0 PlayFromStart)
    (:Update
      (Transformation|SetRelativeRotation (Variables|Default|GetCameraBoom) (Math|Rotator|Lerp(Rotator) (Variables|Default|GetStartingCameraRotation) (Variables|/Game/Blueprint/Player/Components/BP_CameraComponent.BP_CameraComponent_C|GetFinalRotation (Variables|Default|GetBP_CameraComponent)) _time true) false false))))

(event Custom|EndCameraZoom)

(event Custom|StartCameraZoom
  (params (ZoomValue :type Float%20%28double-precision%29)))

(event Custom|MoveCameraToCustomLocation
  (params (Location :type Vector) (Enable :type Boolean))
  (bind _returnvalue (Transformation|GetActorLocation))
  (if Enable
    (Variables|Default|SetCustomCameraLocation Location)
    (Variables|/Script/Engine.SpringArmComponent|SetbDoCollisionTest (Variables|Default|GetCameraBoom) false)
    (Variables|Default|SetCustomStarCameraLocation (Transformation|GetWorldLocation (Variables|Default|GetCameraBoom)))
    (bind (_direction _time) (Timeline|Timeline_2 PlayFromStart)
      (:Update
        (Transformation|SetWorldLocation (Variables|Default|GetCameraBoom) (Math|Vector|Lerp(Vector) (Utilities|Select :Index _direction :Forward (Variables|Default|GetCustomStarCameraLocation) :Backward (Math|Vector|MakeVector (.x _returnvalue) (.y _returnvalue) (+ (.z _returnvalue) 45.0))) (Variables|Default|GetCustomCameraLocation) _time) false false))
      (:Finished
        (switch Utilities|FlowControl|Switch|SwitchonETimelineDirection _direction)))
    (else
      (Timeline|Timeline_2 ReverseFromEnd))))

(event EventCanInteractwithMe
  (params (CanInteract? :type Boolean) (ActorToInteract :type Actor%20Object%20Reference))
  (Variables|InteractSystem|SetCan%20Interact? CanInteract?)
  (Variables|InteractSystem|SetActor%20to%20Interact ActorToInteract)
  (Default|CallInteractionChange))

(fn ConstructionScript
  (|CallParentFunction))

(fn InteractionToggle
  (Utilities|IsValid (Variables|InteractSystem|GetCurrentlyOpenChest)
    (:Is%20Valid
      (Default|ToggleChest (Variables|InteractSystem|GetCurrentlyOpenChest))
      (Variables|InteractSystem|SetCurrentlyOpenChest 0))
    (:Is%20Not%20Valid
      (if (Variables|InteractSystem|GetCan%20Interact?)
        (Class|BPInteractionInterface|InteractwithObject(Message) (Variables|InteractSystem|GetActor%20to%20Interact) self)))))