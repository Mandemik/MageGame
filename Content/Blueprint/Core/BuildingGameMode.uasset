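; Game mode for the building game that syncs previously built grids to joining players and hosts save and cheat events.
; Two seconds after login, it asks every BP_MasterGrid to load its grids for the new player.
; Cheat events save, load, delete or restart through async actor saving, and toggle player 0's damage immunity via a GAS effect or super speed via walk speed.
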(event EventPostLogin
  (params (NewPlayer :type Player%20Controller%20Object%20Reference))
  ;[1 1 1] On login to the server, load past created grids
  (Utilities|FlowControl|Delay 2.0)
  (bind _outactors (Actor|GetAllActorsOfClass "/Game/PlayerBuildingSystem/Blueprints/BuildingBlueprints/BuildGrids/BP_MasterGrid.BP_MasterGrid_C"))
  (if (> (Utilities|Array|Length _outactors) 0)
    (for _array_element _outactors
      (Default|ServerLoadGridsonJoin _array_element NewPlayer))))

(event Custom|NewGame
  (CallFunction|DeleteSave)
  (bind _returnvalue (Game|GetCurrentLevelName true))
  (Game|OpenLevel(byName) (Utilities|String|StringToName _returnvalue)))

(event Custom|SaveGame
  (|AsyncSaveActors 3
    (:OnCompleted
      (Development|PrintString "Saving"))))

(event Custom|DeleteSave
  (Class|EMSFunctionLibrary|DeleteAllSaveDataforSlot (.SaveGameName (Class|EMSFunctionLibrary|GetSlotInfoSaveGame)))
  (Development|PrintString (Utilities|String|Append "Deleting slot = " "")))

(event Custom|LoadGame
  (|AsyncLoadActors 3 true
    (:OnCompleted
      (Development|PrintString "Loaded Success"))
    (:OnFailed
      (Development|PrintString "Loaded Failed"))))

(event EventBlueprintCheatImmortality
  (params (enable :type Boolean))
  (if enable
    (bind _asbp_player_character (Utilities|Casting|CastToBP_PlayerCharacter (Game|GetPlayerCharacter 0)))
    (bind _returnvalue (GameplayEffects|ApplyGameplayEffectToSelf :self (Variables|/Script/MagBuildGame.BaseCharacter|GetAbilitySystemComp _asbp_player_character) :GameplayEffectClass "/Game/AbilitySystem/Status/Blocks/GE_BlockDamageAll.GE_BlockDamageAll_C"))
    (Variables|Default|SetCheatBlockDamageAll _returnvalue)
    (else
      (bind _asbp_player_character_2 (Utilities|Casting|CastToBP_PlayerCharacter (Game|GetPlayerCharacter 0)))
      (GameplayEffects|RemoveActiveGameplayEffect (Variables|/Script/MagBuildGame.BaseCharacter|GetAbilitySystemComp _asbp_player_character_2) (Variables|Default|GetCheatBlockDamageAll) -1))))

(event EventBlueprintCheatSuperSpeed
  (params (enable :type Boolean))
  (if enable
    (bind _asbp_player_character (Utilities|Casting|CastToBP_PlayerCharacter (Game|GetPlayerCharacter 0)))
    (Variables|/Script/Engine.CharacterMovementComponent|SetMaxWalkSpeed (Variables|/Script/Engine.Character|GetCharacterMovement _asbp_player_character) 2e+03)
    (else
      (bind _asbp_player_character_2 (Utilities|Casting|CastToBP_PlayerCharacter (Game|GetPlayerCharacter 0)))
      (Variables|/Script/Engine.CharacterMovementComponent|SetMaxWalkSpeed (Variables|/Script/Engine.Character|GetCharacterMovement _asbp_player_character_2) 475.0))))

(fn ConstructionScript)

(fn ReadytoEndMatch
  (return false))

(fn ComponentstoSave
  (return 0))