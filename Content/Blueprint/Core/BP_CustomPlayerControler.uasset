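; Player controller that caches the possessed BP_PlayerCharacter on BeginPlay and routes input to its camera, inventory, ability and building components.
; Movement follows the camera boom's yaw, and Q/E run looping timers for stepped camera rotation.
; R and T activate Fireball and Magic Barrier through GAS; Q and T are also bound to building options and a damage test.
; Turn and LookUp axes nudge the mouse cursor each Tick.
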(event Custom|StartRotateCameraToLeft
  (Default|RotateCameratoLeft (Variables|/Game/Blueprint/Core/BP_PlayerCharacter.BP_PlayerCharacter_C|GetBP_CameraComponent (Variables|Default|GetControlledCharacter))))

(event Custom|StartRotateCameraToRight
  (Default|RotateCameratoRight (Variables|/Game/Blueprint/Core/BP_PlayerCharacter.BP_PlayerCharacter_C|GetBP_CameraComponent (Variables|Default|GetControlledCharacter))))

(event EventBeginPlay
  (bind _asbp_player_character (Utilities|Casting|CastToBP_PlayerCharacter (Pawn|GetControlledPawn))
    (:then
      (Variables|Default|SetControlledCharacter _asbp_player_character))
    (:CastFailed
      (Development|PrintString "ERROR : Wrrong character is selected on Player Controler." true true "(R=1.000000,G=0.000000,B=0.034709,A=1.000000)"))))

(event EventTick
  (params (DeltaSeconds :type Float%20%28single-precision%29))
  (bind (_locationx _locationy) (Game|Player|GetMousePosition))
  (if (or (!= (Variables|Default|GetControlerX) 0.0) (!= (Variables|Default|GetControlerY) 0.0))
    (Class|PlayerController|SetMouseLocation (Math|Float|Truncate (+ _locationx (Variables|Default|GetControlerX))) (Math|Float|Truncate (+ _locationy (Variables|Default|GetControlerY))))))

(event Input|ActionEvents|InputActionOpenBuildMenu
  (params (Key :type Key%20Structure :default "None"))
  (bind _controlledcharacter (Variables|Default|GetControlledCharacter))
  (bind _playerbuildingcomponent (Variables|/Game/Blueprint/Core/BP_PlayerCharacter.BP_PlayerCharacter_C|GetPlayerBuildingComponent _controlledcharacter))
  ;[1 1 1] Toggle building menu
  (:Pressed
    (Default|ToggleBuildMenu _playerbuildingcomponent (not (Variables|/Game/PlayerBuildingSystem/Blueprints/Components/PlayerBuildingComponent.PlayerBuildingComponent_C|GetBuildMenuOpen _playerbuildingcomponent)))))

(event Input|ActionEvents|InputActionSelectBuildForMenu
  (params (Key :type Key%20Structure :default "None"))
  (bind _controlledcharacter (Variables|Default|GetControlledCharacter))
  (bind _playerbuildingcomponent (Variables|/Game/Blueprint/Core/BP_PlayerCharacter.BP_PlayerCharacter_C|GetPlayerBuildingComponent _controlledcharacter))
  ;[1 1 1] Left mouse button input
  (:Pressed
    (Default|SelectBuildingtoBuild _playerbuildingcomponent))
  (:Released
    (Default|LeftMouseReleased _playerbuildingcomponent)))

(event Input|ActionEvents|InputActionInteract
  (params (Key :type Key%20Structure :default "None"))
  (bind _controlledcharacter (Variables|Default|GetControlledCharacter))
  (bind _playerbuildingcomponent (Variables|/Game/Blueprint/Core/BP_PlayerCharacter.BP_PlayerCharacter_C|GetPlayerBuildingComponent _controlledcharacter))
  ;[1 1 1] Interact input
  (:Pressed
    (Default|ClientInteract _playerbuildingcomponent true))
  (:Released
    (Default|ClientInteract _playerbuildingcomponent false)))

(event Input|ActionEvents|InputActionCancelAction
  (params (Key :type Key%20Structure :default "None"))
  (:Pressed
    (Default|SelectBuildType (Variables|/Game/Blueprint/Core/BP_PlayerCharacter.BP_PlayerCharacter_C|GetPlayerBuildingComponent (Variables|Default|GetControlledCharacter)) (Utilities|Struct|MakeDataTableRowHandle "/Game/PlayerBuildingSystem/Blueprints/BuildingBlueprints/BuildTypes/BuildPartData.BuildPartData" "empty"))))

(event Input|ActionEvents|InputActionOpenInventory
  (params (Key :type Key%20Structure :default "None"))
  (bind _controlledcharacter (Variables|Default|GetControlledCharacter))
  (:Pressed
    (Default|ToggleInventoryOpen (Variables|/Game/Blueprint/Core/BP_PlayerCharacter.BP_PlayerCharacter_C|GetInventoryManager (Variables|Default|GetControlledCharacter)))
    (Variables|/Game/Blueprint/Core/BP_PlayerCharacter.BP_PlayerCharacter_C|SetIsBeingControlled? _controlledcharacter (not (Variables|/Game/Blueprint/Core/BP_PlayerCharacter.BP_PlayerCharacter_C|GetIsBeingControlled? _controlledcharacter)))))

(event Input|ActionEvents|InputActionRotateMesh
  (params (Key :type Key%20Structure :default "None"))
  ;[1 1 1] Rotate mesh
  (:Pressed
    (Default|RotateMesh (Variables|/Game/Blueprint/Core/BP_PlayerCharacter.BP_PlayerCharacter_C|GetPlayerBuildingComponent (Variables|Default|GetControlledCharacter)))))

(event Input|AxisEvents|InputAxisLookUp
  (params (AxisValue :type Float%20%28single-precision%29))
  (if (!= AxisValue 0.0)
    (Variables|Default|SetControlerY (* AxisValue 1e+01))
    (else
      (Variables|Default|SetControlerY 0.0))))

(event Input|AxisEvents|InputAxisTurn
  (params (AxisValue :type Float%20%28single-precision%29))
  (if (!= AxisValue 0.0)
    (Variables|Default|SetControlerX (* AxisValue 1e+01))
    (else
      (Variables|Default|SetControlerX 0.0))))

(event Input|AxisEvents|InputAxisMoveForward
  (params (AxisValue :type Float%20%28single-precision%29))
  (Pawn|Input|AddMovementInput (Variables|Default|GetControlledCharacter) (Math|Vector|GetForwardVector (Math|Rotator|MakeRotator 0.0 0.0 (.Yaw (Math|Rotator|BreakRotator (Variables|/Script/Engine.SceneComponent|GetRelativeRotation (Variables|/Game/Blueprint/Core/BP_PlayerCharacter.BP_PlayerCharacter_C|GetCameraBoom (Variables|Default|GetControlledCharacter))))))) AxisValue false))

(event Input|AxisEvents|InputAxisMoveRight
  (params (AxisValue :type Float%20%28single-precision%29))
  (Pawn|Input|AddMovementInput (Variables|Default|GetControlledCharacter) (Math|Vector|GetRightVector (Math|Rotator|MakeRotator 0.0 0.0 (.Yaw (Math|Rotator|BreakRotator (Variables|/Script/Engine.SceneComponent|GetRelativeRotation (Variables|/Game/Blueprint/Core/BP_PlayerCharacter.BP_PlayerCharacter_C|GetCameraBoom (Variables|Default|GetControlledCharacter))))))) AxisValue false))

(event Input|KeyboardEvents|R
  (params (Key :type Key%20Structure :default "None"))
  (:Pressed
    (Abilities|TryActivateAbilitybyClass (Ability|GetAbilitySystemComponent (Variables|Default|GetControlledCharacter)) "/Game/Prezentacja/5_GameplayAbility/GA_FireBall.GA_FireBall_C" true)))

(event Input|KeyboardEvents|Q
  (params (Key :type Key%20Structure :default "None"))
  (:Pressed
    (bind _returnvalue (Utilities|Time|SetTimerbyEvent (EventDispatchers|CreateEvent :!event Custom|StartRotateCameraToLeft) 0.1 true))
    (Variables|Default|SetRotataeLeftTimer _returnvalue))
  (:Released
    (Utilities|Time|ClearandInvalidateTimerbyHandle (Variables|Default|GetRotataeLeftTimer))))

(event Input|KeyboardEvents|T
  (params (Key :type Key%20Structure :default "None"))
  ;[1 1 1] Damage Demo
  (:Pressed
    (Default|ClientDamageTest (Variables|/Game/Blueprint/Core/BP_PlayerCharacter.BP_PlayerCharacter_C|GetPlayerBuildingComponent (Variables|Default|GetControlledCharacter)))))

(event Input|KeyboardEvents|E
  (params (Key :type Key%20Structure :default "None"))
  (:Pressed
    (bind _returnvalue (Utilities|Time|SetTimerbyEvent (EventDispatchers|CreateEvent :!event Custom|StartRotateCameraToRight) 0.1 true))
    (Variables|Default|SetRotateRightTimer _returnvalue))
  (:Released
    (Utilities|Time|ClearandInvalidateTimerbyHandle (Variables|Default|GetRotateRightTimer))))

(event Input|KeyboardEvents|T
  (params (Key :type Key%20Structure :default "None"))
  (:Pressed
    (Abilities|TryActivateAbilitybyClass (Ability|GetAbilitySystemComponent (Variables|Default|GetControlledCharacter)) "/Game/AbilitySystem/PlayerAbility/MagicBarrier/GA_MagicBarrier.GA_MagicBarrier_C" true)
    (Default|CallPlayerWannaUseDefenciveAbility true))
  (:Released
    (Default|CallPlayerWannaUseDefenciveAbility false)))

(event Input|KeyboardEvents|Q
  (params (Key :type Key%20Structure :default "None"))
  (bind _controlledcharacter (Variables|Default|GetControlledCharacter))
  (bind _playerbuildingcomponent (Variables|/Game/Blueprint/Core/BP_PlayerCharacter.BP_PlayerCharacter_C|GetPlayerBuildingComponent _controlledcharacter))
  ;[1 1 1] Toggle building options menu
  (:Pressed
    (Default|ToggleBuildingOptionsMenu _playerbuildingcomponent true))
  (:Released
    (Default|ToggleBuildingOptionsMenu _playerbuildingcomponent false)))

(fn ConstructionScript)