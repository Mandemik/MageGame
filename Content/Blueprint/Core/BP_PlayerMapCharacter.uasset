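; BP_PlayerMapCharacter is a player character Blueprint, named for a map context, that works with a visible mouse cursor.
; On BeginPlay it caches the inventory manager and custom player controller, then shows the cursor.
; SetControlRotation aims the controller from the capsule toward the world object hit under the cursor, though nothing in this graph calls it.
; ComponentsToSave returns the ability system component for saving.
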(event EventBeginPlay
  (|CallParentFunction)
  (CallFunction|SetVariables)
  (Variables|/Script/Engine.PlayerController|SetbShowMouseCursor (Variables|Default|GetPlayerControlerRef) true))

(fn ConstructionScript)

(fn SetControlRotation
  (bind _returnvalue (Pawn|GetController))
  (bind _asplayer_controller (Utilities|Casting|CastToPlayerController _returnvalue))
  (Pawn|SetControlRotation _asplayer_controller (Math|Rotator|FindLookatRotation (Transformation|GetWorldLocation (Variables|Default|GetCapsuleComponent)) (.location (.HitResult (Class|PlayerController|GetHitResultUnderCursorforObjects _asplayer_controller (Utilities|Array|MakeArray "ObjectTypeQuery1" "ObjectTypeQuery2") true))))))

(fn SetVariables
  (bind _inventorymanagercomponent (CallFunction|GetInventoryManager self))
  (Variables|Default|SetInventoryManager _inventorymanagercomponent)
  (bind _asbp_custom_player_controler (Utilities|Casting|CastToBP_CustomPlayerControler (Pawn|GetController)))
  (Variables|Default|SetPlayerControlerRef _asbp_custom_player_controler))

(fn ComponentstoSave
  (return (Utilities|Array|MakeArray (Variables|Default|GetAbilitySystemComp))))