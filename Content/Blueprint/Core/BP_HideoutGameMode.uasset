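; Game mode for the Hideout game that holds cheat handlers, per-level progress helpers and a play timer.
; Cheat events toggle damage immunity through a gameplay effect and boosted walk speed, grant the Dash skill, or kill all humanoid AI with massive damage.
; Helpers destroy AI pawns recorded as killed on the current level and store each level's best star count in the mage player state.
; A looping, pausable timer counts and prints seconds.
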(event EventBlueprintCheatUnlockAbility
  (params (enable :type Boolean))
  (if enable
    (Default|SetupActiveSkill (Variables|Default|GetPlayerRef) "/Game/AbilitySystem/DataTable/SkillDataAsset/Dash_SkillData.Dash_SkillData" "NewEnumerator2")))

(event EventBlueprintCheatImmortality
  (params (enable :type Boolean))
  (if enable
    (bind _returnvalue (GameplayEffects|ApplyGameplayEffectToSelf :self (Variables|/Script/MagBuildGame.BaseCharacter|GetAbilitySystemComp (Variables|Default|GetPlayerRef)) :GameplayEffectClass "/Game/AbilitySystem/Status/Blocks/GE_BlockDamageAll.GE_BlockDamageAll_C"))
    (Variables|Default|SetCheatBlockDamageAll _returnvalue)
    (else
      (GameplayEffects|RemoveActiveGameplayEffect (Variables|/Script/MagBuildGame.BaseCharacter|GetAbilitySystemComp (Variables|Default|GetPlayerRef)) (Variables|Default|GetCheatBlockDamageAll) -1))))

(event EventBlueprintCheatKillAllAi
  (params (enable :type Boolean))
  (if enable
    (CallFunction|KillAllAi)))

(event EventBlueprintCheatSuperSpeed
  (params (enable :type Boolean))
  (bind _playerref (Variables|Default|GetPlayerRef))
  (bind _charactermovement (Variables|/Script/Engine.Character|GetCharacterMovement _playerref))
  (if enable
    (Variables|/Script/Engine.CharacterMovementComponent|SetMaxWalkSpeed _charactermovement 2e+03)
    (else
      (Variables|/Script/Engine.CharacterMovementComponent|SetMaxWalkSpeed _charactermovement 475.0))))

(fn ConstructionScript)

(fn DestroySavedEnemysonCurrentLevel
  (bind _returnvalue (Game|GetCurrentLevelName true))
  (LocalVariables|SetCurrentLevelName _returnvalue)
  (bind _keys (Utilities|Map|Keys (Variables|Default|GetDestoyedAiPawns)))
  (for _array_element _keys
    (Utilities|IsValid _array_element
      (:Is%20Valid
        (if (and (.ReturnValue (Utilities|Map|Find (Variables|Default|GetDestoyedAiPawns) _array_element)) (Utilities|Enum|Equal(Enum) (LocalVariables|GetCurrentLevelName) (.Value (Utilities|Map|Find (Variables|Default|GetDestoyedAiPawns) _array_element))))
          (Actor|DestroyActor _array_element))))))

(fn AddLevelStars
  (params (LevelName :type Name) (Stars :type Integer))
  (bind _asbp_mage_player_state (Utilities|Casting|CastToBP_MagePlayerState (Variables|/Script/Engine.Pawn|GetPlayerState (Game|GetPlayerCharacter 0))))
  (if (.ReturnValue (Utilities|Map|Find (Variables|/Game/Blueprint/Core/BP_MagePlayerState.BP_MagePlayerState_C|GetStarLevelMap _asbp_mage_player_state) LevelName))
    (if (> Stars (.Value (Utilities|Map|Find (Variables|/Game/Blueprint/Core/BP_MagePlayerState.BP_MagePlayerState_C|GetStarLevelMap _asbp_mage_player_state) LevelName)))
      (Utilities|Map|Remove (Variables|/Game/Blueprint/Core/BP_MagePlayerState.BP_MagePlayerState_C|GetStarLevelMap _asbp_mage_player_state) LevelName)
      (Utilities|Map|Add (Variables|/Game/Blueprint/Core/BP_MagePlayerState.BP_MagePlayerState_C|GetStarLevelMap _asbp_mage_player_state) LevelName Stars :!label _label))
    (else
      (goto _label))))

(fn KillAllAi
  (bind _returnvalue (Game|GetPlayerController 0))
  (bind _outactors (Actor|GetAllActorsOfClass "/Game/Blueprint/AI/BP_AI_Humanoid.BP_AI_Humanoid_C"))
  (for _array_element _outactors
    (Game|Damage|ApplyDamage _array_element 9999999.0 _returnvalue _returnvalue "/Game/Blueprint/Core/DT_MagDamageType.DT_MagDamageType_C")))

(fn StartTimer
  (bind _returnvalue (Utilities|Time|SetTimerbyFunctionName 0 "UpadateTimerEachSec" 1.0 true))
  (Variables|Default|SetTimerHandle _returnvalue))

(fn UpadateTimerEachSec
  (bind _output_get (Variables|Default|SetTimer (+ (Variables|Default|GetTimer) (Math|Timespan|MakeTimespan 0 0 0 1 0))))
  (Development|PrintString (Utilities|String|ToString(Integer) (.seconds _output_get))))

(fn PauseTimer
  (Utilities|Time|PauseTimerbyHandle (Variables|Default|GetTimerHandle)))

(fn ComponentstoSave
  (return 0))