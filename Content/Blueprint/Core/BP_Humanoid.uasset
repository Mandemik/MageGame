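; BP_Humanoid is a humanoid character Blueprint that handles health, damage, healing, death and modular outfit meshes.
; At BeginPlay, body, armor and clothing components follow the main Mesh through master pose.
; Damage is skipped under a blocking gameplay tag, otherwise reduced by a percentage ability-system attribute; healing adds to health.
; At zero health it dies once, playing a death montage and disabling collision; the hit-reaction montage is unwired.
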(event Custom|CharacterDie
  (Variables|Default|SetIsLive false)
  (Animation|Montage|PlayMontage (Variables|Character|GetMesh) (Variables|Death|GetDeathAnim)
    (:then
      (Collision|SetActorEnableCollision false))))

(event Custom|ApplHeal
  (params (HealValue :type Float%20%28double-precision%29) (InstigatedBy :type Actor%20Object%20Reference))
  (Class|BaseCharacter|SetHealthValues (+ (.Health (Class|BaseCharacter|GetHealthValues)) HealValue)))

(event Game|Damage|EventAnyDamage
  (params (Damage :type Float%20%28single-precision%29) (DamageType :type Damage%20Type%20Object%20Reference) (InstigatedBy :type Controller%20Object%20Reference) (DamageCauser :type Actor%20Object%20Reference))
  (if (not (GameplayTags|HasMatchingGameplayTag (Variables|Default|GetAbilitySystemComp) "(TagName=\"Status.BlockAnyDamage\")"))
    (Class|BaseCharacter|SetHealthValues (- (.Health (Class|BaseCharacter|GetHealthValues)) (Math|Float|Max(Float) (* Damage (/ (- 1e+02 (.ReturnValue (Ability|Attribute|GetFloatAttributefromAbilitySystemComponent (Variables|Default|GetAbilitySystemComp) "(AttributeName=\"PhysicArmor\",Attribute=/Script/MagBuildGame.BaseAttributeSet:PhysicArmor,AttributeOwner=Class'\"/Script/MagBuildGame.BaseAttributeSet\"')"))) 1e+02)) 0.0)))
    (if (not (GameplayTags|HasMatchingGameplayTag (Variables|Default|GetAbilitySystemComp) "(TagName=\"Status.Block.Reaction\")"))
      _)))

(event EventBeginPlay
  (|CallParentFunction)
  (CallFunction|SetupClothAnimation))

(event EventOnHealthChanged
  (params (OldValue :type Float%20%28single-precision%29) (NewValue :type Float%20%28single-precision%29))
  (if (<= NewValue 0.0)
    (Utilities|FlowControl|DoOnce false
      (:Completed
        (CallFunction|CharacterDie)))))

(fn ConstructionScript
  (|CallParentFunction))

(fn GetIsLive
  (return (Variables|Default|GetIsLive)))

(fn SetupClothAnimation
  (Class|SkinnedMeshComponent|SetMasterPoseComponent (Variables|Default|GetEars) (Variables|Character|GetMesh) false))