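; BP_MapChooser is an interactable level-select object that loads a configured map when the player interacts with it.
; On BeginPlay it reads PlayerStars from BP_GameInstance and hides itself in game if the count is below its required stars.
; Interaction calls SwitchMap on the game instance with its level name and no monument.
; The construction script writes the map number onto its TextRender label.
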(event EventBeginPlay
  (|CallParentFunction)
  (bind _asbp_game_instance (Utilities|Casting|CastToBP_GameInstance (Game|GetGameInstance)))
  (if (< (Variables|/Game/Blueprint/Core/BP_GameInstance.BP_GameInstance_C|GetPlayerStars _asbp_game_instance) (Variables|Default|GetRequireStars))
    (Rendering|SetActorHiddenInGame true)))

(event EventInteractwithObject
  (params (InteractCauser :type BP%20Player%20Character%201%20Object%20Reference))
  (Default|SwitchMap (.AsBP%20Game%20Instance (Utilities|Casting|CastToBP_GameInstance (Game|GetGameInstance))) (Variables|Default|GetLevel%20Name%20To%20Load) false))

(fn ConstructionScript
  (|CallParentFunction)
  (Rendering|Components|TextRender|SetText (Variables|Default|GetTextRender) (Variables|Default|GetMapNumber)))