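; BP_InteractObject is a world object the player can use to complete a "Use" quest objective.
; A sphere trigger detects BP_PlayerCharacter1, registers or clears itself as that player's interaction target and shows or hides a widget.
; InteractwithObject asks its quest target component, named from QuestTargetName at construction, to finish the objective.
; An optional single-use flag disables the sphere's collision after the first interaction.
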(event OnComponentBeginOverlap(Sphere)
  (params (OverlappedComponent :type Primitive%20Component%20Object%20Reference) (OtherActor :type Actor%20Object%20Reference) (OtherComp :type Primitive%20Component%20Object%20Reference) (OtherBodyIndex :type Integer) (bFromSweep :type Boolean) (SweepResult :type Hit%20Result%20Structure%20%28by%20ref%29))
  (CallFunction|StartOverlap OtherActor))

(event OnComponentEndOverlap(Sphere)
  (params (OverlappedComponent :type Primitive%20Component%20Object%20Reference) (OtherActor :type Actor%20Object%20Reference) (OtherComp :type Primitive%20Component%20Object%20Reference) (OtherBodyIndex :type Integer))
  (CallFunction|EndOverlap OtherActor))

(event EventBeginPlay)

(event Collision|EventActorBeginOverlap
  (params (OtherActor :type Actor%20Object%20Reference)))

(event EventTick
  (params (DeltaSeconds :type Float%20%28single-precision%29)))

(event EventInteractwithObject
  (params (InteractCauser :type BP%20Player%20Character%201%20Object%20Reference))
  (if (Variables|Default|GetCanBeUseOnlyOnes)
    (Utilities|FlowControl|DoOnce false
      (:Completed
        (Collision|SetCollisionEnabled (Variables|Default|GetSphere) "NoCollision"))))
  (Default|TryFinishObjective (Variables|Default|GetManager_QuestTarget) "Use" InteractCauser)
  (Development|PrintString "Interaction"))

(fn ConstructionScript
  (Variables|/Game/QuestManager/Blueprints/Components/Manager_QuestTarget.Manager_QuestTarget_C|SetTargetName (Variables|Default|GetManager_QuestTarget) (Variables|Default|GetQuestTargetName)))

(fn StartOverlap
  (params (Object :type Object%20Object%20Reference))
  (bind _asbp_player_character_1 (Utilities|Casting|CastToBP_PlayerCharacter1 Object)
    (:then
      (Development|PrintString (Utilities|String|Append (Utilities|GetDisplayName Object) " overlap  Start with me"))
      (bind _output_get (Variables|Default|SetPlayerCouser _asbp_player_character_1))
      (Class|BPInteractionInterface|CanInteractwithMe(Message) _output_get true self)
      (Rendering|SetVisibility (Variables|Default|GetWidget) true false))
    (:CastFailed
      (Development|PrintString "BP_InteractObject overlap with wrong pawn"))))

(fn EndOverlap
  (params (Object :type Object%20Object%20Reference))
  (bind _asbp_player_character_1 (Utilities|Casting|CastToBP_PlayerCharacter1 Object)
    (:then
      (Development|PrintString (Utilities|String|Append (Utilities|GetDisplayName Object) " overlap  End with me"))
      (Class|BPInteractionInterface|CanInteractwithMe(Message) _asbp_player_character_1 false)
      (Rendering|SetVisibility (Variables|Default|GetWidget) false false))
    (:CastFailed
      (Development|PrintString "BP_InteractObject overlap with wrong pawn"))))