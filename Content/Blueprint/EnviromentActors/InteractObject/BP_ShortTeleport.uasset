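; BP_ShortTeleport is an interactable teleporter that moves the player to a linked Destiny teleporter when they overlap its sphere while it is active.
; Before moving the player and playing a sound, it blocks the destination for two seconds to prevent bouncing straight back.
; SetTeleportActivation toggles the active flag, fire effect and audio, and is reapplied on BeginPlay and after save loading through ActorLoaded.
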(event OnComponentBeginOverlap(Sphere)
  (params (OverlappedComponent :type Primitive%20Component%20Object%20Reference) (OtherActor :type Actor%20Object%20Reference) (OtherComp :type Primitive%20Component%20Object%20Reference) (OtherBodyIndex :type Integer) (bFromSweep :type Boolean) (SweepResult :type Hit%20Result%20Structure%20%28by%20ref%29))
  (bind (_asbp_player_character _bsuccess) (Utilities|Casting|CastToBP_PlayerCharacter OtherActor))
  (bind _destiny (Variables|Default|GetDestiny))
  (if (Math|Boolean|ANDBoolean _bsuccess (Variables|Default|GetTeleportIsActive) (not (Variables|Default|GetTempolaryBlock)))
    (Variables|Default|SetPlayerRef _asbp_player_character)
    (Variables|BP_ShortTeleport_C|SetTempolaryBlock _destiny true)
    (Utilities|Time|SetTimerbyFunctionName _destiny "UnlockTempolaryBlock" 2.0)
    (CallFunction|HandlePlayerTeleport)))

(event EventBeginPlay
  (CallFunction|SetTeleportActivation (Variables|Default|GetTeleportIsActive)))

(event EventActorLoaded
  (CallFunction|SetTeleportActivation (Variables|Default|GetTeleportIsActive)))

(fn ConstructionScript)

(fn SetTeleportActivation
  (params (Active :type Boolean))
  (bind _output_get (Variables|Default|SetTeleportIsActive Active))
  (if _output_get
    (Components|Activation|Activate (Variables|Default|GetPS_FX_fire_Blue) true)
    (Components|Activation|SetActive (Variables|Default|GetAudio) true true)
    (else
      (Components|Activation|Deactivate (Variables|Default|GetPS_FX_fire_Blue))
      (Components|Activation|SetActive (Variables|Default|GetAudio) false false))))

(fn UnlockTempolaryBlock
  (Variables|Default|SetTempolaryBlock false))

(fn HandlePlayerTeleport
  (Transformation|SetActorLocation (Variables|Default|GetPlayerRef) (Transformation|GetWorldLocation (Variables|BP_ShortTeleport_C|GetTeleportPosition (Variables|Default|GetDestiny))) false false)
  (Audio|SpawnSoundAttached "/Game/AUDIO/SFX/Usables/Short_Teleport/SFX_Teleport_Enter.SFX_Teleport_Enter" (Variables|/Script/Engine.Character|GetMesh (Variables|Default|GetPlayerRef)) "root" "0, 0, 0" "0, 0, 0" "KeepRelativeOffset" false 1.0 1.0 0.0 0 0))

(fn ComponentstoSave
  (return 0))