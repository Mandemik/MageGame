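; Interactable two-way teleport that moves the arena player character between its Sphere and TeleportStart components.
; TeleportStart overlaps feed the overlap start/end functions, and the start override moves the prompt widget above the end where the player stands.
; Interacting plays the HUD's quick fade, waits briefly, then places the character above the opposite end, chosen by whether player 0 overlaps Sphere.
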(event OnComponentBeginOverlap(TeleportStart)
  (params (OverlappedComponent :type Primitive%20Component%20Object%20Reference) (OtherActor :type Actor%20Object%20Reference) (OtherComp :type Primitive%20Component%20Object%20Reference) (OtherBodyIndex :type Integer) (bFromSweep :type Boolean) (SweepResult :type Hit%20Result%20Structure%20%28by%20ref%29))
  (CallFunction|StartOverlap OtherActor))

(event OnComponentEndOverlap(TeleportStart)
  (params (OverlappedComponent :type Primitive%20Component%20Object%20Reference) (OtherActor :type Actor%20Object%20Reference) (OtherComp :type Primitive%20Component%20Object%20Reference) (OtherBodyIndex :type Integer))
  (CallFunction|EndOverlap OtherActor))

(event EventInteractwithObject
  (params (InteractCauser :type BP%20Player%20Character%201%20Object%20Reference))
  (bind _asbp_player_arena_character (Utilities|Casting|CastToBP_PlayerArenaCharacter InteractCauser)
    (:then
      (UserInterface|Animation|PlayAnimation (Variables|/Game/Blueprint/Core/BP_PlayerArenaCharacter.BP_PlayerArenaCharacter_C|GetHudRef _asbp_player_arena_character) (Variables|/Game/UI/W_PlayerHud.W_PlayerHud_C|GetQuickFade (Variables|/Game/Blueprint/Core/BP_PlayerArenaCharacter.BP_PlayerArenaCharacter_C|GetHudRef _asbp_player_arena_character)) 0.0 1 "Forward" 1.0 false)
      (Utilities|FlowControl|Delay 0.15)
      (Transformation|SetActorLocation InteractCauser (+ (Transformation|GetWorldLocation (select (Collision|IsOverlappingActor (Variables|Default|GetSphere) (Game|GetPlayerCharacter 0) :!class /Script/Engine.PrimitiveComponent) (Variables|Default|GetTeleportStart) (Variables|Default|GetSphere))) "0,0,110.000000") false false))
    (:CastFailed
      (Development|PrintString "Teleport has to be use with arena Character"))))

(fn ConstructionScript)

(fn StartOverlap
  (params (Object :type Object%20Object%20Reference))
  (|CallParentFunction Object)
  (Transformation|SetWorldLocation (Variables|Default|GetWidget) (+ (Transformation|GetWorldLocation (select (Collision|IsOverlappingActor (Variables|Default|GetSphere) (Game|GetPlayerCharacter 0) :!class /Script/Engine.PrimitiveComponent) (Variables|Default|GetSphere) (Variables|Default|GetTeleportStart))) "0,0,110.000000") false false))

(fn ComponentstoSave
  (return 0))