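; BP_ArrowTrap is an environment trap that repeatedly fires arrow projectiles from three mesh parts, starting at BeginPlay.
; A looping timer calls SpawnArrow, which spawns projectiles along the trap's forward vector, makes them ignore the trap and plays a launch sound.
; When NeedLever is set, it binds to the levers in LeverArray.
; Lever toggles re-check the array, intending to stop firing once all levers are active and resume otherwise.
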(event Custom|LeverToggle
  (params (Active? :type Boolean))
  (bind _enable (CallFunction|CheckLevers))
  (bind _output_get (Variables|Default|SetTrapActive (not _enable)))
  (CallFunction|ActiveTrap _output_get))

(event EventBeginPlay
  (Utilities|FlowControl|Sequence
    (:then_0
      (CallFunction|SetupLevers))
    (:then_1
      (CallFunction|ActiveTrap true))))

(fn ConstructionScript)

(fn SpawnArrow
  (bind _defaultsceneroot1 (Variables|Default|GetDefaultSceneRoot1))
  (bind _returnvalue (Math|Vector|GetForwardVector _defaultsceneroot1))
  (if (Variables|Default|GetTrapActive)
    (for _array_element (Utilities|Array|MakeArray (Variables|Default|GetSM_PROP_trap_arrow_part_dungeon_07) (Variables|Default|GetSM_PROP_trap_arrow_part_dungeon_04) (Variables|Default|GetSM_PROP_trap_arrow_part_dungeon_09))
      (bind _returnvalue_2 (Game|SpawnActorfromClass "/Game/Blueprint/EnviromentActors/Traps/BP_Arrow_Projectile.BP_Arrow_Projectile_C" (Math|Transform|MakeTransform (+ (Transformation|GetWorldLocation _array_element) (* _returnvalue 1e+02)) (Math|Conversions|RotationFromXVector _returnvalue) "1.000000,1.000000,1.000000") "Undefined" 0 5e+01 2e+02 0))
      (Collision|IgnoreActorwhenMoving (Variables|/Game/Blueprint/EnviromentActors/Traps/BP_Arrow_Projectile.BP_Arrow_Projectile_C|GetSphere1 _returnvalue_2) self true)
      (Audio|PlaySoundatLocation "/Game/AUDIO/SFX/Traps/SFX_Trap_Arrow_Launch_Cue.SFX_Trap_Arrow_Launch_Cue" (Transformation|GetActorLocation) "0, 0, 0" 1.0 1.0 0.0 0 0 0 0))))

(fn SetupLevers
  (if (Variables|Default|GetNeedLever)
    (for _array_element (Variables|Default|GetLeverArray)
      (EventDispatchers|BindEventtoLeverActivation _array_element (EventDispatchers|CreateEvent :!event Custom|LeverToggle)))))

(fn CheckLevers
  (bind _array_element (Utilities|Array|ForEachLoopwithBreak (Variables|Default|GetLeverArray) :!label _label)
    (:LoopBody
      (if (not (Variables|/Game/Blueprint/EnviromentActors/InteractObject/BP_Lever.BP_Lever_C|GetLeverActive _array_element))
        (LocalVariables|SetSuccess false)
        (goto _label Break)))
    (:Completed
      (return (LocalVariables|GetSuccess)))))

(fn ActiveTrap
  (params (Active :type Boolean))
  (if Active
    (bind _returnvalue (Utilities|Time|SetTimerbyFunctionName 0 "SpawnArrow" (Variables|Default|GetSpawnFrequence) true))
    (Variables|Default|SetSpawnArrowTimerLoop _returnvalue)
    (CallFunction|SpawnArrow)
    (else
      (Utilities|Time|ClearandInvalidateTimerbyHandle (Variables|Default|GetSpawnArrowTimerLoop)))))