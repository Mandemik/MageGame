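; BP_Ice_Mine is an environment trap that deals radial damage and applies an ice status when activated.
; ActiveTrap moves the explosion effect to the overlapping actor and restarts it, applies full radial damage around the mine, gives that actor GE_StatusIce through its Ability System Component, then calls the parent trap logic.
; On BeginPlay it starts its water loop sound at a clamped random start time.
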(event EventBeginPlay
  (Audio|Components|Audio|Play (Variables|Default|GetSFX_Mine_Water_LP_Cue) (Math|Float|Clamp(Float) (Math|Random|RandomFloat) 0.1 5.0)))

(event EventActiveTrap
  (Transformation|SetWorldLocation (Variables|Default|GetExplosion_Effect) (Transformation|GetActorLocation (Variables|Default|GetOverlapActor)) false false)
  (Niagara|ResetSystem (Variables|Default|GetExplosion_Effect))
  (Game|Damage|ApplyRadialDamage (Variables|Default|GetDamageValue) (Transformation|GetActorLocation) 2.5e+02 0 0 self 0 true "ECC_Visibility")
  (GameplayEffects|ApplyGameplayEffectToSelf :self (Ability|GetAbilitySystemComponent (Variables|Default|GetOverlapActor)) :GameplayEffectClass "/Game/AbilitySystem/Status/Ice/GE_StatusIce.GE_StatusIce_C")
  (|CallParentFunction))

(fn ConstructionScript
  (|CallParentFunction))