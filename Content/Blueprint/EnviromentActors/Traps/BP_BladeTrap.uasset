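; Swinging blade dungeon trap that damages any BP_Humanoid overlapping its blade mesh.
; The Swap timeline lerps the blade's pitch between two opposite angles and restarts whenever it finishes.
; BeginPlay resets the timeline time and starts it through ActiveTrap, which can also stop it.
; A random or configured start time is selected within the timeline loop.
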(event OnComponentBeginOverlap(SM_PROP_trap_blade_dungeon_02)
  (params (OverlappedComponent :type Primitive%20Component%20Object%20Reference) (OtherActor :type Actor%20Object%20Reference) (OtherComp :type Primitive%20Component%20Object%20Reference) (OtherBodyIndex :type Integer) (bFromSweep :type Boolean) (SweepResult :type Hit%20Result%20Structure%20%28by%20ref%29))
  (bind _asbp_humanoid (Utilities|Casting|CastToBP_Humanoid OtherActor))
  (Game|Damage|ApplyDamage _asbp_humanoid (Variables|Default|GetDamage) 0 0))

(event Custom|ActiveTrap
  (params (Active :type Boolean))
  (if Active
    (bind _progress (Timeline|Swap Play)
      (:Update
        (Transformation|SetRelativeRotation (Variables|Default|GetSM_PROP_trap_blade_dungeon_02) (Math|Rotator|MakeRotator 0.0 (Math|Float|Lerp -6e+01 6e+01 _progress) 0.0) false false))
      (:Finished
        (CallFunction|SwapLoop)))
    (else
      (Timeline|Swap Stop))))

(event Custom|SwapLoop
  (bind _progress (Timeline|Swap PlayFromStart)
    (:Update
      (Transformation|SetRelativeRotation (Variables|Default|GetSM_PROP_trap_blade_dungeon_02) (Math|Rotator|MakeRotator 0.0 (Math|Float|Lerp -6e+01 6e+01 _progress) 0.0) false false))
    (:Finished
      (CallFunction|SwapLoop))))

(event Custom|SetStartingTime
  (bind _progress (Timeline|Swap SetNewTime)
    (:Update
      (Transformation|SetRelativeRotation (Variables|Default|GetSM_PROP_trap_blade_dungeon_02) (Math|Rotator|MakeRotator 0.0 (Math|Float|Lerp -6e+01 6e+01 _progress) 0.0) false false))
    (:Finished
      (CallFunction|SwapLoop))))

(event EventBeginPlay
  (CallFunction|SetStartingTime)
  (CallFunction|ActiveTrap true))

(fn ConstructionScript)