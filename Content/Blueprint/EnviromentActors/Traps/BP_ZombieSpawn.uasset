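; Trapdoor trap that periodically spawns AI humanoids (zombies) at its spawn point while active, capped at a maximum living count.
; A looping timer drives SpawnZombie, which broadcasts each new pawn and binds its death event to free a slot.
; Optional linked levers re-evaluate the trap on toggle, deactivating it when all are active.
; A timeline swings the trapdoor open or closed to match the trap state.
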(event Custom|PlayTrapAnimation
  (params (Condition :type Boolean))
  (if Condition
    (bind _progres (Timeline|TrapOpening Play)
      (:Update
        (Transformation|SetRelativeRotation (Variables|Default|GetSM_PROP_trapdoor_door_dungeon_02) (Math|Rotator|MakeRotator 0.0 (Math|Float|Lerp 0.0 5e+01 _progres) 0.0) false false)))
    (else
      (Timeline|TrapOpening Reverse))))

(event Custom|LeverToggle
  (params (Active? :type Boolean))
  (bind _enable (CallFunction|CheckLevers))
  (bind _output_get (Variables|Default|SetTrapActive (not _enable)))
  (CallFunction|ActiveSpawn _output_get)
  (CallFunction|PlayTrapAnimation (Variables|Default|GetTrapActive)))

(event Custom|SpawnEnemyDie
  (Math|Integer|DecrementInt (Variables|Default|GetSpawnEnemyNumber)))

(event EventBeginPlay
  (Utilities|FlowControl|Sequence
    (:then_0
      (CallFunction|SetupLevers))
    (:then_1
      (CallFunction|ActiveSpawn true))
    (:then_2
      (CallFunction|PlayTrapAnimation (Variables|Default|GetTrapActive)))))

(fn ConstructionScript)

(fn SpawnZombie
  (if (and (Variables|Default|GetTrapActive) (< (Variables|Default|GetSpawnEnemyNumber) (Variables|Default|GetMaxPawnSpawned)))
    (bind _returnvalue (AI|SpawnAIFromClass (Variables|Default|GetSpawnClass) (Variables|Default|GetSpawn_BT) (Transformation|GetWorldLocation (Variables|Default|GetSpawnPosition)) "0, 0, 0" false 0))
    (Default|CallSpawnNewPawn (.AsBP%20AI%20Humanoid (Utilities|Casting|CastToBP_AI_Humanoid _returnvalue)))
    (EventDispatchers|BindEventtoOnDie (.AsBP%20AI%20Humanoid (Utilities|Casting|CastToBP_AI_Humanoid _returnvalue)) (EventDispatchers|CreateEvent :!event Custom|SpawnEnemyDie))
    (Math|Integer|IncrementInt (Variables|Default|GetSpawnEnemyNumber))))

(fn SetupLevers
  (if (Variables|Default|GetNeedLever)
    (for _array_element (Variables|Default|GetLeverArray)
      (EventDispatchers|BindEventtoLeverActivation _array_element (EventDispatchers|CreateEvent :!event Custom|LeverToggle)))))

(fn CheckLevers
  (bind _array_element (Utilities|Array|ForEachLoopwithBreak (Variables|Default|GetLeverArray) :!label _label)
    (:LoopBody
      (if (not (Variables|/Game/Blueprint/EnviromentActors/InteractObject/BP_Lever.BP_Lever_C|GetLeverActive _array_element))
        (LocalVariables|SetSuccess false)
        (goto _label Break)))
    (:Completed
      (return (LocalVariables|GetSuccess)))))

(fn ActiveSpawn
  (params (Active :type Boolean))
  (if Active
    (bind _returnvalue (Utilities|Time|SetTimerbyFunctionName 0 "SpawnZombie" (Variables|Default|GetSpawnFrequence) true))
    (Variables|Default|SetSpawnArrowTimerLoop _returnvalue)
    (CallFunction|SpawnZombie)
    (else
      (Utilities|Time|ClearandInvalidateTimerbyHandle (Variables|Default|GetSpawnArrowTimerLoop)))))