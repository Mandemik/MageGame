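; BP_WaterMine is an environmental trap that explodes when triggered, dealing damage and applying a water status effect.
; Its ActiveTrap override restarts the explosion effect at the overlapping actor's location and applies full radial damage around the mine.
; It then applies GE_StatusWater through the Gameplay Ability System to the overlapping actor only, before handing off to the parent trap logic.
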(event EventActiveTrap
  (Transformation|SetWorldLocation (Variables|Default|GetExplosion_Effect) (Transformation|GetActorLocation (Variables|Default|GetOverlapActor)) false false)
  (Niagara|ResetSystem (Variables|Default|GetExplosion_Effect))
  (Game|Damage|ApplyRadialDamage (Variables|Default|GetDamageValue) (Transformation|GetActorLocation) 2.5e+02 0 0 self 0 true "ECC_Visibility")
  (GameplayEffects|ApplyGameplayEffectToSelf :self (Ability|GetAbilitySystemComponent (Variables|Default|GetOverlapActor)) :GameplayEffectClass "/Game/AbilitySystem/Status/Water/GE_StatusWater.GE_StatusWater_C")
  (|CallParentFunction))

(fn ConstructionScript
  (|CallParentFunction))