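; Destructible environment actor that breaks once, either when the player character overlaps it or when it takes damage, depending on DestructibleType.
; Destruction spawns an optional particle system, tries an item drop through BPItemComponent, and disables collision.
; The actor then hides, immediately or after a reversed timeline animates the "Appearance" parameter on a dynamic material.
; A destroyed flag lets ActorLoaded restore the hidden, non-colliding state after loading.
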(event OnComponentBeginOverlap(StaticMeshComponent)
  (params (OverlappedComponent :type Primitive%20Component%20Object%20Reference) (OtherActor :type Actor%20Object%20Reference) (OtherComp :type Primitive%20Component%20Object%20Reference) (OtherBodyIndex :type Integer) (bFromSweep :type Boolean) (SweepResult :type Hit%20Result%20Structure%20%28by%20ref%29))
  (if (Utilities|Enum|Equal(Enum) (Variables|Default|GetDestructibleType) "NewEnumerator0")
    (Utilities|Casting|CastToBP_PlayerArenaCharacter OtherActor)
    (CallFunction|TriggerExplosion)))

(event Custom|PlayDestroyAnimation
  (bind _showprogress (Timeline|Timeline_0 ReverseFromEnd)
    (:Update
      (Rendering|Material|SetScalarParameterValue (Variables|Default|GetDynamicMaterial) "Appearance" _showprogress :!class /Script/Engine.MaterialInstanceDynamic))
    (:Finished
      (Rendering|SetActorHiddenInGame true))))

(event Custom|TriggerExplosion
  (Utilities|FlowControl|DoOnce false
    (:Completed
      (CallFunction|OnDestruction)
      (Collision|SetActorEnableCollision false)
      (Variables|Default|SetItemDestoyed true))))

(event EventBeginPlay
  (if (Variables|Default|GetAnimationDestroy)
    (CallFunction|PreperMaterialforAnimation)))

(event Game|Damage|EventAnyDamage
  (params (Damage :type Float%20%28single-precision%29) (DamageType :type Damage%20Type%20Object%20Reference) (InstigatedBy :type Controller%20Object%20Reference) (DamageCauser :type Actor%20Object%20Reference))
  (if (Utilities|Enum|Equal(Enum) (Variables|Default|GetDestructibleType) "NewEnumerator1")
    (CallFunction|TriggerExplosion)))

(event EventActorLoaded
  (if (Variables|Default|GetItemDestoyed)
    (Collision|SetActorEnableCollision false)
    (Rendering|SetActorHiddenInGame true)))

(fn ConstructionScript)

(fn OnDestruction
  (Utilities|FlowControl|Sequence
    (:then_0
      (Utilities|IsValid (Variables|Default|GetParticleOnDestory)
        (:Is%20Valid
          (Niagara|SpawnSystematLocation (Variables|Default|GetParticleOnDestory) (Transformation|GetActorLocation) "0, 0, 0" "2.000000,2.000000,2.000000"))))
    (:then_1
      (Default|TryDropItem (Variables|Default|GetBP_ItemComponent)))
    (:then_2
      (if (Variables|Default|GetAnimationDestroy)
        (CallFunction|PlayDestroyAnimation)
        (else
          (Rendering|SetActorHiddenInGame true))))))

(fn PreperMaterialforAnimation
  (bind _staticmeshcomponent (Variables|Debug|GetStaticMeshComponent))
  (bind _returnvalue (Rendering|Material|CreateDynamicMaterialInstance _staticmeshcomponent 0 (Rendering|Material|GetMaterial _staticmeshcomponent 0) "None" :!class /Script/Engine.PrimitiveComponent))
  (Variables|Default|SetDynamicMaterial _returnvalue))

(fn ComponentstoSave
  (return 0))