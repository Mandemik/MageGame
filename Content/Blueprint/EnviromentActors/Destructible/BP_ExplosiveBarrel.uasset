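; Explosive barrel Blueprint that extends a destructible parent and damages nearby characters when destroyed.
; On destruction, it runs the parent logic, then sphere-overlaps for Characters within the explosion radius.
; Each one takes point damage with a barrel-specific damage type and is launched directly away from the blast center.
; It also speeds up the inherited destroy animation by raising its timeline's play rate.
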(event EventBeginPlay
  (|CallParentFunction) ; This node is disabled and will not be called.\nDrag off pins to build functionality.
)

(event Collision|EventActorBeginOverlap
  (params (OtherActor :type Actor%20Object%20Reference)))

(event EventTick
  (params (DeltaSeconds :type Float%20%28single-precision%29)))

(event EventPlayDestroyAnimation
  (Components|Timeline|SetPlayRate (Variables|Default|GetTimeline_0) 2.0)
  (|CallParentFunction))

(fn ConstructionScript
  (|CallParentFunction))

(fn OnDestruction
  (|CallParentFunction)
  (bind _outactors (Collision|SphereOverlapActors (Transformation|GetActorLocation) (Variables|Default|GetExplosionRadius) (Utilities|Array|MakeArray "ObjectTypeQuery3" "ObjectTypeQuery6") "/Script/Engine.Character"))
  (for _array_element _outactors
    (Game|Damage|ApplyPointDamage _array_element (Variables|Default|GetExplosionDamage) (Math|Rotator|GetRotationXVector (Math|Rotator|FindLookatRotation (Transformation|GetActorLocation) (Transformation|GetActorLocation _array_element))) (Collision|MakeHitResult false false 0.0 0.0 "0, 0, 0" "0, 0, 0" "0,0,1" "0,0,1" 0 0 0 "None" "None" 0 0 0 "0, 0, 0" "0, 0, 0") 0 (Variables|Default|GetInstigator) "/Game/Blueprint/EnviromentActors/Destructible/DT_ExplosiveBarrel.DT_ExplosiveBarrel_C")
    (bind _ascharacter (Utilities|Casting|CastToCharacter _array_element))
    (Character|LaunchCharacter _ascharacter (* (Math|Rotator|GetRotationXVector (Math|Rotator|FindLookatRotation (Transformation|GetActorLocation) (Transformation|GetActorLocation _array_element))) 7.5e+02) false false)))