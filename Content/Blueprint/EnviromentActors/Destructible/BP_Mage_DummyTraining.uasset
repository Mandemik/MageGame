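; Destructible mage training dummy that reacts to damage with hit or death animations, sounds and chip particles.
; Until death, AnyDamage passes the damage type's tag and causer to ManagerQuestTarget to try finishing a quest objective, provided it is a DT_MagDamageType.
; EnemyDamage subtracts truncated damage, or zero when Immortal, playing the crash sound only at exactly zero health.
; The hit animation choice is hardwired to the second variant.
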(event EventBeginPlay)

(event Game|Damage|EventAnyDamage
  (params (Damage :type Float%20%28single-precision%29) (DamageType :type Damage%20Type%20Object%20Reference) (InstigatedBy :type Controller%20Object%20Reference) (DamageCauser :type Actor%20Object%20Reference))
  (if (not (Variables|Default|GetDeath))
    (CallFunction|HandleQuestLogic DamageType DamageCauser)
    (CallFunction|EnemyDamage (Math|Integer|SelectInt 0 (Math|Float|Truncate Damage) (Variables|Default|GetImmortal)))
    (Components|Activation|Activate (Variables|Default|GetPS_chips) true)
    (if (<= (Variables|Default|GetHealh) 0)
      (Components|Animation|PlayAnimation (Variables|Default|GetSK_Dummy_Training) "/Game/DummyTraining/Animations/AN_Dummy_Death.AN_Dummy_Death" false)
      (Variables|Default|SetDeath true)
      (else
        (Components|Animation|PlayAnimation (Variables|Default|GetSK_Dummy_Training) (Utilities|Select :Index 1 :Option%200 "/Game/DummyTraining/Animations/AN_Dummy_Hit1.AN_Dummy_Hit1" :Option%201 "/Game/DummyTraining/Animations/AN_Dummy_Hit2.AN_Dummy_Hit2") false)))))

(fn ConstructionScript)

(fn EnemyDamage
  (params (B :type Integer))
  (Variables|Default|SetHealh (- (Variables|Default|GetHealh) B))
  (if (== (Variables|Default|GetHealh) 0)
    (Audio|Components|Audio|Play (Variables|Default|GetSC_crash-wood) 0.0)
    (else
      (Audio|Components|Audio|Play (Variables|Default|GetSC_hit) 0.0))))

(fn HandleQuestLogic
  (params (DamageType :type Damage%20Type%20Object%20Reference) (Causer :type Actor%20Object%20Reference))
  (bind _asdt_mag_damage_type (Utilities|Casting|CastToDT_MagDamageType DamageType)
    (:then
      (Default|TryFinishObjective (Variables|Default|GetManager_QuestTarget) (Variables|/Game/Blueprint/Core/DT_MagDamageType.DT_MagDamageType_C|GetDamageTag _asdt_mag_damage_type) Causer))
    (:CastFailed
      (Development|PrintString "Wrong damage typ to handle quest"))))