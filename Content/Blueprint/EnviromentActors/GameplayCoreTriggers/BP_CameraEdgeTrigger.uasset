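; BP_CameraEdgeTrigger is a box trigger that holds the arena player's third-person camera at a fixed world Y while the character is inside.
; On overlap it captures the camera's Y and starts a fast looping timer, apparently driving CameraChangeLenght to re-apply that Y, cleared on exit.
; A delayed BeginPlay check also catches players already inside, though IsActive is stored without gating anything.
; The construction script sizes the box from BoxSize.
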(event OnComponentBeginOverlap(Box)
  (params (OverlappedComponent :type Primitive%20Component%20Object%20Reference) (OtherActor :type Actor%20Object%20Reference) (OtherComp :type Primitive%20Component%20Object%20Reference) (OtherBodyIndex :type Integer) (bFromSweep :type Boolean) (SweepResult :type Hit%20Result%20Structure%20%28by%20ref%29))
  (bind (_asbp_player_arena_character _bsuccess) (Utilities|Casting|CastToBP_PlayerArenaCharacter OtherActor))
  (if _bsuccess
    (CallFunction|StartOverlap _asbp_player_arena_character)))

(event OnComponentEndOverlap(Box)
  (params (OverlappedComponent :type Primitive%20Component%20Object%20Reference) (OtherActor :type Actor%20Object%20Reference) (OtherComp :type Primitive%20Component%20Object%20Reference) (OtherBodyIndex :type Integer))
  (if (.bSuccess (Utilities|Casting|CastToBP_PlayerArenaCharacter OtherActor))
    (Development|PrintString "CameraLeftEdge!")
    (Utilities|Time|ClearandInvalidateTimerbyHandle (Variables|Default|GetCameraOverlapTimer))))

(event Custom|CameraChangeLenght
  (bind _as_bp_player_arena_character (Variables|Default|GetAs%20BP%20Player%20Arena%20Character))
  (bind _tp_camera (Variables|/Game/Blueprint/Core/BP_PlayerCharacter1.BP_PlayerCharacter1_C|GetTP%20Camera _as_bp_player_arena_character))
  (bind _returnvalue (Transformation|GetWorldLocation _tp_camera))
  (Transformation|SetWorldLocation _tp_camera (Math|Vector|MakeVector (.x _returnvalue) (Variables|Default|GetWidth) (.z _returnvalue)) false false))

(event EventBeginPlay
  (Utilities|FlowControl|Delay 1.0)
  (CallFunction|ChangeTriggerState (Variables|Default|GetIsActive)))

(fn ConstructionScript
  (Components|Box|SetBoxExtent (Variables|Default|GetBox) (Variables|Default|GetBoxSize) true))

(fn ChangeTriggerState
  (params (IsActive :type Boolean))
  (Variables|Default|SetIsActive IsActive)
  (for _array_element (Collision|GetOverlappingActors (Variables|Default|GetBox) "/Game/Blueprint/Core/BP_PlayerArenaCharacter.BP_PlayerArenaCharacter_C" :!class /Script/Engine.PrimitiveComponent)
    (if (.bSuccess (Utilities|Casting|CastToBP_PlayerArenaCharacter _array_element))
      (CallFunction|StartOverlap (.AsBP%20Player%20Arena%20Character (Utilities|Casting|CastToBP_PlayerArenaCharacter _array_element))))))

(fn StartOverlap
  (params (PlayerRef :type BP%20Player%20Arena%20Character%20Object%20Reference))
  (bind _output_get (Variables|Default|SetAs%20BP%20Player%20Arena%20Character PlayerRef))
  (Variables|Default|SetWidth (.y (Transformation|GetWorldLocation (Variables|/Game/Blueprint/Core/BP_PlayerCharacter1.BP_PlayerCharacter1_C|GetTP%20Camera _output_get))))
  (Development|PrintString "CameraEnterEdge!")
  (bind _returnvalue (Utilities|Time|SetTimerbyEvent (EventDispatchers|CreateEvent :!event Custom|CameraChangeLenght) 0.01 true))
  (Variables|Default|SetCameraOverlapTimer _returnvalue))