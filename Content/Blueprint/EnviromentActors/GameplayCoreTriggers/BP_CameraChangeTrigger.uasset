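; BP_CameraChangeTrigger is a box volume, sized in the construction script, that zooms the arena player's camera while the player is inside it.
; Entering while active starts the zoom with the trigger's ZoomValue; exiting ends it only if the player overlaps no other camera trigger.
; ChangeTriggerState toggles the trigger and applies or ends zoom for players already inside.
; It also runs one second after BeginPlay to apply the initial state.
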(event OnComponentBeginOverlap(Box)
  (params (OverlappedComponent :type Primitive%20Component%20Object%20Reference) (OtherActor :type Actor%20Object%20Reference) (OtherComp :type Primitive%20Component%20Object%20Reference) (OtherBodyIndex :type Integer) (bFromSweep :type Boolean) (SweepResult :type Hit%20Result%20Structure%20%28by%20ref%29))
  (bind (_asbp_player_arena_character _bsuccess) (Utilities|Casting|CastToBP_PlayerArenaCharacter OtherActor))
  (if (and _bsuccess (Variables|Default|GetIsActive))
    (Default|StartCameraZoom _asbp_player_arena_character (Variables|Default|GetZoomValue))))

(event OnComponentEndOverlap(Box)
  (params (OverlappedComponent :type Primitive%20Component%20Object%20Reference) (OtherActor :type Actor%20Object%20Reference) (OtherComp :type Primitive%20Component%20Object%20Reference) (OtherBodyIndex :type Integer))
  (bind (_asbp_player_arena_character _bsuccess) (Utilities|Casting|CastToBP_PlayerArenaCharacter OtherActor))
  (if (and _bsuccess (not (> (Utilities|Array|Length (Collision|GetOverlappingActors OtherActor "BP_CameraChangeTrigger_C" :!class /Script/Engine.Actor)) 0)))
    (Default|EndCameraZoom _asbp_player_arena_character)))

(event EventBeginPlay
  (Utilities|FlowControl|Delay 1.0)
  (CallFunction|ChangeTriggerState (Variables|Default|GetIsActive)))

(fn ConstructionScript
  (Components|Box|SetBoxExtent (Variables|Default|GetBox) (Variables|Default|GetBoxSize) true))

(fn ChangeTriggerState
  (params (IsActive :type Boolean))
  (Variables|Default|SetIsActive IsActive)
  (for _array_element (Collision|GetOverlappingActors (Variables|Default|GetBox) "/Game/Blueprint/Core/BP_PlayerArenaCharacter.BP_PlayerArenaCharacter_C" :!class /Script/Engine.PrimitiveComponent)
    (if (Variables|Default|GetIsActive)
      (Default|StartCameraZoom (.AsBP%20Player%20Arena%20Character (Utilities|Casting|CastToBP_PlayerArenaCharacter _array_element)) (Variables|Default|GetZoomValue))
      (else
        (Default|EndCameraZoom (.AsBP%20Player%20Arena%20Character (Utilities|Casting|CastToBP_PlayerArenaCharacter _array_element)))))))