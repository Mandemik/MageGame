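; BP_MapChangeTrigger is a box trigger that moves the player to another level.
; When the player arena character overlaps the box and the game instance is not already loading a map, it tries to finish the "Reach" quest objective.
; It then calls SwitchMap on the game instance with the configured level name.
; The construction script shows that level name on a text render component.
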(event OnComponentBeginOverlap(Box)
  (params (OverlappedComponent :type Primitive%20Component%20Object%20Reference) (OtherActor :type Actor%20Object%20Reference) (OtherComp :type Primitive%20Component%20Object%20Reference) (OtherBodyIndex :type Integer) (bFromSweep :type Boolean) (SweepResult :type Hit%20Result%20Structure%20%28by%20ref%29))
  (bind _returnvalue (Game|GetGameInstance))
  (bind (_asbp_player_arena_character _bsuccess) (Utilities|Casting|CastToBP_PlayerArenaCharacter OtherActor))
  (bind (_asbp_game_instance _bsuccess_2) (Utilities|Casting|CastToBP_GameInstance _returnvalue))
  (if (Math|Boolean|ANDBoolean _bsuccess _bsuccess_2 (not (Variables|/Game/Blueprint/Core/BP_GameInstance.BP_GameInstance_C|GetLoadNewMap _asbp_game_instance)))
    (Default|TryFinishObjective (Variables|Default|GetManager_QuestTarget) "Reach" _asbp_player_arena_character)
    (Default|SwitchMap _asbp_game_instance (Variables|Default|GetLevel%20Name%20To%20Load) false "None")))

(fn ConstructionScript
  (Rendering|Components|TextRender|SetText (Variables|Default|GetTextRender) (Utilities|Text|ToText(Name) (Variables|Default|GetLevel%20Name%20To%20Load))))