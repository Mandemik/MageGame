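; BP_Gore_BloodDeath is a gore actor that places an animated blood decal beneath a character when it spawns, apparently on death.
; On BeginPlay it spawns a downward-projecting decal with random yaw at the owner mesh's spine_02 socket.
; It then creates a dynamic material instance for the decal and drives its Dissolve parameter from a timeline curve played at half speed.
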(event EventBeginPlay
  (bind _returnvalue (Rendering|Decal|SpawnDecalatLocation (Variables|Default|GetDecalRef) "64.000000,128.000000,128.000000" (Transformation|GetSocketLocation (Variables|/Script/Engine.Character|GetMesh (Variables|Default|GetOwnerRef)) "spine_02") (Math|Rotator|MakeRotator 0.0 -9e+01 (Math|Random|RandomFloatinRange -1.8e+02 1.8e+02)) 0.0))
  (Utilities|IsValid _returnvalue
    (:Is%20Valid
      (bind _returnvalue_2 (Rendering|Material|CreateDynamicMaterialInstance _returnvalue :!class /Script/Engine.DecalComponent))
      (Variables|Default|SetBloodDecalDynamic _returnvalue_2)
      (Components|Timeline|SetPlayRate (Variables|Decal|GetDecal) 0.5)
      (bind _curve (Timeline|Decal PlayFromStart)
        (:Update
          (bind _blooddecaldynamic (Variables|Default|GetBloodDecalDynamic)
            (:then
              (Rendering|Material|SetScalarParameterValue _blooddecaldynamic "Dissolve" _curve :!class /Script/Engine.MaterialInstanceDynamic))
            (:else)))))))

(fn ConstructionScript)