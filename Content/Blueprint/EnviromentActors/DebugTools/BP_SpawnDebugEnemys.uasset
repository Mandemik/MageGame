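; BP_SpawnDebugEnemys is a debug trigger actor that spawns enemies when the player walks into its box.
; On overlap by BP_PlayerCharacter, it spawns an AI of the EnemyToSpawn class at the transform of each actor in SpawnArray.
; The construction script previews the chosen enemy by setting the skeletal mesh from SkeletonMeshMap, falling back to the Mixamo mannequin.
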(event OnComponentBeginOverlap(Box)
  (params (OverlappedComponent :type Primitive%20Component%20Object%20Reference) (OtherActor :type Actor%20Object%20Reference) (OtherComp :type Primitive%20Component%20Object%20Reference) (OtherBodyIndex :type Integer) (bFromSweep :type Boolean) (SweepResult :type Hit%20Result%20Structure%20%28by%20ref%29))
  (if (.bSuccess (Utilities|Casting|CastToBP_PlayerCharacter OtherActor))
    (for _array_element (Variables|Default|GetSpawnArray)
      (AI|SpawnAIFromClass (Variables|Default|GetEnemyToSpawn) 0 (.location (Transformation|GetActorTransform _array_element)) (.rotation (Transformation|GetActorTransform _array_element)) false 0))))

(fn ConstructionScript
  (bind _skeletonmeshmap (Variables|Default|GetSkeletonMeshMap))
  (bind _enemytospawn (Variables|Default|GetEnemyToSpawn))
  (bind (_value _returnvalue) (Utilities|Map|Find _skeletonmeshmap _enemytospawn))
  (Class|SkinnedMeshComponent|SetSkeletalMesh (Variables|Default|GetSkeletalMesh) (select _returnvalue _value "/Game/Animation/Base/UE4_Mixamo_Mannequin.UE4_Mixamo_Mannequin") true))