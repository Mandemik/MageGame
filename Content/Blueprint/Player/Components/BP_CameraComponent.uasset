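; Player camera component that tracks a target rotation for the owning BP_PlayerCharacter's camera boom.
; On BeginPlay it caches the player and the boom's starting rotation, printing a warning for any other owner.
; Fixed-step left/right and mouse X events adjust the stored rotation, then call StartCameraMove on the player.
; ComponentLoaded applies the stored rotation directly to the boom.
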(event Custom|RotateCameraToRight
  (Variables|Default|SetFinalRotation (Math|Rotator|CombineRotators (Variables|Default|GetFinalRotation) "0,10.000000, 0"))
  (Default|StartCameraMove (Variables|Default|GetPlayerRef)))

(event Custom|RotateCameraByMouseX
  (params (InputX :type Float%20%28single-precision%29))
  (Variables|Default|SetFinalRotation (Math|Rotator|CombineRotators (Variables|Default|GetFinalRotation) (Math|Rotator|MakeRotator 0.0 0.0 InputX)))
  (Default|StartCameraMove (Variables|Default|GetPlayerRef)))

(event Custom|RotateCameraToLeft
  (Variables|Default|SetFinalRotation (Math|Rotator|CombineRotators (Variables|Default|GetFinalRotation) "0,-10.000000, 0"))
  (Default|StartCameraMove (Variables|Default|GetPlayerRef)))

(event EventComponentLoaded
  (Transformation|SetRelativeRotation (Variables|/Game/Blueprint/Core/BP_PlayerCharacter.BP_PlayerCharacter_C|GetCameraBoom (Variables|Default|GetPlayerRef)) (Variables|Default|GetFinalRotation) false false))

(event EventBeginPlay
  (bind _asbp_player_character (Utilities|Casting|CastToBP_PlayerCharacter (Components|GetOwner))
    (:then
      (Variables|Default|SetPlayerRef _asbp_player_character)
      (Variables|Default|SetFinalRotation (Variables|/Script/Engine.SceneComponent|GetRelativeRotation (Variables|/Game/Blueprint/Core/BP_PlayerCharacter.BP_PlayerCharacter_C|GetCameraBoom (Variables|Default|GetPlayerRef)))))
    (:CastFailed
      (Development|PrintString "Wrong Parent Class"))))