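; Dialogue component that opens a custom dialogue widget for the player character that owns it.
; On BeginPlay it caches the owner as BP_PlayerCharacter.
; ShowDialoguWidget creates the widget from DialogueFiles with itself as NPCActor, binds its close delegate, switches to UI-only input and hides the HUD.
; OnDialogueClose is empty; the logic restoring AI focus, game-and-UI input and HUD visibility is disconnected and never runs.
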(event Custom|ShowDialoguWidget
  (bind _returnvalue (UserInterface|CreateWidget "/Game/UI/Dialogue/W_CustomDialogueWidget.W_CustomDialogueWidget_C" 0 (Variables|Default|GetDialogueFiles) self))
  (UserInterface|Viewport|AddtoViewport _returnvalue 0)
  (EventDispatchers|BindEventtoOnDialogueClose _returnvalue (EventDispatchers|CreateEvent :!event Custom|OnDialogueClose))
  (Input|SetInputModeUIOnly (.AsPlayer%20Controller (Utilities|Casting|CastToPlayerController (Pawn|GetController (Variables|Default|GetPlayerRef)))) _returnvalue "DoNotLock")
  (Widget|SetVisibility (Variables|/Game/Blueprint/Core/BP_PlayerCharacter.BP_PlayerCharacter_C|GetHudRef (Variables|Default|GetPlayerRef)) "Hidden"))

(event Custom|OnDialogueClose
  (params (Dialogue :type Dialogue%20Object%20Reference) (NPCActor :type Actor%20Object%20Reference)))

(event EventBeginPlay
  (bind _asbp_player_character (Utilities|Casting|CastToBP_PlayerCharacter (Components|GetOwner)))
  (Variables|Default|SetPlayerRef _asbp_player_character))