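; Zombie AI Blueprint that chases the player and applies a suicide gameplay effect to itself after a fixed time.
; On BeginPlay it runs parent logic, waits briefly, then issues a single simple move-to-actor order toward the first player character through its AI controller.
; After a further delay it applies GE_Suicide to itself through its Ability System component, with no proximity check.
; Overlap and Tick events are disabled.
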(event EventBeginPlay
  (|CallParentFunction)
  (Utilities|FlowControl|Delay 0.2)
  (AI|Navigation|SimpleMovetoActor (AI|GetAIController self) (Game|GetPlayerCharacter 0))
  (Utilities|FlowControl|Delay 5.0)
  (GameplayEffects|ApplyGameplayEffectToSelf :self (Variables|Default|GetAbilitySystemComp) :GameplayEffectClass "/Game/AbilitySystem/Ability/Common/GE_Suicide.GE_Suicide_C"))

(event Collision|EventActorBeginOverlap
  (params (OtherActor :type Actor%20Object%20Reference))
  (|CallParentFunction OtherActor) ; This node is disabled and will not be called.\nDrag off pins to build functionality.
)

(event EventTick
  (params (DeltaSeconds :type Float%20%28single-precision%29))
  (|CallParentFunction DeltaSeconds) ; This node is disabled and will not be called.\nDrag off pins to build functionality.
)

(fn ConstructionScript
  (|CallParentFunction))