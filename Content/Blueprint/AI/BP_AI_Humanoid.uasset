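; BP_AI_Humanoid is a humanoid AI character with a health bar widget and abilities granted from AIAbilities at BeginPlay.
; Taking damage reports a damage event at its location, likely for AI perception, and reveals the health bar on the first hit.
; On death it stops movement and brain logic, hides the widget, attempts an item drop through BPItemComponent, and expires after a set lifespan.
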(event EventBeginPlay
  (|CallParentFunction)
  (CallFunction|SetupAIWidget)
  (Class|BaseCharacter|InitializeAbilityMulti (Variables|Default|GetAIAbilities)))

(event EventAnyDamage
  (params (Damage :type Float%20%28single-precision%29) (DamageType :type Damage%20Type%20Object%20Reference) (InstigatedBy :type Controller%20Object%20Reference) (DamageCauser :type Actor%20Object%20Reference))
  (bind _self self)
  (|CallParentFunction Damage DamageType InstigatedBy DamageCauser)
  (Class|AISenseDamage|ReportDamageEvent _self DamageCauser Damage (Transformation|GetActorLocation _self) (Transformation|GetActorLocation) "None")
  (Utilities|FlowControl|DoOnce false
    (:Completed
      (Rendering|SetVisibility (Variables|Default|GetWidget) true false))))

(event EventCharacterDie
  (|CallParentFunction)
  (CallFunction|StopAILogic)
  (Actor|SetLifeSpan (Variables|Default|GetLifeSpanAfterDeath))
  (Rendering|SetVisibility (Variables|Default|GetWidget) false false)
  (Default|TryDropItem (Variables|Default|GetBP_ItemComponent)))

(fn ConstructionScript
  (|CallParentFunction))

(fn SetupAIWidget
  (bind _asw_aihealth_bar (Utilities|Casting|CastToW_AIHealthBar (UserInterface|GetWidget (Variables|Default|GetWidget))))
  (Variables|/Game/UI/W_AIHealthBar.W_AIHealthBar_C|SetAICharacterRef _asw_aihealth_bar self))

(fn StopAILogic
  (AI|Navigation|StopMovement (Pawn|GetController))
  (AI|Logic|StopLogic (Variables|/Script/AIModule.AIController|GetBrainComponent (AI|GetAIController self)) "AI is dead"))