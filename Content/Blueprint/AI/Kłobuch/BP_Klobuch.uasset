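; BP_Klobuch is the Kłobuch conversation NPC, which can start hidden and materialises when talked to.
; ShowUpKlobuch toggles visibility and the HideKlobuch flag with a dark-magic blink Niagara effect, paired with an entry sound on conversation events.
; Ending a conversation always hides it and tries to finish the "Talk" quest objective through ManagerQuestTarget.
; AnyDamage only prints a debug "Immortality" string.
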(event EventAnyDamage
  (params (Damage :type Float%20%28single-precision%29) (DamageType :type Damage%20Type%20Object%20Reference) (InstigatedBy :type Controller%20Object%20Reference) (DamageCauser :type Actor%20Object%20Reference))
  (Development|PrintString "Immortality"))

(event EventBeginPlay
  (|CallParentFunction)
  (if (Variables|Default|GetHideKlobuch)
    (Rendering|SetActorHiddenInGame true)))

(event EventConversationEnd
  (params (Dialogue :type Dialogue%20Object%20Reference) (NPCActor :type Actor%20Object%20Reference))
  (CallFunction|ShowUpKlobuch false)
  (Audio|PlaySoundatLocation "/Game/AUDIO/SFX/Klobuch/SFX_Klobuch_enter.SFX_Klobuch_enter" (Transformation|GetActorLocation) "0, 0, 0" 1.0 1.0 0.0 0 0 0 0)
  (|CallParentFunction Dialogue NPCActor)
  (Default|TryFinishObjective (Variables|Default|GetManager_QuestTarget) "Talk" (Variables|Default|GetCauserActor)))

(fn ConstructionScript
  (|CallParentFunction))

(fn ConversationStart
  (params (Causer :type BP%20Player%20Arena%20Character%20Object%20Reference))
  (if (Variables|Default|GetHideKlobuch)
    (CallFunction|ShowUpKlobuch true)
    (Audio|PlaySoundatLocation "/Game/AUDIO/SFX/Klobuch/SFX_Klobuch_enter.SFX_Klobuch_enter" (Transformation|GetActorLocation) "0, 0, 0" 1.0 1.0 0.0 0 0 0 0))
  (|CallParentFunction Causer))

(fn ShowUpKlobuch
  (params (On? :type Boolean))
  (bind _mesh (Variables|Character|GetMesh))
  (bind _returnvalue (not On?))
  (Niagara|SpawnSystematLocation "/Game/BlinkAndDashVFX/VFX_Niagara/NS_Blink_DarkMagic.NS_Blink_DarkMagic" (Transformation|GetWorldLocation _mesh) (Transformation|GetWorldRotation _mesh))
  (Rendering|SetActorHiddenInGame _returnvalue)
  (Variables|Default|SetHideKlobuch _returnvalue))