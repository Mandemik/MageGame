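; Zombie AI controller that runs BT_Zombie and stores the first player character as the blackboard Target on BeginPlay.
; AI perception updates about that player write the sensed state to the SeeTarget blackboard key.
; Each such update, whether sight is gained or lost, also plays a zombie grunt at the stimulus receiver location.
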(event OnTargetPerceptionUpdated(AIPerception)
  (params (Actor :type Actor%20Object%20Reference) (Stimulus :type AI%20Stimulus%20Structure))
  (if (== Actor (Variables|Default|GetPlayerRef))
    (AI|Components|Blackboard|SetValueasBool (Variables|Default|GetBlackboard) (Utilities|Name|MakeLiteralName "SeeTarget") (.bsuccessfullysensed Stimulus))
    (Audio|SpawnSoundatLocation "/Game/AUDIO/VO/Grunts/Zombie/Grunt_Zombie_Def_Cue.Grunt_Zombie_Def_Cue" (.receiverlocation Stimulus) "0, 0, 0" 1.0 1.0 0.0 0 0)))

(event EventBeginPlay
  (bind _returnvalue (Game|GetPlayerCharacter 0))
  (|CallParentFunction)
  (AI|RunBehaviorTree "/Game/Blueprint/AI/Zombie/BT_Zombie.BT_Zombie")
  (AI|Components|Blackboard|SetValueasObject (Variables|Default|GetBlackboard) (Utilities|Name|MakeLiteralName "Target") _returnvalue)
  (Variables|Default|SetPlayerRef _returnvalue))

(fn ConstructionScript
  (|CallParentFunction))