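; BP_AI_Bandit_Commander coordinates a shared alarm across the bandit AI in a level.
; On BeginPlay it binds an event to the alarm of each bandit in BanditArray, which FindAllBanditAtLevel fills by class search.
; CallAlarm fires once, switching every listed bandit to the Hostile team and reporting an AI noise event at the alarmed bandit's location.
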(event Custom|FindAllBanditAtLevel
  (bind _outactors (Actor|GetAllActorsOfClass "/Game/Blueprint/AI/Bandit/BP_AI_Bandit.BP_AI_Bandit_C"))
  (Variables|Default|SetBanditArray _outactors))

(event Custom|CallAlarm
  (params (BanditLocation :type Vector) (Instigator :type Actor%20Object%20Reference))
  (Utilities|FlowControl|DoOnce false
    (:Completed
      (CallFunction|SetBanditasHostile)
      (Class|AISenseHearing|ReportNoiseEvent BanditLocation 2.0 Instigator 2e+03 "Ability"))))

(event Custom|SetBanditAsHostile
  (for _array_element (Variables|Default|GetBanditArray)
    (Default|ChangeTeam _array_element "Hostile")))

(event EventBeginPlay
  (for _array_element (Variables|Default|GetBanditArray)
    (EventDispatchers|BindEventtoBanditAlarm _array_element (EventDispatchers|CreateEvent :!event Custom|CallAlarm))))

(fn ConstructionScript)