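; Bandit AI Blueprint that reflects its team allegiance through its armor and weapon materials.
; Construction and team changes both run SetTeamMaterial, which picks Friendly, Neutral or Hostile materials for two mesh slots.
; Turning Hostile also equips the weapon, on top of the parent's team-change logic.
; CreateDynamicMaterial makes dynamic instances of materials on the mesh and its child mesh components, collecting them in MaterialArray.
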(event EventBeginPlay
  (|CallParentFunction))

(event EventAnyDamage
  (params (Damage :type Float%20%28single-precision%29) (DamageType :type Damage%20Type%20Object%20Reference) (InstigatedBy :type Controller%20Object%20Reference) (DamageCauser :type Actor%20Object%20Reference))
  (|CallParentFunction Damage DamageType InstigatedBy DamageCauser))

(fn ConstructionScript
  (|CallParentFunction)
  (CallFunction|SetTeamMaterial (Variables|Default|GetTeam)))

(fn ChangeTeam
  (params (NewTeam :type ETeamAttitude%20Enum :default "Friendly"))
  (|CallParentFunction NewTeam)
  (CallFunction|SetTeamMaterial NewTeam)
  (switch Utilities|FlowControl|Switch|SwitchonETeamAttitude NewTeam
    (:Hostile
      (CallFunction|EquipWeapon true))))

(fn SetTeamMaterial
  (params (NewTeam :type ETeamAttitude%20Enum :default "Friendly"))
  (bind _mesh (Variables|Character|GetMesh))
  (Rendering|Material|SetMaterial _mesh 1 (Utilities|Select :Index NewTeam :Friendly "/Game/UndeadPack/WarriorHero/Materials/MI_Armor_Friendly.MI_Armor_Friendly" :Neutral "/Game/UndeadPack/WarriorHero/Materials/MI_Armor_Neutral.MI_Armor_Neutral" :Hostile "/Game/UndeadPack/WarriorHero/Materials/MI_Armor_Hostile.MI_Armor_Hostile"))
  (Rendering|Material|SetMaterial _mesh 2 (Utilities|Select :Index NewTeam :Friendly "/Game/UndeadPack/WarriorHero/Materials/MI_Weapon_Friendly.MI_Weapon_Friendly" :Neutral "/Game/UndeadPack/WarriorHero/Materials/MI_Weapon_Neutral.MI_Weapon_Neutral" :Hostile "/Game/UndeadPack/WarriorHero/Materials/MI_Weapon_Hostile.MI_Weapon_Hostile")))

(fn CreateDynamicMaterial
  (bind _mesh (Variables|Character|GetMesh))
  (bind _children (Components|GetChildrenComponents _mesh false))
  (bind _output_get (LocalVariables|SetComponentArrey _children))
  (Utilities|Array|Add _output_get _mesh)
  (Utilities|Array|Add _children 0)
  (for _array_element (LocalVariables|GetComponentArrey)
    (bind _asmesh_component (Utilities|Casting|CastToMeshComponent _array_element))
    (for (_array_element_2 _array_index) (Rendering|Material|GetMaterials _asmesh_component)
      (bind _returnvalue (Rendering|Material|CreateDynamicMaterialInstance _asmesh_component _array_index _array_element_2 "None" :!class /Script/Engine.PrimitiveComponent))
      (Utilities|IsValid _returnvalue
        (:Is%20Valid
          (Utilities|Array|Add (Variables|Default|GetMaterialArray) _returnvalue))))))