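; AI controller for the goblin enemy that runs its behavior tree and reports whether it senses the player.
; On BeginPlay it starts BT_Goblin, writes player character 0 to the Target blackboard key and caches it.
; AI Perception updates for that player set the SeeTarget key to the stimulus's sensed state, while updates for other actors are ignored.
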(event OnTargetPerceptionUpdated(AIPerception)
  (params (Actor :type Actor%20Object%20Reference) (Stimulus :type AI%20Stimulus%20Structure))
  (if (== Actor (Variables|Default|GetPlayerRef))
    (AI|Components|Blackboard|SetValueasBool (Variables|Default|GetBlackboard) (Utilities|Name|MakeLiteralName "SeeTarget") (.bsuccessfullysensed Stimulus))))

(event EventBeginPlay
  (bind _returnvalue (Game|GetPlayerCharacter 0))
  (|CallParentFunction)
  (AI|RunBehaviorTree "/Game/Blueprint/AI/Goblin/BT_Goblin.BT_Goblin")
  (AI|Components|Blackboard|SetValueasObject (Variables|Default|GetBlackboard) (Utilities|Name|MakeLiteralName "Target") _returnvalue)
  (Variables|Default|SetPlayerRef _returnvalue))

(fn ConstructionScript
  (|CallParentFunction))