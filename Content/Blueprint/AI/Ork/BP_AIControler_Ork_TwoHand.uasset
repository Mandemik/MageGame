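; AI controller for the two-handed Ork enemy, which runs the BT_Ork_TwoHand behavior tree.
; On BeginPlay it writes the player character into the blackboard's Target key and caches it in PlayerRef, so the target does not depend on perception.
; The perception update event does nothing; disconnected nodes hold logic to retarget to the perceived actor and play a grunt sound on successful sensing.
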(event OnTargetPerceptionUpdated(AIPerception)
  (params (Actor :type Actor%20Object%20Reference) (Stimulus :type AI%20Stimulus%20Structure)))

(event EventBeginPlay
  (bind _returnvalue (Game|GetPlayerCharacter 0))
  (|CallParentFunction)
  (AI|RunBehaviorTree "/Game/Blueprint/AI/Ork/BT_Ork_TwoHand.BT_Ork_TwoHand")
  (AI|Components|Blackboard|SetValueasObject (Variables|Default|GetBlackboard) (Utilities|Name|MakeLiteralName "Target") _returnvalue)
  (Variables|Default|SetPlayerRef _returnvalue))

(fn ConstructionScript
  (|CallParentFunction))