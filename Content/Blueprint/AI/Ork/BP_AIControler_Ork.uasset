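; AI controller Blueprint for the Ork enemy that starts the BT_Ork behavior tree on BeginPlay.
; Its perception update event is bound but does nothing.
; Disconnected nodes remain that would set the blackboard Target to the sensed actor or the player character and play a grunt sound at the stimulus location, but they never run.
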(event OnTargetPerceptionUpdated(AIPerception)
  (params (Actor :type Actor%20Object%20Reference) (Stimulus :type AI%20Stimulus%20Structure)))

(event EventBeginPlay
  (|CallParentFunction)
  (AI|RunBehaviorTree "/Game/Blueprint/AI/Ork/BT_Ork.BT_Ork"))

(fn ConstructionScript
  (|CallParentFunction))