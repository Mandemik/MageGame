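; Talking NPC child Blueprint that lets the player start a dialogue with it.
; Sphere overlaps tell BP_PlayerCharacter whether it can interact and toggle a widget on the NPC.
; Interacting opens W_CustomDialogueWidget with TestingDialogue, switches to UI-only input, hides the HUD and focuses the AI controller on the player.
; ConversationEnd clears that focus and restores game-and-UI input and the HUD.
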(event OnComponentBeginOverlap(Sphere)
  (params (OverlappedComponent :type Primitive%20Component%20Object%20Reference) (OtherActor :type Actor%20Object%20Reference) (OtherComp :type Primitive%20Component%20Object%20Reference) (OtherBodyIndex :type Integer) (bFromSweep :type Boolean) (SweepResult :type Hit%20Result%20Structure%20%28by%20ref%29))
  (bind _asbp_player_character (Utilities|Casting|CastToBP_PlayerCharacter OtherActor))
  (Development|PrintString (Utilities|String|Append (Utilities|GetDisplayName OtherActor) " overlap  Start with me"))
  (Class|BPInteractionInterface|CanInteractwithMe(Message) _asbp_player_character true self)
  (Rendering|SetVisibility (Variables|Default|GetWidget1) true false))

(event OnComponentEndOverlap(Sphere)
  (params (OverlappedComponent :type Primitive%20Component%20Object%20Reference) (OtherActor :type Actor%20Object%20Reference) (OtherComp :type Primitive%20Component%20Object%20Reference) (OtherBodyIndex :type Integer))
  (bind _asbp_player_character (Utilities|Casting|CastToBP_PlayerCharacter OtherActor))
  (Development|PrintString (Utilities|String|Append (Utilities|GetDisplayName OtherActor) " overlap  End with me"))
  (Class|BPInteractionInterface|CanInteractwithMe(Message) _asbp_player_character false)
  (Rendering|SetVisibility (Variables|Default|GetWidget1) false false))

(event Custom|ConversationEnd
  (params (Dialogue :type Dialogue%20Object%20Reference) (NPCActor :type Actor%20Object%20Reference))
  (bind _causer (Variables|Default|GetCauser))
  (AI|SetFocus (AI|GetAIController self))
  (Input|SetInputModeGameandUI (.AsPlayer%20Controller (Utilities|Casting|CastToPlayerController (Pawn|GetController (Variables|Default|GetCauser)))) (Variables|/Game/Blueprint/Core/BP_PlayerCharacter.BP_PlayerCharacter_C|GetHudRef _causer) "DoNotLock" true)
  (Widget|SetVisibility (Variables|/Game/Blueprint/Core/BP_PlayerCharacter.BP_PlayerCharacter_C|GetHudRef _causer) "Visible"))

(event EventInteractwithObject
  (params (InteractCauser :type BP%20Player%20Character%20Object%20Reference))
  (Variables|Default|SetCauser InteractCauser)
  (Development|PrintString "Interact")
  (bind _returnvalue (UserInterface|CreateWidget "/Game/UI/Dialogue/W_CustomDialogueWidget.W_CustomDialogueWidget_C" (.AsPlayer%20Controller (Utilities|Casting|CastToPlayerController (Pawn|GetController InteractCauser))) "/Game/Blueprint/Dialogue/TestingDialogue.TestingDialogue" self))
  (UserInterface|Viewport|AddtoViewport _returnvalue 0)
  (EventDispatchers|BindEventtoOnDialogueClose _returnvalue (EventDispatchers|CreateEvent :!event Custom|ConversationEnd))
  (Input|SetInputModeUIOnly (.AsPlayer%20Controller (Utilities|Casting|CastToPlayerController (Pawn|GetController (Variables|Default|GetCauser)))) _returnvalue "DoNotLock")
  (AI|SetFocus (AI|GetAIController self) (Variables|Default|GetCauser))
  (Widget|SetVisibility (Variables|/Game/Blueprint/Core/BP_PlayerCharacter.BP_PlayerCharacter_C|GetHudRef (Variables|Default|GetCauser)) "Hidden"))

(fn ConstructionScript
  (|CallParentFunction))