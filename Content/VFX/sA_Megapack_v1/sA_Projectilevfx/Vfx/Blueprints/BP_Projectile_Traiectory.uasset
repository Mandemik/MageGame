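; Projectile actor from a VFX pack that deals explosive damage on impact, with configurable Niagara trail and hit effects.
; BeginPlay assigns both effect assets to their components.
; The actor Hit event pushes physics bodies along its velocity and applies flat damage to BP_Humanoid pawns within ExplosionRadius.
; Sphere1's hit handler swaps trail for impact effect, disables collision, removes the light and destroys the actor after a short delay.
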(event OnComponentHit(Sphere1)
  (params (HitComponent :type Primitive%20Component%20Object%20Reference) (OtherActor :type Actor%20Object%20Reference) (OtherComp :type Primitive%20Component%20Object%20Reference) (NormalImpulse :type Vector :default "0, 0, 0") (Hit :type Hit%20Result%20Structure%20%28by%20ref%29))
  (bind _hiteffects (Variables|Default|GetHiteffects))
  (Components|Activation|Deactivate (Variables|Default|GetProjectileEffect))
  (Components|Activation|SetActive _hiteffects true false)
  (Transformation|SetWorldLocation _hiteffects (.Location (Collision|BreakHitResult Hit)) false false)
  (Collision|SetCollisionEnabled (Variables|Default|GetSphere1) "NoCollision")
  (Components|DestroyComponent (Variables|Default|GetPointLight))
  (Utilities|FlowControl|Delay 1.0)
  (Actor|DestroyActor))

(event EventBeginPlay
  (Class|NiagaraComponent|SetAsset (Variables|Default|GetProjectileEffect) (Variables|Default|GetProjectilefx) true)
  (Class|NiagaraComponent|SetAsset (Variables|Default|GetHiteffects) (Variables|Default|GetHitEffect) true))

(event Collision|EventHit
  (params (MyComp :type Primitive%20Component%20Object%20Reference) (Other :type Actor%20Object%20Reference) (OtherComp :type Primitive%20Component%20Object%20Reference) (bSelfMoved :type Boolean) (HitLocation :type Vector :default "0, 0, 0") (HitNormal :type Vector :default "0, 0, 0") (NormalImpulse :type Vector :default "0, 0, 0") (Hit :type Hit%20Result%20Structure%20%28by%20ref%29))
  (if (Physics|IsSimulatingPhysics OtherComp "None")
    (Physics|AddImpulseatLocation OtherComp (* (Transformation|GetVelocity) 1e+02) (Transformation|GetActorLocation) "None"))
  (bind _outactors (Collision|SphereOverlapActors (Transformation|GetActorLocation) (Variables|Default|GetExplosionRadius) (Utilities|Array|MakeArray "ObjectTypeQuery3") "/Game/Blueprint/Core/BP_Humanoid.BP_Humanoid_C"))
  (for _array_element _outactors
    (Game|Damage|ApplyDamage _array_element 1e+02 0 (Variables|Actor|GetInstigator)))
  (Actor|SetLifeSpan 3.0))

(fn ConstructionScript)