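; Gameplay ability for the Toxic status on a humanoid, dealing periodic damage credited to the instigator of the granting effect.
; A looping timer drives the damage until the ability ends.
; Gaining Status.InFire triggers a one-off explosion with extra damage, tinted Niagara burst and camera shake for player-controlled victims.
; After a short placeholder delay, it removes the fire effects and its own granting effect, so the reaction consumes both statuses.
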(event Custom|ApplyToxicDamage
  (bind _characterref (Variables|Default|GetCharacterRef))
  (Game|Damage|ApplyDamage _characterref (Variables|Default|GetBase%20Damage) (Variables|Default|GetIntigatorControler) _characterref "/Script/Engine.DamageType"))

(event Custom|SpawnToxicExplosion
  (bind _characterref (Variables|Default|GetCharacterRef))
  (Game|Damage|ApplyDamage _characterref (Variables|Default|GetToxicExplosionDamage) (Variables|Default|GetIntigatorControler) _characterref "/Script/Engine.DamageType")
  (bind _returnvalue (Niagara|SpawnSystematLocation "/Game/VFX/sA_Megapack_v1/sA_StylizedAttacksPack/FX/NiagaraSystems/NS_BasicHit.NS_BasicHit" (Transformation|GetActorLocation (Variables|Default|GetCharacterRef)) "0, 0, 0" "10.000000,10.000000,10.000000"))
  (Effects|Components|ParticleSystem|SetColorParameter _returnvalue "Color" "(R=5.000000,G=0.351182,B=0.000000,A=1.000000)")
  (bind _asplayer_controller (Utilities|Casting|CastToPlayerController (Pawn|GetController (Variables|Default|GetCharacterRef))))
  (Class|MatineeCameraShake|StartMatineeCameraShake (Variables|/Script/Engine.PlayerController|GetPlayerCameraManager _asplayer_controller) "/Game/AbilitySystem/Status/Toxic/CS_ToxicExplosion.CS_ToxicExplosion_C" 1.0 "CameraLocal" "0, 0, 0"))

(event Ability|EventActivateAbility
  (CallFunction|SetVariables)
  (bind _returnvalue (Utilities|Time|SetTimerbyEvent (EventDispatchers|CreateEvent :!event Custom|ApplyToxicDamage) 0.5 true))
  (Variables|Default|SetRegenerationLoopTimer _returnvalue)
  (Ability|Tasks|WaitGameplayTagAdd "(TagName=\"Status.InFire\")" 0 true
    (:Added
      (CallFunction|SpawnToxicExplosion)
      ;[1 1 1] TODO - Do it properly
      (Utilities|FlowControl|Delay 0.2)
      (Ability|RemoveGameplayEffectFromOwnerWithGrantedTags "(GameplayTags=((TagName=\"Status.InFire\")))")
      (Ability|RemoveGrantedbyEffect))))

(event Ability|EventOnEndAbility
  (params (bWasCancelled :type Boolean))
  (Utilities|Time|ClearandInvalidateTimerbyHandle (Variables|Default|GetRegenerationLoopTimer)))

(fn SetVariables
  (bind _asbp_humanoid (Utilities|Casting|CastToBP_Humanoid (.owneractor (Ability|GetActorInfo)))
    (:then
      (Variables|Default|SetCharacterRef _asbp_humanoid)
      (bind _aspawn (Utilities|Casting|CastToPawn (Class|AbilitySystemBlueprintLibrary|EffectContextGetInstigatorActor (Ability|GetGrantedbyEffectContext)))
        (:then
          (Variables|Default|SetIntigatorControler (Pawn|GetController _aspawn)))
        (:CastFailed
          (Development|PrintString (Utilities|String|Append "WARNING: Wrong instigator in " (Utilities|GetDisplayName self))))))
    (:CastFailed
      (Development|PrintString (Utilities|String|Append "WARNING: Wrong Character in " (Utilities|GetDisplayName self))))))