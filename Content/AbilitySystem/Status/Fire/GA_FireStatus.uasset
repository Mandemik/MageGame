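; Gameplay ability for the fire status, dealing periodic damage to the BP_Humanoid that owns it.
; On activation it caches that character and the controller of the granting effect's instigator pawn, printing warnings if either cast fails.
; A looping half-second timer drives the damage, credited to that controller with the victim as damage causer.
; Ending the ability clears the timer.
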(event Custom|ApplyFireDamae
  (bind _characterref (Variables|Default|GetCharacterRef))
  (Game|Damage|ApplyDamage _characterref (Variables|Default|GetBase%20Damage) (Variables|Default|GetIntigatorControler) _characterref))

(event Ability|EventActivateAbility
  (CallFunction|SetVariables)
  (bind _returnvalue (Utilities|Time|SetTimerbyEvent (EventDispatchers|CreateEvent :!event Custom|ApplyFireDamae) 0.5 true))
  (Variables|Default|SetRegenerationLoopTimer _returnvalue))

(event Ability|EventOnEndAbility
  (params (bWasCancelled :type Boolean))
  (Utilities|Time|ClearandInvalidateTimerbyHandle (Variables|Default|GetRegenerationLoopTimer)))

(fn SetVariables
  (bind _asbp_humanoid (Utilities|Casting|CastToBP_Humanoid (.owneractor (Ability|GetActorInfo)))
    (:then
      (Variables|Default|SetCharacterRef _asbp_humanoid)
      (bind _aspawn (Utilities|Casting|CastToPawn (Class|AbilitySystemBlueprintLibrary|EffectContextGetInstigatorActor (Ability|GetGrantedbyEffectContext)))
        (:then
          (Variables|Default|SetIntigatorControler (Pawn|GetController _aspawn)))
        (:CastFailed
          (Development|PrintString (Utilities|String|Append "WARNING: Wrong instigator in " (Utilities|GetDisplayName self))))))
    (:CastFailed
      (Development|PrintString (Utilities|String|Append "WARNING: Wrong Character in " (Utilities|GetDisplayName self))))))