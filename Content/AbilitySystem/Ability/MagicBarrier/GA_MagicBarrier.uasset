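; GA_MagicBarrier is a gameplay ability that sustains a defensive magic barrier on the player at a recurring mana cost.
; On activation it spawns BP_MagicBarrier, attaches it to the pelvis socket, plays the barrier montage and starts a looping cost timer.
; A failed cost commit or the player releasing defensive ability input clears the timer, destroys the sphere and plays the EndSkill montage section before ending the ability.
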(event Custom|PlayerChangeInput
  (params (WannaUse :type Boolean))
  (if (not WannaUse)
    (CallFunction|PreEndAbility)))

(event Custom|ApplyCostAndCheck
  (bind _returnvalue (Ability|CommitAbilityCost false))
  (if (not _returnvalue)
    (CallFunction|PreEndAbility)))

(event Custom|PreEndAbility
  (Utilities|Time|ClearandInvalidateTimerbyHandle (Variables|Default|GetPayManaCostTask))
  (Default|DestroySphere (Variables|Default|GetMagicSphereRef))
  (Animation|Montage|PlayMontage (Variables|/Script/Engine.Character|GetMesh (Variables|Default|GetPlayerRef)) "/Game/Animation/MagPacket/AM_MagicBarrier.AM_MagicBarrier" 1.0 0.0 "EndSkill"
    (:OnCompleted
      _)
    (:OnInterrupted
      _))
  (Ability|EndAbility))

(event Ability|EventActivateAbility
  (CallFunction|SetVariables)
  (bind _spawnedactor (|SpawnActor :Class "/Game/AbilitySystem/Ability/MagicBarrier/BP_MagicBarrier.BP_MagicBarrier_C" :Instigator 0)
    (:then
      (bind _returnvalue (Utilities|Time|SetTimerbyEvent (EventDispatchers|CreateEvent :!event Custom|ApplyCostAndCheck) (Variables|Default|GetManaCostFrequence) true))
      (Variables|Default|SetPayManaCostTask _returnvalue)
      (Animation|Montage|PlayMontage (Variables|/Script/Engine.Character|GetMesh (Variables|Default|GetPlayerRef)) "/Game/Animation/MagPacket/AM_MagicBarrier.AM_MagicBarrier"
        (:OnCompleted
          (Ability|EndAbility))))
    (:Success
      (bind _output_get (Variables|Default|SetMagicSphereRef (.AsBP%20Magic%20Barrier (Utilities|Casting|CastToBP_MagicBarrier _spawnedactor))))
      (Transformation|AttachComponentToComponent _output_get (Variables|/Script/Engine.Character|GetMesh (Variables|Default|GetPlayerRef)) "pelvis" "SnapToTarget" "KeepRelative" "KeepRelative" true))))

(fn SetVariables
  (bind _returnvalue (Ability|GetActorInfo))
  (bind _asbp_player_character (Utilities|Casting|CastToBP_PlayerCharacter (.owneractor _returnvalue)))
  (Variables|Default|SetPlayerRef _asbp_player_character)
  (bind _asbp_custom_player_controler (Utilities|Casting|CastToBP_CustomPlayerControler (.playercontroller _returnvalue)))
  (bind _output_get (Variables|Default|SetPlayerControlerRef _asbp_custom_player_controler))
  (EventDispatchers|BindEventtoPlayerWannaUseDefenciveAbility _output_get (EventDispatchers|CreateEvent :!event Custom|PlayerChangeInput)))