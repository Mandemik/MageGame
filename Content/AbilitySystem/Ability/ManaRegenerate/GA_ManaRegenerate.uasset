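; Gameplay ability that regenerates the owning PlayerCharacter's mana over time while active.
; On activation it caches the player and starts a looping one-second timer, which is cleared when the ability ends.
; ApplyManaRegeneration applies GE_ManaRegeneratePerSec to the owner, passing a player attribute value as a SetByCaller magnitude under the Ability.ManaRegenerate.ApplyValue tag.
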(event Custom|ApplyManaRegeneration
  (bind _returnvalue (Ability|GameplayEffect|AssignTagSetbyCallerMagnitude (Ability|MakeOutgoingGameplayEffectSpec "/Game/AbilitySystem/Ability/ManaRegenerate/GE_ManaRegeneratePerSec.GE_ManaRegeneratePerSec_C") "(TagName=\"Ability.ManaRegenerate.ApplyValue\")" (.ReturnValue (Ability|Attribute|GetFloatAttribute (Variables|Default|GetPlayerRef) "(AttributeName=\"ManaRegeneration\",Attribute=/Script/MagBuildGame.BaseAttributeSet:ManaRegeneration,AttributeOwner=Class'\"/Script/MagBuildGame.BaseAttributeSet\"')"))))
  (Ability|ApplyGameplayEffectSpecToOwner _returnvalue))

(event Ability|EventActivateAbility
  (CallFunction|SetVariables)
  (bind _returnvalue (Utilities|Time|SetTimerbyEvent (EventDispatchers|CreateEvent :!event Custom|ApplyManaRegeneration) 1.0 true))
  (Variables|Default|SetRegenerationLoopTimer _returnvalue))

(event Ability|EventOnEndAbility
  (params (bWasCancelled :type Boolean))
  (Utilities|Time|ClearandInvalidateTimerbyHandle (Variables|Default|GetRegenerationLoopTimer)))

(fn SetVariables
  (bind _asbuilding_character (Utilities|Casting|CastToPlayerCharacter (.owneractor (Ability|GetActorInfo))))
  (Variables|Default|SetPlayerRef _asbuilding_character))