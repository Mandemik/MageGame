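; Player gameplay ability that casts a fireball toward the point under the mouse cursor.
; On activation it checks mana, applies the cost through a SetByCaller gameplay effect, commits the cooldown and plays a self-cast montage, ending immediately if mana is short.
; A montage notify spawns the projectile offset toward the cursor hit, rotated by yaw only.
; The ability ends when the montage completes or is interrupted.
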(event Ability|EventActivateAbility
  (CallFunction|SetVariables)
  (if (>= (.Mana (Class|BaseCharacter|GetManaValues (Variables|Default|GetPlayerRef))) (Variables|Default|GetManaCost))
    (CallFunction|ApplyManaCost)
    (Ability|CommitAbilityCooldown false)
    (bind _notifyname (Animation|Montage|PlayMontage (Variables|/Script/Engine.Character|GetMesh (Variables|Default|GetPlayerRef)) "/Game/Animation/MagPacket/AM_SelfCast.AM_SelfCast")
      (:OnCompleted
        (Ability|EndAbility :!label _label))
      (:OnInterrupted
        (goto _label))
      (:OnNotifyBegin
        (switch name _notifyname
          (:Cast
            (CallFunction|SpawnFireBall)))))
    (else
      (Ability|EndAbility))))

(event Ability|EventOnEndAbility
  (params (bWasCancelled :type Boolean)))

(fn SpawnFireBall
  (bind _playerref (Variables|Default|GetPlayerRef))
  (bind _returnvalue (Pawn|GetController _playerref))
  (bind _returnvalue_2 (Transformation|GetActorLocation _playerref))
  (bind _asplayer_controller (Utilities|Casting|CastToPlayerController _returnvalue))
  (bind _hitresult (Game|Player|GetHitResultUnderCursorbyChannel _asplayer_controller "TraceTypeQuery1" true))
  (bind _returnvalue_3 (Math|Rotator|FindLookatRotation _returnvalue_2 (.location _hitresult)))
  (Game|SpawnActorfromClass "/Game/VFX/sA_Megapack_v1/sA_Projectilevfx/Vfx/Blueprints/BP_Projectile_2_Small.BP_Projectile_2_Small_C" (Math|Transform|MakeTransform (+ (Transformation|GetActorLocation (Variables|Default|GetPlayerRef)) (* (Math|Vector|GetForwardVector (Math|Rotator|MakeRotator (.roll _returnvalue_3) (.pitch _returnvalue_3) (.yaw _returnvalue_3))) (Variables|Default|GetFireballOffset))) (Math|Rotator|MakeRotator 0.0 0.0 (.yaw _returnvalue_3))) "AdjustIfPossibleButDontSpawnIfColliding" 0 (Variables|Default|GetPlayerRef)) ; Spawn projectile
)

(fn SetVariables
  (bind _asbuilding_character (Utilities|Casting|CastToPlayerCharacter (.owneractor (Ability|GetActorInfo))))
  (Variables|Default|SetPlayerRef _asbuilding_character))

(fn ApplyManaCost
  (bind _result (Math|Float|NegateFloat (Variables|Default|GetManaCost))
    (:%20%20
      (bind _returnvalue (Ability|GameplayEffect|AssignTagSetbyCallerMagnitude (Ability|MakeOutgoingGameplayEffectSpec "/Game/AbilitySystem/Ability/Fireball/GE_Fireball_ManaCost.GE_Fireball_ManaCost_C") "(TagName=\"Ability.Fireball.ManaCost\")" _result))
      (Ability|ApplyGameplayEffectSpecToOwner _returnvalue))))