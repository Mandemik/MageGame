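; Fire Hand player ability that spawns a damaging hand collider on a montage notify.
; On activation it records the cursor hit, flags Destructible targets for precision aiming and turns the player toward the mouse.
; The notify plays the cast sound, reports AI noise, spawns the collider, then commits and ends the ability.
; GetSkillSlot is empty, and the aim-based transform math in CalculateSpawnTransform is left unconnected.
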(event Ability|EventActivateAbility
  (bind _returnvalue (Game|Player|GetPlayerPawn 0))
  (bind _returnvalue_2 (Transformation|GetActorLocation _returnvalue))
  (CallFunction|SetVariables)
  (CallFunction|FindAimLocation)
  (Default|EnableRotationtoMousePosition (Variables|Default|GetPlayerRef) true true 2.0)
  (bind _notifyname (Animation|Montage|PlayMontage (Variables|/Script/Engine.Character|GetMesh (Variables|Default|GetPlayerRef)) "/Game/Animation/WarriorAnimation/AM_SimpleHand.AM_SimpleHand" 2.0)
    (:OnCompleted
      (Ability|EndAbility :!label _label))
    (:OnInterrupted
      (goto _label))
    (:OnNotifyBegin
      (switch name _notifyname
        (:Cast
          (Audio|PlaySoundatLocation (Variables|Default|GetCastSound) _returnvalue_2 "0, 0, 0" 1.0 1.0 0.0 0 0 (Variables|Default|GetPlayerRef) 0)
          (Class|AISenseHearing|ReportNoiseEvent _returnvalue_2 1.0 (Variables|Default|GetPlayerRef) 1.5e+03 "Ability")
          (CallFunction|SpawnFireHandCollision)
          (Ability|CommitAbility)
          (Ability|EndAbility))))))

(fn SpawnFireHandCollision
  (Game|SpawnActorfromClass (Variables|Default|GetHandColliderActor) (Utilities|CalculateSpawnTransform) "Undefined" 0 (Variables|Default|GetBaseDamage) (Variables|Default|GetPlayerRef)))

(fn SetVariables
  (bind _asbp_player_character (Utilities|Casting|CastToBP_PlayerCharacter (.owneractor (Ability|GetActorInfo))))
  (Variables|Default|SetPlayerRef _asbp_player_character))

(fn GetSkillSlot)

(fn FindAimLocation
  (bind _array (Utilities|Array|MakeArray "ObjectTypeQuery1" "ObjectTypeQuery2" "ObjectTypeQuery6"))
  (bind _playerref (Variables|Default|GetPlayerRef))
  (bind _returnvalue (Pawn|GetController _playerref))
  (bind _asplayer_controller (Utilities|Casting|CastToPlayerController _returnvalue))
  (bind _hitresult (Class|PlayerController|GetHitResultUnderCursorforObjects _asplayer_controller _array true))
  (Variables|Default|SetHitAimLocation (.location _hitresult))
  (Variables|Default|SetPrecisionAiming (Utilities|Enum|Equal(Enum) (Collision|GetCollisionObjectType (.hitcomponent _hitresult)) "ECC_Destructible")))