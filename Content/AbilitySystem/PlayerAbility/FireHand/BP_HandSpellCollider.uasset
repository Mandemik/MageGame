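; BP_HandSpellCollider is a short-lived hit volume for the player's Fire Hand ability that damages humanoid AI and sets them on fire.
; Shortly after BeginPlay it takes a single snapshot of BP_AI_Humanoid actors overlapping its static mesh.
; Each gets point damage along the instigator's forward vector, then ApplyStatus applies the fire status.
; The actor destroys itself a couple of seconds later.
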(event EventBeginPlay
  (bind _instigator (Variables|Actor|GetInstigator))
  (Utilities|FlowControl|Delay 0.1)
  (for _array_element (Collision|GetOverlappingActors (Variables|Default|GetStaticMesh) "/Game/Blueprint/AI/BP_AI_Humanoid.BP_AI_Humanoid_C" :!class /Script/Engine.PrimitiveComponent)
    (Game|Damage|ApplyPointDamage _array_element (Variables|Default|GetBase%20Damage) (Transformation|GetActorForwardVector (Variables|Actor|GetInstigator)) (Collision|MakeHitResult false false 0.0 0.0 "0, 0, 0" "0, 0, 0" "0,0,1" "0,0,1" 0 0 0 "None" "None" 0 0 0 "0, 0, 0" "0, 0, 0") (Pawn|GetController _instigator) _instigator (Variables|Default|GetDamage%20Type%20Class))
    (CallFunction|ApplyStatus _instigator _array_element))
  (Utilities|FlowControl|Delay 2.0)
  (Actor|DestroyActor))

(fn ConstructionScript)

(fn ApplyStatus
  (params (InstigatorCharacter :type Actor%20Object%20Reference) (Target :type Actor%20Object%20Reference))
  (CallFunction|ApplyFire InstigatorCharacter Target))