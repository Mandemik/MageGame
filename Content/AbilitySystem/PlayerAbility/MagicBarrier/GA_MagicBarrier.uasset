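; Player gameplay ability for a held magic barrier that drains its cost over time.
; On activation it starts the skill slot's HUD cast animation, spawns BP_MagicBarrier attached to the pelvis, plays a montage and runs a looping cost timer.
; Input release or a failed cost commit triggers PreEndAbility, which stops the HUD animation and timer, destroys the sphere and plays the EndSkill montage section before ending.
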(event Custom|PlayerChangeInput
  (params (WannaUse :type Boolean))
  (if WannaUse
    _))

(event Custom|ApplyCostAndCheck
  (bind _returnvalue (Ability|CommitAbilityCost false))
  (if (not _returnvalue)
    (CallFunction|PreEndAbility)))

(event Custom|PreEndAbility
  (Default|StopCastAnimation (Variables|/Game/Blueprint/Core/BP_PlayerCharacter.BP_PlayerCharacter_C|GetHudRef (Variables|Default|GetPlayerRef)) (Variables|Default|GetSkillSlot))
  (Utilities|Time|ClearandInvalidateTimerbyHandle (Variables|Default|GetPayManaCostTask))
  (Utilities|IsValid (Variables|Default|GetMagicSphereRef)
    (:Is%20Valid
      (Default|DestroySphere (Variables|Default|GetMagicSphereRef)))
    (:Is%20Not%20Valid
      _))
  (Animation|Montage|PlayMontage (Variables|/Script/Engine.Character|GetMesh (Variables|Default|GetPlayerRef)) "/Game/Animation/MagPacket/AM_MagicBarrier.AM_MagicBarrier" 1.0 0.0 "EndSkill"
    (:OnCompleted
      _)
    (:OnInterrupted
      _))
  (Ability|EndAbility))

(event Ability|EventActivateAbility
  (CallFunction|SetVariables)
  (CallFunction|GetSkillSlot)
  (Default|StartCastAnimation (Variables|/Game/Blueprint/Core/BP_PlayerCharacter.BP_PlayerCharacter_C|GetHudRef (Variables|Default|GetPlayerRef)) (Variables|Default|GetSkillSlot))
  (bind _spawnedactor (|SpawnActor :Class "/Game/AbilitySystem/PlayerAbility/MagicBarrier/BP_MagicBarrier.BP_MagicBarrier_C" :Instigator 0)
    (:then
      (bind _returnvalue (Utilities|Time|SetTimerbyEvent (EventDispatchers|CreateEvent :!event Custom|ApplyCostAndCheck) (Variables|Default|GetManaCostFrequence) true))
      (Variables|Default|SetPayManaCostTask _returnvalue)
      (Animation|Montage|PlayMontage (Variables|/Script/Engine.Character|GetMesh (Variables|Default|GetPlayerRef)) "/Game/Animation/MagPacket/AM_MagicBarrier.AM_MagicBarrier"
        (:then
          (Ability|Tasks|WaitInputRelease false
            (:OnRelease
              (CallFunction|PreEndAbility))))
        (:OnCompleted
          (Ability|EndAbility))))
    (:Success
      (bind _output_get (Variables|Default|SetMagicSphereRef (.AsBP%20Magic%20Barrier (Utilities|Casting|CastToBP_MagicBarrier _spawnedactor))))
      (Transformation|AttachComponentToComponent _output_get (Variables|/Script/Engine.Character|GetMesh (Variables|Default|GetPlayerRef)) "pelvis" "SnapToTarget" "KeepRelative" "KeepRelative" true))))

(fn SetVariables
  (bind _returnvalue (Ability|GetActorInfo))
  (bind _asbp_player_character (Utilities|Casting|CastToBP_PlayerCharacter (.owneractor _returnvalue)))
  (Variables|Default|SetPlayerRef _asbp_player_character)
  (bind _asbp_custom_player_controler (Utilities|Casting|CastToBP_CustomPlayerControler (.playercontroller _returnvalue)))
  (Variables|Default|SetPlayerControlerRef _asbp_custom_player_controler))

(fn GetSkillSlot
  (bind _playerref (Variables|Default|GetPlayerRef))
  (bind _activeskills (Variables|/Game/Blueprint/Core/BP_PlayerCharacter.BP_PlayerCharacter_C|GetActiveSkills _playerref))
  (bind _keys (Utilities|Map|Keys _activeskills))
  (bind _array_element (Utilities|Array|ForEachLoopwithBreak _keys :!label _label)
    (:LoopBody
      (if (== (.Value (Utilities|Map|Find _activeskills _array_element)) (Utilities|GetClass self))
        (Variables|Default|SetSkillSlot _array_element)
        (goto _label Break)))))