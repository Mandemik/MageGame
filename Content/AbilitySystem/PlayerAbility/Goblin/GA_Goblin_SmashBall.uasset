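; Gameplay ability in which an AI Goblin throws a smash-ball projectile at its blackboard Target.
; On activation it pauses the AI's brain logic and plays the smash-ball montage, restarting the logic when the ability ends.
; A montage notify spawns BP_Projectile_Traiectory ahead of and above the projectile socket, yawed toward the target, and sets its velocity from the look-at plus an upward bias.
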(event Ability|EventActivateAbility
  (bind _goblinref (Variables|Default|GetGoblinRef))
  (bind _returnvalue (AI|GetAIController _goblinref))
  (CallFunction|SetVariables)
  (AI|Logic|StopLogic (Variables|/Script/AIModule.AIController|GetBrainComponent _returnvalue) "Playing Ability")
  (bind _asactor (Utilities|Casting|CastToActor (AI|Components|Blackboard|GetValueasObject (Variables|/Script/AIModule.AIController|GetBlackboard _returnvalue) (Utilities|Name|MakeLiteralName "Target")))
    (:then
      (Variables|Default|SetTarget _asactor)
      (bind _notifyname (Animation|Montage|PlayMontage (Variables|/Script/Engine.Character|GetMesh (Variables|Default|GetGoblinRef)) "/Game/UndeadPack/EnemyGoblin/Animations/AM_Goblin_SmashBall.AM_Goblin_SmashBall" 1.5)
        (:OnCompleted
          (Ability|EndAbility :!label _label))
        (:OnInterrupted
          (goto _label))
        (:OnNotifyBegin
          (switch name _notifyname
            (:SpawnProjectile
              (CallFunction|SpawnSmashBall))))))
    (:CastFailed
      (Ability|EndAbility))))

(event Ability|EventOnEndAbility
  (params (bWasCancelled :type Boolean))
  (bind _goblinref (Variables|Default|GetGoblinRef))
  (bind _returnvalue (AI|GetAIController _goblinref))
  (bind _braincomponent (Variables|/Script/AIModule.AIController|GetBrainComponent _returnvalue))
  (Utilities|IsValid _braincomponent
    (:Is%20Valid
      (AI|Logic|StartLogic _braincomponent))))

(fn SetVariables
  (bind _asbp_ai_goblin (Utilities|Casting|CastToBP_AI_Goblin (.owneractor (Ability|GetActorInfo)))
    (:then
      (Variables|Default|SetGoblinRef _asbp_ai_goblin))
    (:CastFailed
      (Ability|EndAbility))))

(fn SpawnSmashBall
  (bind _goblinref (Variables|Default|GetGoblinRef))
  (bind _target (Variables|Default|GetTarget))
  (bind _goblinref_2 (Variables|Default|GetGoblinRef))
  (bind _projectialoffset (Variables|Default|GetProjectialOffset))
  (bind _returnvalue (Transformation|GetActorLocation _target))
  (bind _mesh (Variables|/Script/Engine.Character|GetMesh _goblinref))
  (bind _returnvalue_2 (Transformation|GetSocketLocation _mesh "ProjectileSocket"))
  (bind _returnvalue_3 (Math|Rotator|FindLookatRotation _returnvalue_2 _returnvalue))
  (bind _returnvalue_4 (+ _returnvalue_2 "0,0,50.000000"))
  (bind _returnvalue_5 (Math|Vector|GetForwardVector (Math|Rotator|MakeRotator 0.0 0.0 (.yaw _returnvalue_3))))
  (bind _returnvalue_6 (* _returnvalue_5 _projectialoffset))
  (bind _returnvalue_7 (+ _returnvalue_4 _returnvalue_6))
  (bind _returnvalue_8 (Math|Transform|MakeTransform _returnvalue_7 (Math|Rotator|MakeRotator 0.0 0.0 (.yaw _returnvalue_3))))
  (bind _returnvalue_9 (Game|SpawnActorfromClass "/Game/VFX/sA_Megapack_v1/sA_Projectilevfx/Vfx/Blueprints/BP_Projectile_Traiectory.BP_Projectile_Traiectory_C" (Math|Transform|MakeTransform (.location _returnvalue_8) (.rotation _returnvalue_8) "1.000000,1.000000,1.000000") "AdjustIfPossibleButAlwaysSpawn" 0 (Variables|Default|GetGoblinRef))) ; Spawn projectile
  (Variables|/Script/Engine.MovementComponent|SetVelocity (Variables|/Game/VFX/sA_Megapack_v1/sA_Projectilevfx/Vfx/Blueprints/BP_Projectile_Traiectory.BP_Projectile_Traiectory_C|GetProjectile _returnvalue_9) (* (+ (Math|Rotator|FindLookatRotation (Transformation|GetActorLocation _goblinref_2) (Transformation|GetActorLocation (Variables|Default|GetTarget))) (* (Transformation|GetActorUpVector _goblinref_2) 2.0)) 4.5e+02)))