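; Gameplay ability that lets a humanoid AI advance on its blackboard target behind a spawned shield at a fixed walk speed.
; On activation it attaches BP_ShieldBlock to the pelvis, commits the cooldown and starts AIMoveTo, alongside a looping mana-cost timer.
; When the move finishes or fails, PreEndAbility clears the timer, destroys the shield sphere, restores the original speed and ends the ability.
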(event Custom|PreEndAbility
  (Utilities|Time|ClearandInvalidateTimerbyHandle (Variables|Default|GetPayManaCostTask))
  (Utilities|IsValid (Variables|Default|GetShieldRef)
    (:Is%20Valid
      (Default|DestroySphere (Variables|Default|GetShieldRef))
      (Variables|/Script/Engine.CharacterMovementComponent|SetMaxWalkSpeed (Variables|/Script/Engine.Character|GetCharacterMovement (Variables|Default|GetAIRef)) (Variables|Default|GetStartingWalkSpeed)))
    (:Is%20Not%20Valid
      _))
  (Ability|EndAbility))

(event Ability|EventActivateAbility
  (bind _airef (Variables|Default|GetAIRef))
  (bind _charactermovement (Variables|/Script/Engine.Character|GetCharacterMovement _airef))
  (CallFunction|SetVariables)
  (bind _spawnedactor (|SpawnActor :Class "/Game/AbilitySystem/PlayerAbility/ShieldBlock/BP_ShieldBlock.BP_ShieldBlock_C" :Instigator (Variables|Default|GetAIRef))
    (:then
      (bind _returnvalue (Utilities|Time|SetTimerbyEvent (EventDispatchers|CreateEvent :!event Custom|PreEndAbility) (Variables|Default|GetManaCostFrequence) true))
      (Variables|Default|SetPayManaCostTask _returnvalue))
    (:Success
      (bind _output_get (Variables|Default|SetShieldRef (.AsBP%20Shield%20Block (Utilities|Casting|CastToBP_ShieldBlock _spawnedactor))))
      (Transformation|AttachComponentToComponent _output_get (Variables|/Script/Engine.Character|GetMesh (Variables|Default|GetAIRef)) "pelvis" "SnapToTarget" "KeepWorld" "KeepRelative" true)
      (Transformation|SetRelativeLocation (Variables|/Game/AbilitySystem/PlayerAbility/ShieldBlock/BP_ShieldBlock.BP_ShieldBlock_C|GetSphere (Variables|Default|GetShieldRef)) (Math|Vector|MakeVector 0.0 1e+02 -7e+01) false false)
      (Variables|Default|SetStartingWalkSpeed (Variables|/Script/Engine.CharacterMovementComponent|GetMaxWalkSpeed _charactermovement))
      (Variables|/Script/Engine.CharacterMovementComponent|SetMaxWalkSpeed _charactermovement 2.5e+02)
      (Ability|CommitAbilityCooldown false)
      (AI|AIMoveTo (AI|GetAIController (Variables|Default|GetAIRef)) "0, 0, 0" (Variables|Default|GetAI_Target) -1.0 "Default" "Default" true true
        (:OnRequestFailed
          _)
        (:OnMoveFinished
          _))
      (CallFunction|PreEndAbility))
    (:DidNotSpawn
      (Ability|EndAbility))))

(fn SetVariables
  (bind _asbp_ai_humanoid (Utilities|Casting|CastToBP_AI_Humanoid (.owneractor (Ability|GetActorInfo))))
  (bind _output_get (Variables|Default|SetAIRef _asbp_ai_humanoid))
  (bind _asactor (Utilities|Casting|CastToActor (AI|Components|Blackboard|GetValueasObject (Variables|/Script/AIModule.AIController|GetBlackboard (AI|GetAIController _output_get)) (Utilities|Name|MakeLiteralName "Target"))))
  (Variables|Default|SetAI_Target _asactor))