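; Gameplay ability for the zombie's melee slash against arena player characters.
; It pauses the AI's behavior logic and plays the attack montage from a random right- or left-hand section.
; Montage notifies sphere-overlap at the matching hand socket and damage players hit; only right-hand hits add a pain sound and damage type.
; The ability ends when the montage completes or is interrupted, restarting AI logic if the zombie is alive.
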(event Ability|EventActivateAbility
  (bind _zombieref (Variables|Default|GetZombieRef))
  (bind _zombieref_2 (Variables|Default|GetZombieRef))
  (CallFunction|SetVariables)
  (AI|Logic|StopLogic (Variables|/Script/AIModule.AIController|GetBrainComponent (AI|GetAIController (Variables|Default|GetZombieRef))) "Playing Ability")
  (bind _notifyname (Animation|Montage|PlayMontage (Variables|/Script/Engine.Character|GetMesh (Variables|Default|GetZombieRef)) "/Game/UndeadPack/Zombie/Animations/Anim_Attack1_Montage.Anim_Attack1_Montage" 1.5 0.0 (.OutItem (Utilities|Array|Random (Utilities|Array|MakeArray "RightHand" "LeftHand"))))
    (:OnCompleted
      (Ability|EndAbility :!label _label))
    (:OnInterrupted
      (goto _label))
    (:OnNotifyBegin
      (switch name _notifyname
        (:RightHit
          (bind _outactors (Collision|SphereOverlapActors (Transformation|GetSocketLocation (Variables|/Script/Engine.Character|GetMesh (Variables|Default|GetZombieRef)) "hand_r") 1e+02 (Utilities|Array|MakeArray "ObjectTypeQuery3") "/Game/Blueprint/Core/BP_PlayerArenaCharacter.BP_PlayerArenaCharacter_C" (Utilities|Array|MakeArray (Variables|Default|GetZombieRef))))
          (for _array_element _outactors
            (Game|Damage|ApplyDamage _array_element (Variables|Default|GetBase%20Damage) (AI|GetAIController _zombieref) _zombieref "/Engine/EngineDamageTypes/DmgTypeBP_Environmental.DmgTypeBP_Environmental_C")
            (Audio|PlaySoundatLocation "/Game/AUDIO/VO/Grunts/Human/Grunt_Male_Pain_Short_Cue.Grunt_Male_Pain_Short_Cue" (Transformation|GetActorLocation _array_element) "0, 0, 0" 1.0 1.0 0.0 0 0 0 0)))
        (:LeftHit
          (bind _outactors_2 (Collision|SphereOverlapActors (Transformation|GetSocketLocation (Variables|/Script/Engine.Character|GetMesh (Variables|Default|GetZombieRef)) "hand_l") 1e+02 (Utilities|Array|MakeArray "ObjectTypeQuery3") "/Game/Blueprint/Core/BP_PlayerArenaCharacter.BP_PlayerArenaCharacter_C" (Utilities|Array|MakeArray (Variables|Default|GetZombieRef))))
          (for _array_element_2 _outactors_2
            (Game|Damage|ApplyDamage _array_element_2 (Variables|Default|GetBase%20Damage) (AI|GetAIController _zombieref_2) _zombieref_2)))))))

(event Ability|EventOnEndAbility
  (params (bWasCancelled :type Boolean))
  (bind _zombieref (Variables|Default|GetZombieRef))
  (Utilities|IsValid _zombieref
    (:Is%20Valid
      (if (Default|GetIsLive _zombieref)
        (AI|Logic|StartLogic (Variables|/Script/AIModule.AIController|GetBrainComponent (AI|GetAIController _zombieref)))))))

(fn SetVariables
  (bind _asbp_ai_zombie (Utilities|Casting|CastToBP_AI_Zombie (.owneractor (Ability|GetActorInfo)))
    (:then
      (Variables|Default|SetZombieRef _asbp_ai_zombie))
    (:CastFailed
      (Ability|EndAbility))))