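; Player gameplay ability that channels a fire laser from the character toward the mouse cursor.
; On activation it starts the HUD cast animation, montage, attached emitter and a looping cost timer.
; Each successful cost commit re-aims the beam's yaw and capsule-traces pawns, applying fire and damage, with debug drawing enabled.
; A failed commit or elapsed duration clears the timer, stops the effects and plays the montage's EndSkill section.
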(event Custom|ApplyCostAndCheck
  (bind _returnvalue (Ability|CommitAbilityCost false))
  (if _returnvalue
    (CallFunction|FindTargetsandApplyDamage)
    (else
      (CallFunction|PreEndAbility))))

(event Custom|PreEndAbility
  (Default|StopCastAnimation (Variables|/Game/Blueprint/Core/BP_PlayerCharacter.BP_PlayerCharacter_C|GetHudRef (Variables|Default|GetPlayerRef)) (Variables|Default|GetSkillSlot))
  (Utilities|Time|ClearandInvalidateTimerbyHandle (Variables|Default|GetPayManaCostTask))
  (Components|Activation|Deactivate (Variables|Default|GetFireLaserPartickle))
  (Animation|Montage|PlayMontage (Variables|/Script/Engine.Character|GetMesh (Variables|Default|GetPlayerRef)) "/Game/Animation/MagPacket/AM_MagicBarrier.AM_MagicBarrier" 1.0 0.0 "EndSkill"
    (:then
      (Ability|EndAbility))))

(event Ability|EventActivateAbility
  (CallFunction|SetVariables)
  (CallFunction|GetSkillSlot)
  (Default|StartCastAnimation (Variables|/Game/Blueprint/Core/BP_PlayerCharacter.BP_PlayerCharacter_C|GetHudRef (Variables|Default|GetPlayerRef)) (Variables|Default|GetSkillSlot))
  (CallFunction|SpawnPartickle)
  (bind _returnvalue (Utilities|Time|SetTimerbyEvent (EventDispatchers|CreateEvent :!event Custom|ApplyCostAndCheck) (Variables|Default|GetManaCostFrequence) true))
  (Variables|Default|SetPayManaCostTask _returnvalue)
  (Animation|Montage|PlayMontage (Variables|/Script/Engine.Character|GetMesh (Variables|Default|GetPlayerRef)) "/Game/Animation/MagPacket/AM_MagicBarrier.AM_MagicBarrier"
    (:then
      (Utilities|FlowControl|Delay (Variables|Default|GetOneUseDuration))
      (CallFunction|PreEndAbility))
    (:OnCompleted
      (Ability|EndAbility))))

(fn SetVariables
  (bind _returnvalue (Ability|GetActorInfo))
  (bind _asbp_player_character (Utilities|Casting|CastToBP_PlayerCharacter (.owneractor _returnvalue)))
  (Variables|Default|SetPlayerRef _asbp_player_character)
  (bind _asbp_custom_player_controler (Utilities|Casting|CastToBP_CustomPlayerControler (.playercontroller _returnvalue)))
  (Variables|Default|SetPlayerControlerRef _asbp_custom_player_controler))

(fn GetSkillSlot
  (bind _playerref (Variables|Default|GetPlayerRef))
  (bind _activeskills (Variables|/Game/Blueprint/Core/BP_PlayerCharacter.BP_PlayerCharacter_C|GetActiveSkills _playerref))
  (bind _keys (Utilities|Map|Keys _activeskills))
  (bind _array_element (Utilities|Array|ForEachLoopwithBreak _keys :!label _label)
    (:LoopBody
      (if (== (.Value (Utilities|Map|Find _activeskills _array_element)) (Utilities|GetClass self))
        (Variables|Default|SetSkillSlot _array_element)
        (goto _label Break)))))

(fn FindTargetsandApplyDamage
  (bind _array (Utilities|Array|MakeArray "ObjectTypeQuery1" "ObjectTypeQuery2"))
  (bind _playerref (Variables|Default|GetPlayerRef))
  (bind _playerref_2 (Variables|Default|GetPlayerRef))
  (bind _laserrange (Variables|Default|GetLaserRange))
  (bind _firelaserpartickle (Variables|Default|GetFireLaserPartickle))
  (bind _returnvalue (Transformation|GetWorldRotation _firelaserpartickle))
  (bind _returnvalue_2 (Pawn|GetController _playerref_2))
  (bind _capsulecomponent (Variables|/Script/Engine.Character|GetCapsuleComponent _playerref))
  (bind _returnvalue_3 (Transformation|GetWorldLocation _capsulecomponent))
  (bind _asplayer_controller (Utilities|Casting|CastToPlayerController _returnvalue_2))
  (bind _hitresult (Class|PlayerController|GetHitResultUnderCursorforObjects _asplayer_controller _array true))
  (bind _returnvalue_4 (Math|Rotator|FindLookatRotation _returnvalue_3 (.location _hitresult)))
  (bind _returnvalue_5 (Math|Rotator|GetRotationXVector _returnvalue_4))
  (bind _returnvalue_6 (* _returnvalue_5 _laserrange))
  (LocalVariables|SetLookAtRotation _returnvalue_4)
  (bind (_outhits _returnvalue_7) (Class|KismetSystemLibrary|CapsuleTraceMultiforObjects (+ (* (Math|Vector|GetForwardVector _capsulecomponent) 5e+01) _returnvalue_3) (+ (Math|Vector|MakeVector (.x _returnvalue_6) (.y _returnvalue_6) 0.0) _returnvalue_3) 75.0 75.0 (Utilities|Array|MakeArray "ObjectTypeQuery3") false 0 "ForDuration" true "(R=1.000000,G=0.000000,B=0.000000,A=1.000000)" "(R=0.000000,G=1.000000,B=0.000000,A=1.000000)" (Variables|Default|GetManaCostFrequence)))
  (Transformation|SetWorldRotation _firelaserpartickle (Math|Rotator|MakeRotator (.roll _returnvalue) (.pitch _returnvalue) (- (.yaw (LocalVariables|GetLookAtRotation)) 9e+01)) false false)
  (if _returnvalue_7
    (for _array_element _outhits
      (CallFunction|ApplyFire (Variables|Default|GetPlayerRef) (.HitActor (Collision|BreakHitResult _array_element)))
      (Game|Damage|ApplyDamage (.HitActor (Collision|BreakHitResult _array_element)) (Variables|Default|GetLaserDamage) (Variables|Default|GetPlayerControlerRef) (Variables|Default|GetPlayerRef) "/Script/Engine.DamageType"))))

(fn SpawnPartickle
  (bind _output_get (LocalVariables|SetLookAtRotation (Math|Rotator|FindLookatRotation (Transformation|GetWorldLocation (Variables|/Script/Engine.Character|GetCapsuleComponent (Variables|Default|GetPlayerRef))) (.location (.HitResult (Class|PlayerController|GetHitResultUnderCursorforObjects (.AsPlayer%20Controller (Utilities|Casting|CastToPlayerController (Pawn|GetController (Variables|Default|GetPlayerRef)))) (Utilities|Array|MakeArray "ObjectTypeQuery1" "ObjectTypeQuery2") true))))))
  (bind _returnvalue (Effects|SpawnEmitterAttached "/Game/VFX/VFX_Toolkit_V1/ParticleSystems/356Days/P_FireLaser.P_FireLaser" (Variables|/Script/Engine.Character|GetMesh (Variables|Default|GetPlayerRef)) "root" "0.000000,50.000000,150.000000" (Math|Rotator|MakeRotator 9e+01 0.0 (- (.yaw _output_get) 9e+01))))
  (Variables|Default|SetFireLaserPartickle _returnvalue))