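; Player Gameplay Ability for a lightning hand attack, which turns the player toward the mouse and plays a cast montage.
; On the montage notify it plays a sound, reports AI noise, spawns a damage collider attached to the left hand, then commits and ends.
; The cursor trace still records aim location and precision aiming, but the spawn-transform math using them is unused, as is the skill-slot lookup.
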(event Ability|EventActivateAbility
  (bind _returnvalue (Game|Player|GetPlayerPawn 0))
  (bind _returnvalue_2 (Transformation|GetActorLocation _returnvalue))
  (CallFunction|SetVariables)
  (CallFunction|FindAimLocation)
  (Variables|/Game/Blueprint/Core/BP_Humanoid.BP_Humanoid_C|SetAttacking (Variables|Default|GetPlayerRef) true)
  (Default|EnableRotationtoMousePosition (Variables|Default|GetPlayerRef) true true 2.0)
  (bind _notifyname (Animation|Montage|PlayMontage (Variables|/Script/Engine.Character|GetMesh (Variables|Default|GetPlayerRef)) "/Game/Animation/WarriorAnimation/AM_LightningHand.AM_LightningHand")
    (:OnCompleted
      (Ability|EndAbility :!label _label))
    (:OnInterrupted
      (goto _label))
    (:OnNotifyBegin
      (switch name _notifyname
        (:Cast
          (Audio|PlaySoundatLocation (Variables|Default|GetCastSound) _returnvalue_2 "0, 0, 0" 1.0 1.0 0.0 0 0 (Variables|Default|GetPlayerRef) 0)
          (Class|AISenseHearing|ReportNoiseEvent _returnvalue_2 1.0 (Variables|Default|GetPlayerRef) 1.5e+03 "Ability")
          (CallFunction|SpawnHandCollision)
          (Ability|CommitAbility)
          (Ability|EndAbility))))))

(event Ability|EventOnEndAbility
  (params (bWasCancelled :type Boolean))
  (Variables|/Game/Blueprint/Core/BP_Humanoid.BP_Humanoid_C|SetAttacking (Variables|Default|GetPlayerRef) false))

(fn SpawnHandCollision
  (bind _playerref (Variables|Default|GetPlayerRef))
  (bind _mesh (Variables|/Script/Engine.Character|GetMesh _playerref))
  (bind _returnvalue (Game|SpawnActorfromClass (Variables|Default|GetHandColliderActor) (Math|Transform|MakeTransform (+ (* (Math|Vector|GetRightVector _mesh) (Variables|Default|GetHandlOffset)) (Transformation|GetSocketLocation _mesh "spine_02")) "0, 0, 0" "1.000000,1.000000,1.000000") "Undefined" 0 (Variables|Default|GetBaseDamage) (Variables|Default|GetPlayerRef)))
  (Transformation|AttachActorToActor _returnvalue (Variables|Default|GetPlayerRef) "hand_l" "KeepWorld" "SnapToTarget" "KeepWorld" true))

(fn SetVariables
  (bind _asbp_player_arena_character (Utilities|Casting|CastToBP_PlayerArenaCharacter (.owneractor (Ability|GetActorInfo))))
  (Variables|Default|SetPlayerRef _asbp_player_arena_character))

(fn GetSkillSlot)

(fn FindAimLocation
  (bind _array (Utilities|Array|MakeArray "ObjectTypeQuery1" "ObjectTypeQuery2" "ObjectTypeQuery6"))
  (bind _playerref (Variables|Default|GetPlayerRef))
  (bind _returnvalue (Pawn|GetController _playerref))
  (bind _asplayer_controller (Utilities|Casting|CastToPlayerController _returnvalue))
  (bind _hitresult (Class|PlayerController|GetHitResultUnderCursorforObjects _asplayer_controller _array true))
  (Variables|Default|SetHitAimLocation (.location _hitresult))
  (Variables|Default|SetPrecisionAiming (Utilities|Enum|Equal(Enum) (Collision|GetCollisionObjectType (.hitcomponent _hitresult)) "ECC_Destructible")))