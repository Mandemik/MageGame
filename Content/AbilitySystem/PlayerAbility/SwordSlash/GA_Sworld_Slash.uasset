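; Gameplay ability for an AI humanoid's sword slash that damages player arena characters.
; Activation pauses the owner's AI brain logic and plays the slash montage from a random right- or left-hand section.
; Only the Right Hit notify is handled: a sphere overlap at the right hand applies slash damage and plays pain grunts.
; Montage completion or interruption ends the ability, restarting AI logic if the owner is alive.
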(event Ability|EventActivateAbility
  (bind _humanref (Variables|Default|GetHumanRef))
  (CallFunction|SetVariables)
  (AI|Logic|StopLogic (Variables|/Script/AIModule.AIController|GetBrainComponent (AI|GetAIController (Variables|Default|GetHumanRef))) "Playing Ability")
  (bind _notifyname (Animation|Montage|PlayMontage (Variables|/Script/Engine.Character|GetMesh (Variables|Default|GetHumanRef)) "/Game/Animation/WarriorAnimation/AM_Sword_Slash.AM_Sword_Slash" 1.5 0.0 (.OutItem (Utilities|Array|Random (Utilities|Array|MakeArray "RightHand" "LeftHand"))))
    (:OnCompleted
      (Ability|EndAbility :!label _label))
    (:OnInterrupted
      (Development|PrintString "Hello")
      (goto _label))
    (:OnNotifyBegin
      (switch name _notifyname
        (:RightHit
          (bind _outactors (Collision|SphereOverlapActors (Transformation|GetSocketLocation (Variables|/Script/Engine.Character|GetMesh (Variables|Default|GetHumanRef)) "hand_r") 1e+02 (Utilities|Array|MakeArray "ObjectTypeQuery3") "/Game/Blueprint/Core/BP_PlayerArenaCharacter.BP_PlayerArenaCharacter_C" (Utilities|Array|MakeArray (Variables|Default|GetHumanRef))))
          (for _array_element _outactors
            (Game|Damage|ApplyDamage _array_element (Variables|Default|GetBase%20Damage) (AI|GetAIController _humanref) _humanref "/Game/AbilitySystem/PlayerAbility/SwordSlash/DT_SworldSlash.DT_SworldSlash_C")
            (Audio|PlaySoundatLocation "/Game/AUDIO/VO/Grunts/Human/Grunt_Male_Pain_Short_Cue.Grunt_Male_Pain_Short_Cue" (Transformation|GetActorLocation _array_element) "0, 0, 0" 1.0 1.0 0.0 0 0 0 0)))))))

(event Ability|EventOnEndAbility
  (params (bWasCancelled :type Boolean))
  (bind _humanref (Variables|Default|GetHumanRef))
  (Utilities|IsValid _humanref
    (:Is%20Valid
      (if (Default|GetIsLive _humanref)
        (AI|Logic|StartLogic (Variables|/Script/AIModule.AIController|GetBrainComponent (AI|GetAIController _humanref)))))))

(fn SetVariables
  (bind _asbp_humanoid (Utilities|Casting|CastToBP_Humanoid (.owneractor (Ability|GetActorInfo)))
    (:then
      (Variables|Default|SetHumanRef _asbp_humanoid))
    (:CastFailed
      (Ability|EndAbility))))