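; Projectile for the player's Wind Push ability that damages actors caught in a forward-sweeping box.
; On BeginPlay a timeline lerps the box's relative X from a start to an end offset.
; Each overlapped actor is recorded so it takes point damage only once, using the wind push damage type, the projectile's forward vector as hit direction and the instigator as damage causer.
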(event OnComponentBeginOverlap(Box)
  (params (OverlappedComponent :type Primitive%20Component%20Object%20Reference) (OtherActor :type Actor%20Object%20Reference) (OtherComp :type Primitive%20Component%20Object%20Reference) (OtherBodyIndex :type Integer) (bFromSweep :type Boolean) (SweepResult :type Hit%20Result%20Structure%20%28by%20ref%29))
  (if (not (Utilities|Array|ContainsItem (Variables|Default|GetOverlapedActors) OtherActor))
    (Utilities|Array|Add (Variables|Default|GetOverlapedActors) OtherActor)
    (Game|Damage|ApplyPointDamage OtherActor (Variables|Default|GetBase%20Damage) (Transformation|GetActorForwardVector) SweepResult 0 (Variables|Actor|GetInstigator) "/Game/AbilitySystem/PlayerAbility/WindPush/DT_WindPush.DT_WindPush_C")))

(event EventBeginPlay
  (bind _progress (Timeline|Timeline_0 PlayFromStart)
    (:Update
      (Transformation|SetRelativeLocation (Variables|Default|GetBox) (Math|Vector|MakeVector (Math|Float|Lerp (Variables|Default|GetStartOffset) (Variables|Default|GetEndOffset) _progress) 0.0 0.0) false false))))

(fn ConstructionScript)