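; Player gameplay ability named WindPush that actually casts a BP_FireBall_Projectile.
; Activation traces under the cursor for an aim point, flags Destructible hits for precision aiming, turns the player toward the mouse and plays a cast montage.
; The montage notify reports AI noise, spawns the projectile, commits, starts the HUD cooldown and ends the ability.
; The aim-based spawn transform math and skill-slot lookup are left unconnected.
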(event Ability|EventActivateAbility
  (CallFunction|SetVariables)
  (CallFunction|FindAimLocation)
  (Variables|/Game/Blueprint/Core/BP_Humanoid.BP_Humanoid_C|SetAttacking (Variables|Default|GetPlayerRef) true)
  (Default|EnableRotationtoMousePosition (Variables|Default|GetPlayerRef) true true 2.0)
  (bind _notifyname (Animation|Montage|PlayMontage (Variables|/Script/Engine.Character|GetMesh (Variables|Default|GetPlayerRef)) "/Game/Animation/UE_Manekin/Base/AM_SelfCast_Retargeted.AM_SelfCast_Retargeted")
    (:OnCompleted
      (Ability|EndAbility :!label _label))
    (:OnInterrupted
      (goto _label))
    (:OnNotifyBegin
      (switch name _notifyname
        (:Cast
          (Class|AISenseHearing|ReportNoiseEvent (Transformation|GetActorLocation (Game|Player|GetPlayerPawn 0)) 1.0 (Variables|Default|GetPlayerRef) 1.5e+03 "Ability")
          (CallFunction|SpawnFireBall)
          (Ability|CommitAbility)
          (Default|StartCooldownAnimation (Variables|/Game/Blueprint/Core/BP_PlayerArenaCharacter.BP_PlayerArenaCharacter_C|GetHudRef (Variables|Default|GetPlayerRef)) (Class|GameplayAbility|GetCooldownTimeRemaining) (Variables|Default|GetSkill%20Slot))
          (Ability|EndAbility))))))

(event Ability|EventOnEndAbility
  (params (bWasCancelled :type Boolean))
  (Variables|/Game/Blueprint/Core/BP_Humanoid.BP_Humanoid_C|SetAttacking (Variables|Default|GetPlayerRef) false))

(fn SpawnFireBall
  (bind _returnvalue (Game|SpawnActorfromClass "/Game/AbilitySystem/PlayerAbility/Fireball/BP_FireBall_Projectile.BP_FireBall_Projectile_C" (Utilities|CalculateSpawnTransform) "AdjustIfPossibleButAlwaysSpawn" 0 (Variables|Default|GetExplosion%20Radius) (Variables|Default|GetBaseDamage) (Variables|Default|GetPlayerRef) :!pinned true)) ; Spawn projectile
  (Collision|IgnoreActorwhenMoving (Variables|/Game/AbilitySystem/PlayerAbility/Fireball/BP_FireBall_Projectile.BP_FireBall_Projectile_C|GetSphere1 _returnvalue) (Variables|Default|GetPlayerRef) true))

(fn SetVariables
  (bind _asbp_player_arena_character (Utilities|Casting|CastToBP_PlayerArenaCharacter (.owneractor (Ability|GetActorInfo))))
  (Variables|Default|SetPlayerRef _asbp_player_arena_character))

(fn GetSkillSlot)

(fn FindAimLocation
  (bind _array (Utilities|Array|MakeArray "ObjectTypeQuery1" "ObjectTypeQuery2" "ObjectTypeQuery6"))
  (bind _playerref (Variables|Default|GetPlayerRef))
  (bind _returnvalue (Pawn|GetController _playerref))
  (bind _asplayer_controller (Utilities|Casting|CastToPlayerController _returnvalue))
  (bind _hitresult (Class|PlayerController|GetHitResultUnderCursorforObjects _asplayer_controller _array true))
  (Variables|Default|SetHitAimLocation (.location _hitresult))
  (Variables|Default|SetPrecisionAiming (Utilities|Enum|Equal(Enum) (Collision|GetCollisionObjectType (.hitcomponent _hitresult)) "ECC_Destructible")))