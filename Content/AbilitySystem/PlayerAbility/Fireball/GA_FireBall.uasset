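; Player fireball Gameplay Ability that plays a sped-up cast montage and spawns a projectile with the ability's damage and explosion radius.
; On the montage notify, it spawns the projectile ignoring the caster, then commits the ability, starts the HUD cooldown and ends.
; The HUD slot comes from matching this class in the player's active skills.
; CalculateSpawnTransform holds cursor-aim math with height-dependent pitch, left unconnected.
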(event Ability|EventActivateAbility
  (CallFunction|SetVariables)
  (CallFunction|GetSkillSlot)
  (bind _notifyname (Animation|Montage|PlayMontage (Variables|/Script/Engine.Character|GetMesh (Variables|Default|GetPlayerRef)) "/Game/Animation/MagPacket/AM_SelfCast.AM_SelfCast" 1.4)
    (:OnCompleted
      (Ability|EndAbility :!label _label))
    (:OnInterrupted
      (goto _label))
    (:OnNotifyBegin
      (switch name _notifyname
        (:Cast
          (CallFunction|SpawnFireBall)
          (Ability|CommitAbility)
          (Default|StartCooldownAnimation (Variables|/Game/Blueprint/Core/BP_PlayerCharacter.BP_PlayerCharacter_C|GetHudRef (Variables|Default|GetPlayerRef)) (Class|GameplayAbility|GetCooldownTimeRemaining) (Variables|Default|GetSkill%20Slot))
          (Ability|EndAbility))))))

(fn SpawnFireBall
  (bind _returnvalue (Game|SpawnActorfromClass "/Game/AbilitySystem/PlayerAbility/Fireball/BP_FireBall_Projectile.BP_FireBall_Projectile_C" (Utilities|CalculateSpawnTransform) "AdjustIfPossibleButAlwaysSpawn" 0 (Variables|Default|GetExplosion%20Radius) (Variables|Default|GetBaseDamage) (Variables|Default|GetPlayerRef) :!pinned true)) ; Spawn projectile
  (Collision|IgnoreActorwhenMoving (Variables|/Game/AbilitySystem/PlayerAbility/Fireball/BP_FireBall_Projectile.BP_FireBall_Projectile_C|GetSphere1 _returnvalue) (Variables|Default|GetPlayerRef) true))

(fn SetVariables
  (bind _asbp_player_character (Utilities|Casting|CastToBP_PlayerCharacter (.owneractor (Ability|GetActorInfo))))
  (Variables|Default|SetPlayerRef _asbp_player_character))

(fn GetSkillSlot
  (bind _playerref (Variables|Default|GetPlayerRef))
  (bind _activeskills (Variables|/Game/Blueprint/Core/BP_PlayerCharacter.BP_PlayerCharacter_C|GetActiveSkills _playerref))
  (bind _keys (Utilities|Map|Keys _activeskills))
  (bind _array_element (Utilities|Array|ForEachLoopwithBreak _keys :!label _label)
    (:LoopBody
      (if (== (.Value (Utilities|Map|Find _activeskills _array_element)) (Utilities|GetClass self))
        (Variables|Default|SetSkill%20Slot _array_element)
        (goto _label Break)))))