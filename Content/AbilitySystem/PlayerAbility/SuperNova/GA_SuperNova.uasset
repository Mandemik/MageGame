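; SuperNova player gameplay ability: a self-cast burst that consumes the burning status on nearby humanoids to damage them.
; On activation it finds its HUD skill slot and plays a montage, ending when that completes or is interrupted.
; The montage notify runs a sphere overlap, strips Status.InFire effects and damages those targets, then commits and starts the HUD cooldown.
; An input press after the notify also ends it; CalculateSpawnTransform holds only unused nodes.
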(event Ability|EventActivateAbility
  (CallFunction|SetVariables)
  (CallFunction|GetSkillSlot)
  (bind _notifyname (Animation|Montage|PlayMontage (Variables|/Script/Engine.Character|GetMesh (Variables|Default|GetPlayerRef)) "/Game/Animation/MagPacket/AM_SelfCast.AM_SelfCast" 1.4)
    (:OnCompleted
      (Ability|EndAbility :!label _label))
    (:OnInterrupted
      (goto _label))
    (:OnNotifyBegin
      (switch name _notifyname
        (:Cast
          (CallFunction|ConsumeFireStatus)
          (Ability|CommitAbility)
          (Default|StartCooldownAnimation (Variables|/Game/Blueprint/Core/BP_PlayerCharacter.BP_PlayerCharacter_C|GetHudRef (Variables|Default|GetPlayerRef)) (Class|GameplayAbility|GetCooldownTimeRemaining) (Variables|Default|GetSkill%20Slot))
          (Ability|Tasks|WaitInputPress true
            (:OnPress
              (Ability|EndAbility))))))))

(fn SetVariables
  (bind _asbp_player_character (Utilities|Casting|CastToBP_PlayerCharacter (.owneractor (Ability|GetActorInfo))))
  (Variables|Default|SetPlayerRef _asbp_player_character))

(fn GetSkillSlot
  (bind _playerref (Variables|Default|GetPlayerRef))
  (bind _activeskills (Variables|/Game/Blueprint/Core/BP_PlayerCharacter.BP_PlayerCharacter_C|GetActiveSkills _playerref))
  (bind _keys (Utilities|Map|Keys _activeskills))
  (bind _array_element (Utilities|Array|ForEachLoopwithBreak _keys :!label _label)
    (:LoopBody
      (if (== (.Value (Utilities|Map|Find _activeskills _array_element)) (Utilities|GetClass self))
        (Variables|Default|SetSkill%20Slot _array_element)
        (goto _label Break)))))

(fn ConsumeFireStatus
  (bind _playerref (Variables|Default|GetPlayerRef))
  (bind _outactors (Collision|SphereOverlapActors (Transformation|GetActorLocation (Variables|Default|GetPlayerRef)) (Variables|Default|GetSphere%20Radius) (Utilities|Array|MakeArray "ObjectTypeQuery3") "/Game/Blueprint/Core/BP_Humanoid.BP_Humanoid_C"))
  (for _array_element _outactors
    (LocalVariables|SetTarget _array_element)
    (if (GameplayTags|HasMatchingGameplayTag (Ability|GetAbilitySystemComponent _array_element) "(TagName=\"Status.InFire\")")
      (Development|PrintString "Target")
      (GameplayEffects|RemoveActiveEffectswithGrantedTags (Ability|GetAbilitySystemComponent (LocalVariables|GetTarget)) "(GameplayTags=((TagName=\"Status.InFire\")))")
      (Game|Damage|ApplyDamage (LocalVariables|GetTarget) (Variables|Default|GetConsumeDamage) (Pawn|GetController _playerref) _playerref "/Script/Engine.DamageType"))))