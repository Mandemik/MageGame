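; GA_FireWave is a player gameplay ability that casts a wave of fire toward the cursor.
; On activation it finds its skill slot and cursor aim point, commits the cost and plays a cast montage.
; The montage notify spawns the Niagara effect and capsule-traces for pawns, applying fire and damage once per actor via the ActorsHit list.
; It then starts the slot's HUD cooldown animation and ends the ability.
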(event Ability|EventActivateAbility
  (CallFunction|SetVariables)
  (CallFunction|GetSkillSlot)
  (CallFunction|FindAimLocation)
  (Ability|CommitAbilityCost false)
  (bind _notifyname (Animation|Montage|PlayMontage (Variables|/Script/Engine.Character|GetMesh (Variables|Default|GetPlayerRef)) "/Game/Animation/UE_Manekin/Base/AM_SelfCast_Retargeted.AM_SelfCast_Retargeted" 1.4)
    (:OnCompleted
      (Ability|EndAbility :!label _label))
    (:OnInterrupted
      (goto _label))
    (:OnNotifyBegin
      (switch name _notifyname
        (:Cast
          (CallFunction|SpawnFireWave)
          (Default|StartCooldownAnimation (Variables|/Game/Blueprint/Core/BP_PlayerCharacter.BP_PlayerCharacter_C|GetHudRef (Variables|Default|GetPlayerRef)) (Class|GameplayAbility|GetCooldownTimeRemaining) (Variables|Default|GetSkill%20Slot))
          (Ability|EndAbility))))))

(fn SpawnFireWave
  (bind _returnvalue (Utilities|CalculateSpawnTransform))
  (bind _hitaimlocation (Variables|Default|GetHitAimLocation))
  (bind _playerref (Variables|Default|GetPlayerRef))
  (bind _playerref_2 (Variables|Default|GetPlayerRef))
  (bind _returnvalue_2 (Transformation|GetActorLocation _playerref))
  (Audio|PlaySoundatLocation "/Game/AUDIO/SFX/Abilities/Heatwave/SFX_Heatwave_Shot_Cue.SFX_Heatwave_Shot_Cue" _returnvalue_2 "0, 0, 0" 1.0 1.0 0.0 0 0 0 0)
  (Niagara|SpawnSystematLocation "/Game/BlinkAndDashVFX/VFX_Niagara/NS_Dash_Fire.NS_Dash_Fire" (.location _returnvalue) (.rotation _returnvalue) "1.000000,1.000000,0.500000")
  (bind _outhits (Class|KismetSystemLibrary|CapsuleTraceMultiforObjects (.location _returnvalue) (+ (* (Math|Rotator|FindLookatRotation _returnvalue_2 (Math|Vector|MakeVector (.x _hitaimlocation) (.y _hitaimlocation) (.Z (Math|Vector|BreakVector _returnvalue_2)))) 1e+03) (.location _returnvalue)) 1e+02 1e+02 (Utilities|Array|MakeArray "ObjectTypeQuery3") false 0 "None" true))
  (for _array_element _outhits
    (if (not (Utilities|Array|ContainsItem (LocalVariables|GetActorsHit) (.hitactor _array_element)))
      (Utilities|Array|Add (LocalVariables|GetActorsHit) (.hitactor _array_element))
      (CallFunction|ApplyFire (Variables|Default|GetPlayerRef) (.hitactor _array_element))
      (Game|Damage|ApplyDamage (.hitactor _array_element) (Variables|Default|GetBaseDamage) (Pawn|GetController _playerref_2) _playerref_2 "/Script/Engine.DamageType")
      (Audio|PlaySoundatLocation "/Game/AUDIO/SFX/Abilities/Fireball/Fireball_Impact.Fireball_Impact" _returnvalue_2 "0, 0, 0" 1.0 1.0 0.0 0 0 0 0))))

(fn SetVariables
  (bind _asbp_player_character (Utilities|Casting|CastToBP_PlayerCharacter (.owneractor (Ability|GetActorInfo))))
  (Variables|Default|SetPlayerRef _asbp_player_character))

(fn GetSkillSlot
  (bind _playerref (Variables|Default|GetPlayerRef))
  (bind _activeskills (Variables|/Game/Blueprint/Core/BP_PlayerCharacter.BP_PlayerCharacter_C|GetActiveSkills _playerref))
  (bind _keys (Utilities|Map|Keys _activeskills))
  (bind _array_element (Utilities|Array|ForEachLoopwithBreak _keys :!label _label)
    (:LoopBody
      (if (== (.Value (Utilities|Map|Find _activeskills _array_element)) (Utilities|GetClass self))
        (Variables|Default|SetSkill%20Slot _array_element)
        (goto _label Break)))))

(fn FindAimLocation
  (Variables|Default|SetHitAimLocation (.location (.HitResult (Class|PlayerController|GetHitResultUnderCursorforObjects (.AsPlayer%20Controller (Utilities|Casting|CastToPlayerController (Pawn|GetController (Variables|Default|GetPlayerRef)))) (Utilities|Array|MakeArray "ObjectTypeQuery1" "ObjectTypeQuery2") true)))))