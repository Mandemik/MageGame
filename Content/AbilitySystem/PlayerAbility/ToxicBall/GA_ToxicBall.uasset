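; GA_ToxicBall is a player gameplay ability that casts a toxic ball projectile toward the mouse cursor.
; On activation it traces under the cursor, flags precision aiming on destructible hits, turns the player to the mouse and plays a cast montage.
; The montage notify plays sound, reports AI noise, spawns the projectile with radius and damage, then commits and starts the HUD cooldown.
; Skill-slot lookup logic is present but never runs.
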(event Ability|EventActivateAbility
  (bind _returnvalue (Game|Player|GetPlayerPawn 0))
  (bind _returnvalue_2 (Transformation|GetActorLocation _returnvalue))
  (CallFunction|SetVariables)
  (CallFunction|FindAimLocation)
  (Default|EnableRotationtoMousePosition (Variables|Default|GetPlayerRef) true true 2.0)
  (bind _notifyname (Animation|Montage|PlayMontage (Variables|/Script/Engine.Character|GetMesh (Variables|Default|GetPlayerRef)) "/Game/Animation/UE_Manekin/Base/AM_SelfCast_Retargeted.AM_SelfCast_Retargeted" 1.4)
    (:OnCompleted
      (Ability|EndAbility :!label _label))
    (:OnInterrupted
      (goto _label))
    (:OnNotifyBegin
      (switch name _notifyname
        (:Cast
          (Audio|PlaySoundatLocation "/Game/AUDIO/SFX/Abilities/Fireball/Fireball_Cast.Fireball_Cast" _returnvalue_2 "0, 0, 0" 1.0 1.0 0.0 0 0 (Variables|Default|GetPlayerRef) 0)
          (Class|AISenseHearing|ReportNoiseEvent _returnvalue_2 1.0 (Variables|Default|GetPlayerRef) 1.5e+03 "Ability")
          (CallFunction|SpawnToxicBall)
          (Ability|CommitAbility)
          (Default|StartCooldownAnimation (Variables|/Game/Blueprint/Core/BP_PlayerArenaCharacter.BP_PlayerArenaCharacter_C|GetHudRef (Variables|Default|GetPlayerRef)) (Class|GameplayAbility|GetCooldownTimeRemaining) (Variables|Default|GetSkill%20Slot))
          (Ability|EndAbility))))))

(fn SpawnToxicBall
  (bind _returnvalue (Game|SpawnActorfromClass "/Game/AbilitySystem/PlayerAbility/ToxicBall/BP_ToxicBall_Projectile.BP_ToxicBall_Projectile_C" (Utilities|CalculateSpawnTransform) "AdjustIfPossibleButAlwaysSpawn" 0 (Variables|Default|GetExplosion%20Radius) (Variables|Default|GetBaseDamage) (Variables|Default|GetPlayerRef) :!pinned true)) ; Spawn projectile
  (Collision|IgnoreActorwhenMoving (Variables|/Game/AbilitySystem/PlayerAbility/ToxicBall/BP_ToxicBall_Projectile.BP_ToxicBall_Projectile_C|GetSphere1 _returnvalue) (Variables|Default|GetPlayerRef) true))

(fn SetVariables
  (bind _asbp_player_arena_character (Utilities|Casting|CastToBP_PlayerArenaCharacter (.owneractor (Ability|GetActorInfo))))
  (Variables|Default|SetPlayerRef _asbp_player_arena_character))

(fn GetSkillSlot)

(fn FindAimLocation
  (bind _array (Utilities|Array|MakeArray "ObjectTypeQuery1" "ObjectTypeQuery2" "ObjectTypeQuery6"))
  (bind _playerref (Variables|Default|GetPlayerRef))
  (bind _returnvalue (Pawn|GetController _playerref))
  (bind _asplayer_controller (Utilities|Casting|CastToPlayerController _returnvalue))
  (bind _hitresult (Class|PlayerController|GetHitResultUnderCursorforObjects _asplayer_controller _array true))
  (Variables|Default|SetHitAimLocation (.location _hitresult))
  (Variables|Default|SetPrecisionAiming (Utilities|Enum|Equal(Enum) (Collision|GetCollisionObjectType (.hitcomponent _hitresult)) "ECC_Destructible")))