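; Player Gameplay Ability for a normal dash that sends the character forward with a sound and Niagara effect.
; On activation it hides the mesh, disables input, ignores Pawn and WorldDynamic collision, then calls the character's MakeDash.
; It commits only the cooldown and animates it on the HUD slot found by matching its class in ActiveSkills.
; A roll-ended callback restores mesh and collision and ends the ability, which re-enables input.
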(event Custom|CustomEvent_1
  (bind _playerref (Variables|Default|GetPlayerRef))
  (Niagara|SpawnSystematLocation (Variables|Default|GetDashEffect) (Class|CharacterMovementComponent|GetLastUpdateLocation (Variables|/Script/Engine.Character|GetCharacterMovement _playerref)) (Math|Conversions|RotationFromXVector (Transformation|GetActorForwardVector _playerref)) (Math|Vector|MakeVector 0.3 0.3 0.3))
  (CallFunction|RevertChangefromDash)
  (Ability|EndAbility))

(event Ability|EventActivateAbility
  (bind _playerref (Variables|Default|GetPlayerRef))
  (CallFunction|SetVariables)
  (CallFunction|GetSkillShot)
  (CallFunction|FindDashLocation)
  (CallFunction|PreperPlayertoDash)
  (Audio|PlaySoundatLocation "/Game/AUDIO/SFX/Abilities/Dash/SFX_Ability_Dash_Cue.SFX_Ability_Dash_Cue" (Variables|Default|GetDashLocation) "0, 0, 0" 1.0 1.0 0.0 0 0 0 0)
  (Ability|CommitAbilityCooldown false true)
  (Default|StartCooldownAnimation (Variables|/Game/Blueprint/Core/BP_PlayerCharacter.BP_PlayerCharacter_C|GetHudRef (Variables|Default|GetPlayerRef)) (Class|GameplayAbility|GetCooldownTimeRemaining) (Variables|Default|GetSkill%20Slot))
  (Niagara|SpawnSystematLocation (Variables|Default|GetDashEffect) (Class|CharacterMovementComponent|GetLastUpdateLocation (Variables|/Script/Engine.Character|GetCharacterMovement _playerref)) (Math|Conversions|RotationFromXVector (Transformation|GetActorForwardVector _playerref)) (Math|Vector|MakeVector (/ (Variables|Default|GetDashDistance) 1e+03) 0.5 0.5))
  (Default|MakeDash (Variables|Default|GetPlayerRef) 1.5e+03))

(event Ability|EventOnEndAbility
  (params (bWasCancelled :type Boolean))
  (Input|EnableInput (Variables|Default|GetPlayerRef) (Variables|Default|GetPlayerControlerRef)))

(fn SetVariables
  (bind _returnvalue (Ability|GetActorInfo))
  (bind _asbp_player_character (Utilities|Casting|CastToBP_PlayerCharacter (.owneractor _returnvalue))
    (:then
      (bind _output_get (Variables|Default|SetPlayerRef _asbp_player_character))
      (Variables|Default|SetMesh (Variables|/Script/Engine.Character|GetMesh _output_get))
      (Variables|Default|SetPlayerControlerRef (.playercontroller _returnvalue)))
    (:CastFailed
      (Development|PrintString (Utilities|String|Append (Utilities|GetObjectName self) "faild cast to Player"))
      (Ability|EndAbility))))

(fn FindDashLocation
  (bind _playerref (Variables|Default|GetPlayerRef))
  (Variables|Default|SetDashLocation (+ (Class|CharacterMovementComponent|GetLastUpdateLocation (Variables|/Script/Engine.Character|GetCharacterMovement _playerref)) (* (Transformation|GetActorForwardVector _playerref) (Variables|Default|GetDashDistance)))))

(fn PreperPlayertoDash
  (bind _playerref (Variables|Default|GetPlayerRef))
  (bind _playerref_2 (Variables|Default|GetPlayerRef))
  (Development|SetHiddeninGame (Variables|Default|GetMesh) true false)
  (Input|DisableInput _playerref_2 (Variables|Default|GetPlayerControlerRef))
  (EventDispatchers|BindEventtoRollEnded _playerref_2 (EventDispatchers|CreateEvent :!event Custom|CustomEvent_1))
  (Collision|SetCollisionResponsetoChannel (Variables|/Script/Engine.Character|GetMesh _playerref) "ECC_WorldDynamic" "ECR_Ignore")
  (Collision|SetCollisionResponsetoChannel (Variables|/Script/Engine.Character|GetCapsuleComponent _playerref) "ECC_Pawn" "ECR_Ignore"))

(fn GetSkillShot
  (bind _playerref (Variables|Default|GetPlayerRef))
  (bind _activeskills (Variables|/Game/Blueprint/Core/BP_PlayerCharacter.BP_PlayerCharacter_C|GetActiveSkills _playerref))
  (bind _keys (Utilities|Map|Keys _activeskills))
  (bind _array_element (Utilities|Array|ForEachLoopwithBreak _keys :!label _label)
    (:LoopBody
      (if (== (.Value (Utilities|Map|Find _activeskills _array_element)) (Utilities|GetClass self))
        (Variables|Default|SetSkill%20Slot _array_element)
        (goto _label Break)))))

(fn RevertChangefromDash
  (bind _playerref (Variables|Default|GetPlayerRef))
  (Development|SetHiddeninGame (Variables|Default|GetMesh) false false)
  (Collision|SetCollisionResponsetoChannel (Variables|/Script/Engine.Character|GetMesh _playerref) "ECC_WorldDynamic" "ECR_Block")
  (Collision|SetCollisionResponsetoChannel (Variables|/Script/Engine.Character|GetCapsuleComponent _playerref) "ECC_Pawn" "ECR_Block"))