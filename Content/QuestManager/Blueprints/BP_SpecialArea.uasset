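; BP_SpecialArea is a box trigger volume that marks a named, colored special area for the quest manager.
; When a pawn begins or ends overlap, it gets the quest manager through that pawn's controller and calls UpdateSpecialArea to add or remove the area with its name and color.
; The construction script sizes the box from an extent variable and raises it by the Z extent from its relative location.
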(event OnComponentBeginOverlap(Box)
  (params (OverlappedComponent :type Primitive%20Component%20Object%20Reference) (OtherActor :type Actor%20Object%20Reference) (OtherComp :type Primitive%20Component%20Object%20Reference) (OtherBodyIndex :type Integer) (bFromSweep :type Boolean) (SweepResult :type Hit%20Result%20Structure%20%28by%20ref%29))
  (bind _aspawn (Utilities|Casting|CastToPawn OtherActor))
  (bind _returnvalue (Utilities|GetQuestManager (Pawn|GetController _aspawn))
    (:then
      (Default|UpdateSpecialArea _returnvalue true (Variables|SpecialAreaSettings|GetName) (Variables|SpecialAreaSettings|GetColor)))))

(event OnComponentEndOverlap(Box)
  (params (OverlappedComponent :type Primitive%20Component%20Object%20Reference) (OtherActor :type Actor%20Object%20Reference) (OtherComp :type Primitive%20Component%20Object%20Reference) (OtherBodyIndex :type Integer))
  (bind _aspawn (Utilities|Casting|CastToPawn OtherActor))
  (bind _returnvalue (Utilities|GetQuestManager (Pawn|GetController _aspawn))
    (:then
      (Default|UpdateSpecialArea _returnvalue false (Variables|SpecialAreaSettings|GetName) (Variables|SpecialAreaSettings|GetColor)))))

(fn ConstructionScript
  (bind _box (Variables|Default|GetBox))
  (bind _relativelocation (Variables|/Script/Engine.SceneComponent|GetRelativeLocation _box))
  (Components|Box|SetBoxExtent (Variables|Default|GetBox) (Variables|SpecialAreaSettings|GetInBoxExtent) true)
  (Transformation|SetRelativeLocation (Variables|Default|GetBox) (Math|Vector|MakeVector (.x _relativelocation) (.y _relativelocation) (+ (.z _relativelocation) (.z (Variables|SpecialAreaSettings|GetInBoxExtent)))) false false))