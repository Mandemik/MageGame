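; BP_QuestManager is a central registry for quest targets and start points.
; Adding or removing a target triggers a server update that calls OnTargetArrayUpdated on each PlayerState's Manager_Mission component.
; Helper functions look up targets and their owners by name, and pick a random start point filtered by name.
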(event Custom|SR_Update_Targets_On_Players
  ;[1 1 1] Update Quest Targets On Every Player By Server
  (for _array_element (Variables|/Script/Engine.GameStateBase|GetPlayerArray (Game|GetGameState))
    (Utilities|IsValid (Actor|GetComponentbyClass _array_element "/Game/QuestManager/Blueprints/Components/Manager_Mission.Manager_Mission_C")
      (:Is%20Valid
        (Default|OnTargetArrayUpdated (Actor|GetComponentbyClass _array_element "/Game/QuestManager/Blueprints/Components/Manager_Mission.Manager_Mission_C"))))))

(event EventTick
  (params (DeltaSeconds :type Float%20%28single-precision%29)))

(fn ConstructionScript)

(fn AssignTarget
  (params (QuestTarget :type Manager%20Quest%20Target%20Object%20Reference))
  (Utilities|Array|Add (Variables|Default|GetCurrentTargets) QuestTarget)
  (CallFunction|SRUpdateTargetsonPlayers))

(fn RemoveTarget
  (params (QuestTarget :type Manager%20Quest%20Target%20Object%20Reference))
  (Utilities|Array|RemoveItem (Variables|Default|GetCurrentTargets) QuestTarget)
  (CallFunction|SRUpdateTargetsonPlayers))

(fn FindinTargets
  (params (TargetName :type Name))
  (bind _array_element (Utilities|Array|ForEachLoopwithBreak (Variables|Default|GetCurrentTargets) :!label _label)
    (:LoopBody
      (if (Utilities|Name|Equal(Name) (Variables|/Game/QuestManager/Blueprints/Components/Manager_QuestTarget.Manager_QuestTarget_C|GetTargetName _array_element) TargetName)
        (LocalVariables|SetLocReturn _array_element)
        (goto _label Break)))
    (:Completed
      (return (LocalVariables|GetLocReturn)))))

(fn GetTargetOwner
  (params (TargetName :type Name))
  (bind _returnvalue (CallFunction|FindinTargets TargetName))
  (bind _returnvalue_2 (Components|GetOwner _returnvalue))
  (Utilities|IsValid _returnvalue
    (:Is%20Valid
      (Utilities|IsValid _returnvalue_2
        (:Is%20Valid
          (return _returnvalue_2))))))

(fn FindRandomStartPoint
  (params (StartPoints :type Array%20of%20Names))
  (for _array_element (Variables|Default|GetStartPoints)
    (if (Utilities|Array|ContainsItem StartPoints (Variables|/Game/QuestManager/Blueprints/BP_QuestStartPoint.BP_QuestStartPoint_C|GetStartPointName _array_element))
      (Utilities|Array|Add (LocalVariables|GetLocPoints) _array_element)))
  (bind _output_get (LocalVariables|SetLocReturn (.OutItem (Utilities|Array|Random (LocalVariables|GetLocPoints)))))
  (return (Utilities|IsValid _output_get) (LocalVariables|GetLocReturn)))

(fn AddStartPoint
  (params (StartPoint :type BP%20Quest%20Start%20Point%20Object%20Reference))
  (Utilities|Array|AddUnique (Variables|Default|GetStartPoints) StartPoint))

(fn RemoveStartPoint
  (params (StartPoint :type BP%20Quest%20Start%20Point%20Object%20Reference))
  (Utilities|Array|RemoveItem (Variables|Default|GetStartPoints) StartPoint))