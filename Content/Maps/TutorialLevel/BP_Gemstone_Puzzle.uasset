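; BP_Gemstone_Puzzle is a tutorial-level puzzle gemstone that lights up when it takes any damage and reports to a door master.
; On BeginPlay it creates a dynamic material instance from its static mesh's material.
; Damage calls ActiveGemstone, which stores the active state and switches the emissive color between the active color and black, then passes itself to DoorMaster through NewGemStoneActive.
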(event Game|Damage|EventAnyDamage
  (params (Damage :type Float%20%28single-precision%29) (DamageType :type Damage%20Type%20Object%20Reference) (InstigatedBy :type Controller%20Object%20Reference) (DamageCauser :type Actor%20Object%20Reference))
  (CallFunction|ActiveGemstone true)
  (Default|NewGemStoneActive (Variables|Default|GetDoorMaster) self))

(event EventBeginPlay
  (bind _returnvalue (Rendering|Material|CreateDynamicMaterialInstance (Variables|Debug|GetStaticMeshComponent) 0 (Rendering|Material|GetMaterial (Variables|Debug|GetStaticMeshComponent) 0) "None" :!class /Script/Engine.PrimitiveComponent))
  (Variables|Default|SetM_Gemstone _returnvalue))

(fn ConstructionScript)

(fn ActiveGemstone
  (params (Active? :type Boolean))
  (bind _output_get (Variables|Default|SetIsActive Active?))
  (if _output_get
    (Rendering|Material|SetVectorParameterValue (Variables|Default|GetM_Gemstone) "EmissiveColor" (Variables|Default|GetL_Color_Active) :!class /Script/Engine.MaterialInstanceDynamic)
    (else
      (Rendering|Material|SetVectorParameterValue :self (Variables|Default|GetM_Gemstone) :ParameterName "EmissiveColor" :!class /Script/Engine.MaterialInstanceDynamic))))