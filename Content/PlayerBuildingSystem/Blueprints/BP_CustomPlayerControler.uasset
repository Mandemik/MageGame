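; Player controller for the building system that turns input into movement, building and ability actions on the possessed BuildingCharacter.
; BeginPlay caches the character, then key and action events forward build menus, selection, interaction and a damage test to its PlayerBuildingComponent.
; R activates the GA_FireBall gameplay ability.
; Turn and LookUp axes store scaled offsets that Tick uses to move the mouse cursor, with a debug print.
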(event EventBeginPlay
  (bind _asbuilding_character (Utilities|Casting|CastToBuildingCharacter (Pawn|GetControlledPawn))
    (:then
      (Variables|Default|SetControlledCharacter _asbuilding_character))
    (:CastFailed
      (Development|PrintString "ERROR : Wrrong character is selected on Player Controler." true true "(R=1.000000,G=0.000000,B=0.034709,A=1.000000)"))))

(event EventTick
  (params (DeltaSeconds :type Float%20%28single-precision%29))
  (bind (_locationx _locationy) (Game|Player|GetMousePosition))
  (if (or (!= (Variables|Default|GetControlerX) 0.0) (!= (Variables|Default|GetControlerY) 0.0))
    (Development|PrintString (Utilities|String|Append "Controler X = " (Utilities|String|ToString(Float) (Variables|Default|GetControlerX)) " Controler Y = " (Utilities|String|ToString(Float) (Variables|Default|GetControlerY))) true true "(R=0.000000,G=0.660000,B=1.000000,A=1.000000)" 0.1)
    (Class|PlayerController|SetMouseLocation (Math|Float|Truncate (+ _locationx (Variables|Default|GetControlerX))) (Math|Float|Truncate (+ _locationy (Variables|Default|GetControlerY))))))

(event Input|ActionEvents|InputActionOpenBuildMenu
  (params (Key :type Key%20Structure))
  (bind _controlledcharacter (Variables|Default|GetControlledCharacter))
  (bind _playerbuildingcomponent (Variables|/Game/PlayerBuildingSystem/Blueprints/BuildingCharacter.BuildingCharacter_C|GetPlayerBuildingComponent _controlledcharacter))
  ;[1 1 1] Toggle building menu
  (:Pressed
    (Default|ToggleBuildMenu _playerbuildingcomponent (not (Variables|/Game/PlayerBuildingSystem/Blueprints/Components/PlayerBuildingComponent.PlayerBuildingComponent_C|GetBuildMenuOpen _playerbuildingcomponent)))))

(event Input|ActionEvents|InputActionSelectBuildForMenu
  (params (Key :type Key%20Structure))
  (bind _controlledcharacter (Variables|Default|GetControlledCharacter))
  (bind _playerbuildingcomponent (Variables|/Game/PlayerBuildingSystem/Blueprints/BuildingCharacter.BuildingCharacter_C|GetPlayerBuildingComponent _controlledcharacter))
  ;[1 1 1] Left mouse button input
  (:Pressed
    (Default|SelectBuildingtoBuild _playerbuildingcomponent))
  (:Released
    (Default|LeftMouseReleased _playerbuildingcomponent)))

(event Input|ActionEvents|InputActionInteract
  (params (Key :type Key%20Structure))
  (bind _controlledcharacter (Variables|Default|GetControlledCharacter))
  (bind _playerbuildingcomponent (Variables|/Game/PlayerBuildingSystem/Blueprints/BuildingCharacter.BuildingCharacter_C|GetPlayerBuildingComponent _controlledcharacter))
  ;[1 1 1] Interact input
  (:Pressed
    (Default|ClientInteract _playerbuildingcomponent true))
  (:Released
    (Default|ClientInteract _playerbuildingcomponent false)))

(event Input|ActionEvents|InputActionAttack
  (params (Key :type Key%20Structure)))

(event Input|AxisEvents|InputAxisLookUp
  (params (AxisValue :type Float%20%28single-precision%29))
  (if (!= AxisValue 0.0)
    (Variables|Default|SetControlerY (* AxisValue 1e+01))
    (else
      (Variables|Default|SetControlerY 0.0))))

(event Input|AxisEvents|InputAxisTurn
  (params (AxisValue :type Float%20%28single-precision%29))
  (if (!= AxisValue 0.0)
    (Variables|Default|SetControlerX (* AxisValue 1e+01))
    (else
      (Variables|Default|SetControlerX 0.0))))

(event Input|AxisEvents|InputAxisMoveForward
  (params (AxisValue :type Float%20%28single-precision%29))
  (Pawn|Input|AddMovementInput (Variables|Default|GetControlledCharacter) (Math|Vector|GetForwardVector (Math|Rotator|MakeRotator 0.0 0.0 (.Yaw (Math|Rotator|BreakRotator (Pawn|GetControlRotation :!class /Script/Engine.Controller))))) AxisValue false))

(event Input|AxisEvents|InputAxisMoveRight
  (params (AxisValue :type Float%20%28single-precision%29))
  (Pawn|Input|AddMovementInput (Variables|Default|GetControlledCharacter) (Math|Vector|GetRightVector (Math|Rotator|MakeRotator 0.0 0.0 (.Yaw (Math|Rotator|BreakRotator (Pawn|GetControlRotation :!class /Script/Engine.Controller))))) AxisValue false))

(event Input|KeyboardEvents|R
  (params (Key :type Key%20Structure))
  (:Pressed
    (Abilities|TryActivateAbilitybyClass (Ability|GetAbilitySystemComponent (Variables|Default|GetControlledCharacter)) "/Game/AbilitySystem/Ability/Fireball/GA_FireBall.GA_FireBall_C" true)))

(event Input|KeyboardEvents|T
  (params (Key :type Key%20Structure))
  ;[1 1 1] Damage Demo
  (:Pressed
    (Default|ClientDamageTest (Variables|/Game/PlayerBuildingSystem/Blueprints/BuildingCharacter.BuildingCharacter_C|GetPlayerBuildingComponent (Variables|Default|GetControlledCharacter)))))

(event Input|KeyboardEvents|Q
  (params (Key :type Key%20Structure))
  (bind _controlledcharacter (Variables|Default|GetControlledCharacter))
  (bind _playerbuildingcomponent (Variables|/Game/PlayerBuildingSystem/Blueprints/BuildingCharacter.BuildingCharacter_C|GetPlayerBuildingComponent _controlledcharacter))
  ;[1 1 1] Toggle building options menu
  (:Pressed
    (Default|ToggleBuildingOptionsMenu _playerbuildingcomponent true))
  (:Released
    (Default|ToggleBuildingOptionsMenu _playerbuildingcomponent false)))

(fn ConstructionScript)