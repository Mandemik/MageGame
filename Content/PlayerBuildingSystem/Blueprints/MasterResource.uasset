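; MasterResource is a collectible resource actor in the player building system that gives an item to the player who interacts with it.
; Its Interact event calls ResourceCollected, which casts the building component's owning player to BP_PlayerCharacter, adds the item and amount to its InventoryManager, then destroys the actor.
; An unconnected branch holds partial-harvest logic that would deplete CurrentResources through the ResourceAmount lookup and report to the building component's server call.
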(event EventInteract
  (params (Player%20Building%20Component :type Player%20Building%20Component%20Object%20Reference))
  (CallFunction|ResourceCollected Player%20Building%20Component (Variables|Default|GetAmmount)))

(fn ConstructionScript)

(fn ResourceCollected
  (params (PlayerBuilding :type Player%20Building%20Component%20Object%20Reference) (Ammount :type Integer))
  (Default|AddItem (Variables|/Game/Blueprint/Core/BP_PlayerCharacter.BP_PlayerCharacter_C|GetInventoryManager (.AsBP%20Player%20Character (Utilities|Casting|CastToBP_PlayerCharacter (Variables|/Game/PlayerBuildingSystem/Blueprints/Components/PlayerBuildingComponent.PlayerBuildingComponent_C|GetOwning%20Player PlayerBuilding)))) (Variables|Default|GetItem) Ammount)
  (Actor|DestroyActor))

(fn ResourceAmount
  (params (Resource :type EItems%20Enum :default "NewEnumerator0"))
  (for _array_element (Variables|Default|GetCurrentResources)
    (if (Utilities|Enum|Equal(Enum) (.Resource (Utilities|Struct|BreakS_ResourceValues _array_element)) Resource)
      (return (.Amount (Utilities|Struct|BreakS_ResourceValues _array_element))))))